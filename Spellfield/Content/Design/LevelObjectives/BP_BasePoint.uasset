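; BP_BasePoint is a base level-objective point that tracks which players stand inside its radius while active.
; Sphere overlaps add or remove player IDs through BPI_Character_And_Controller and fire empty PlayerEntered and PlayerLeft hooks.
; Activation, immediate or timer-delayed, registers players already inside, while deactivation notifies via OnPointDeactivated and clears the list.
; The construction script sizes the sphere and debug displays from Radius, and debug materials distinguish pending from active.
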(event OnComponentBeginOverlap(Sphere)
  (params (OverlappedComponent :type Primitive%20Component%20Object%20Reference) (OtherActor :type Actor%20Object%20Reference) (OtherComp :type Primitive%20Component%20Object%20Reference) (OtherBodyIndex :type Integer) (bFromSweep :type Boolean) (SweepResult :type Hit%20Result%20Structure%20%28by%20ref%29))
  ;[0.15 0.15 0.15 0.5] Collision handling to detect entering and exiting point
  (if (and (Utilities|DoesObjectImplementInterface OtherActor "/Game/Design/Blueprints/Interfaces/BPI_Character_And_Controller.BPI_Character_And_Controller_C") (Variables|Default|GetIsActive))
    (bind _id (Class|BPICharacterandController|GetID(Message) OtherActor))
    (if (not (Utilities|Set|Contains (Variables|Default|GetPlayersOnPoint) _id))
      (Utilities|Set|Add (Variables|Default|GetPlayersOnPoint) _id)
      (CallFunction|PlayerEntered _id))))

(event OnComponentEndOverlap(Sphere)
  (params (OverlappedComponent :type Primitive%20Component%20Object%20Reference) (OtherActor :type Actor%20Object%20Reference) (OtherComp :type Primitive%20Component%20Object%20Reference) (OtherBodyIndex :type Integer))
  ;[0.15 0.15 0.15 0.5] Collision handling to detect entering and exiting point
  (if (and (Utilities|DoesObjectImplementInterface OtherActor "/Game/Design/Blueprints/Interfaces/BPI_Character_And_Controller.BPI_Character_And_Controller_C") (Variables|Default|GetIsActive))
    (bind _id (Class|BPICharacterandController|GetID(Message) OtherActor))
    (if (Utilities|Set|Contains (Variables|Default|GetPlayersOnPoint) _id)
      (Utilities|Set|Remove (Variables|Default|GetPlayersOnPoint) _id)
      (CallFunction|PlayerLeft _id))))

(event Custom|Player%20Entered
  (params (ID :type Integer))
  ;[0.15 0.15 0.15 0.5] Players entering and exiting point
)

(event Custom|PlayerLeft
  (params (ID :type Integer))
  ;[0.15 0.15 0.15 0.5] Players entering and exiting point
)

(event Custom|SetActiveIn
  (params (TimeSeconds :type Float%20%28double-precision%29))
  (if (> TimeSeconds 0.0)
    (Utilities|Time|SetTimerbyEvent (EventDispatchers|CreateEvent :!event Custom|ActivatePoint) TimeSeconds)
    (Rendering|SetVisibility (Variables|Default|GetDebugRadiusDisplay) true false)
    (Rendering|Material|SetMaterial (Variables|Default|GetDebugRadiusDisplay) 0 "/Game/Design/LevelObjectives/M_DebugRadiusMatInactive.M_DebugRadiusMatInactive")
    (else
      (CallFunction|ActivatePoint))))

(event Custom|DeactivatePoint
  ;[0.15 0.15 0.15 0.5] Deactivate point and clear queue
  (Default|CallOnPointDeactivated)
  (Variables|Default|SetIsActive false)
  (Utilities|Set|Clear (Variables|Default|GetPlayersOnPoint))
  (Rendering|SetVisibility (Variables|Default|GetDebugRadiusDisplay) false false))

(event Custom|ActivatePoint
  ;[0.15 0.15 0.15 0.5] Activate point, perform check for players already on point and add to queue
  (Variables|Default|SetIsActive true)
  (Utilities|Set|Clear (Variables|Default|GetPlayersOnPoint))
  (for _array_element (Collision|GetOverlappingActors (Variables|Default|GetSphere) "/Game/Design/Blueprints/Character/BP_PlayerCharacter.BP_PlayerCharacter_C" :!class /Script/Engine.PrimitiveComponent)
    (bind _id (Class|BPICharacterandController|GetID(Message) _array_element))
    (Utilities|Set|Add (Variables|Default|GetPlayersOnPoint) _id)
    (CallFunction|PlayerEntered _id))
  (Rendering|SetVisibility (Variables|Default|GetDebugRadiusDisplay) true false)
  (Rendering|Material|SetMaterial (Variables|Default|GetDebugRadiusDisplay) 0 "/Game/Design/LevelObjectives/M_DebugRadiusMat.M_DebugRadiusMat"))

(event EventBeginPlay
  (bind _aswbp_debug_cpdisplay (Utilities|Casting|CastToWBP_DebugCPDisplay (UserInterface|GetWidget (Variables|Default|GetDebugFillDisplay))))
  (Variables|Default|SetFill _aswbp_debug_cpdisplay))

(fn ConstructionScript
  (bind _radius (Variables|Default|GetRadius))
  (bind _radius_2 (Variables|Default|GetRadius))
  (bind _returnvalue (* _radius_2 0.02))
  (bind _returnvalue_2 (* _radius 2.0))
  (|CallParentFunction)
  (Components|Sphere|SetSphereRadius (Variables|Default|GetSphere) (Variables|Default|GetRadius) false)
  (Transformation|SetWorldScale3D (Variables|Default|GetDebugRadiusDisplay) (Math|Vector|MakeVector _returnvalue _returnvalue _returnvalue))
  (Class|WidgetComponent|SetDrawSize (Variables|Default|GetDebugFillDisplay) (Math|Vector2D|MakeVector2D _returnvalue_2 _returnvalue_2)))