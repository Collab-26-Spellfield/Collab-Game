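; Control point objective that grants points at a set interval to a player standing alone inside its sphere.
; Overlaps with actors implementing the character interface add IDs to a set, though end overlap also calls PlayerEntered, leaving PlayerLeft unused.
; Each change checks for a single occupant against IsCounting to start or clear a looping timer for awarding points.
; The construction script sizes the sphere and debug display from Radius.
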(event OnComponentBeginOverlap(Sphere)
  (params (OverlappedComponent :type Primitive%20Component%20Object%20Reference) (OtherActor :type Actor%20Object%20Reference) (OtherComp :type Primitive%20Component%20Object%20Reference) (OtherBodyIndex :type Integer) (bFromSweep :type Boolean) (SweepResult :type Hit%20Result%20Structure%20%28by%20ref%29))
  ;[0.15 0.15 0.15 0.5] Collision handling to detect entering and exiting point
  (if (Utilities|DoesObjectImplementInterface OtherActor "/Game/Design/Blueprints/Interfaces/BPI_Character_And_Controller.BPI_Character_And_Controller_C")
    (bind _id (Class|BPICharacterandController|GetID(Message) OtherActor))
    (CallFunction|PlayerEntered _id)))

(event OnComponentEndOverlap(Sphere)
  (params (OverlappedComponent :type Primitive%20Component%20Object%20Reference) (OtherActor :type Actor%20Object%20Reference) (OtherComp :type Primitive%20Component%20Object%20Reference) (OtherBodyIndex :type Integer))
  ;[0.15 0.15 0.15 0.5] Collision handling to detect entering and exiting point
  (if (Utilities|DoesObjectImplementInterface OtherActor "/Game/Design/Blueprints/Interfaces/BPI_Character_And_Controller.BPI_Character_And_Controller_C")
    (bind _id (Class|BPICharacterandController|GetID(Message) OtherActor))
    (CallFunction|PlayerEntered _id)))

(event Custom|Player%20Entered
  (params (ID :type Integer))
  ;[0.15 0.15 0.15 0.5] Players entering and exiting point
  (Utilities|Set|Add (Variables|Default|GetPlayers%20On%20Point) ID)
  (CallFunction|PlayersChanged))

(event Custom|PlayerLeft
  (params (ID :type Integer))
  ;[0.15 0.15 0.15 0.5] Players entering and exiting point
  (Utilities|Set|Remove (Variables|Default|GetPlayers%20On%20Point) ID)
  (CallFunction|PlayersChanged))

(event Custom|PlayersChanged
  ;[0.15 0.15 0.15 0.5] Start timer if there is only 1 player on the point. Otherwise, stop timer.
  (if (Class|KismetMathLibrary|XORBoolean (== (Utilities|Set|Length (Variables|Default|GetPlayers%20On%20Point)) 1) (Variables|Default|GetIsCounting))
    (if (== (Utilities|Set|Length (Variables|Default|GetPlayers%20On%20Point)) 1)
      (bind _returnvalue (Utilities|Time|SetTimerbyEvent (EventDispatchers|CreateEvent :!event Custom|Grant%20Point) (Variables|Default|GetTimeBetweenPointAssignment) true))
      (Variables|Default|SetTimer _returnvalue)
      (else
        (Utilities|Time|ClearandInvalidateTimerbyHandle (Variables|Default|GetTimer))))))

(event Custom|Grant%20Point
  ;[0.15 0.15 0.15 0.5] Give points to the only player on the point
  (Default|CallGrantPoints (Utilities|Set|GetItemByIndex (Variables|Default|GetPlayers%20On%20Point)) (Variables|Default|GetPointsToGrant)))

(fn ConstructionScript
  (bind _radius (Variables|Default|GetRadius))
  (bind _returnvalue (* _radius 0.02))
  (|CallParentFunction)
  (Components|Sphere|SetSphereRadius (Variables|Default|GetSphere) (Variables|Default|GetRadius) false)
  (Transformation|SetWorldScale3D (Variables|Default|GetDebugRadiusDisplay) (Math|Vector|MakeVector _returnvalue _returnvalue _returnvalue)))