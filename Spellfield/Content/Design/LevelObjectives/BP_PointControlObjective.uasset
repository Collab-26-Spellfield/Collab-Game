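; Point-control level objective that grants a point to a player who holds it alone until capture completes, then deactivates.
; Player enter and leave events re-count occupants: none resets, one sets the capturer and runs the Capture timeline, more halts it.
; The timeline drives a Fill indicator coloured per player, and progress resets when the capturer changes or leaves.
; Activation and deactivation extend the parent objective's logic with a capture reset.
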(event Custom|ResumeCapturing
  (Utilities|FlowControl|Sequence
    (:then_0
      (bind _t (Timeline|Capture SetNewTime)
        (:Update
          (bind _output_get (Variables|Default|SetCaptureProgress _t))
          (Default|SetFill (Variables|Default|GetFill) _output_get))
        (:Finished
          (CallFunction|GrantPoint))))
    (:then_1
      (Timeline|Capture Play))))

(event Custom|ResetCapturing
  (CallFunction|StopCapturing)
  (Variables|Default|SetCaptureProgress 0.0)
  (Variables|Default|SetCapturerer -1)
  (Default|SetFill (Variables|Default|GetFill) 1.0)
  (Default|SetColour (Variables|Default|GetFill) "(R=0.200000,G=0.200000,B=0.200000,A=1.000000)"))

(event Custom|Grant%20Point
  ;[0.15 0.15 0.15 0.5] Give points to the next player in queue and move them to the end of the queue
  (Default|CallGrantPoints (Variables|Default|GetCapturerer) 1)
  (CallFunction|DeactivatePoint))

(event Custom|StopCapturing
  (bind _t (Timeline|Capture Stop)
    (:Update
      (bind _output_get (Variables|Default|SetCaptureProgress _t))
      (Default|SetFill (Variables|Default|GetFill) _output_get))
    (:Finished
      (CallFunction|GrantPoint))))

(event Custom|PlayersChanged
  (params (PlayerCount :type Integer))
  (switch int PlayerCount
    (:Default
      (CallFunction|StopCapturing))
    (:0
      (CallFunction|ResetCapturing))
    (:1
      (CallFunction|SetCapturer (Utilities|Set|GetItemByIndex (Variables|Default|GetPlayersOnPoint)))
      (CallFunction|ResumeCapturing))))

(event Custom|SetCapturer
  (params (ID :type Integer))
  (if (!= ID (Variables|Default|GetCapturerer))
    (bind _output_get (Variables|Default|SetCapturerer ID))
    (Variables|Default|SetCaptureProgress 0.0)
    (Default|SetColour (Variables|Default|GetFill) (Utilities|Select :Index _output_get :Option%200 "(R=0.075298,G=0.058214,B=0.302083,A=1.000000)" :Option%201 "(R=0.395833,G=0.028863,B=0.037106,A=1.000000)" :Option%202 "(R=0.078187,G=0.270498,B=0.024158,A=1.000000)" :Option%203 "(R=0.715694,G=0.603828,B=0.066626,A=1.000000)"))))

(event EventPlayerEntered
  (params (ID :type Integer))
  ;[0.15 0.15 0.15 0.5] Players entering and exiting point
  (CallFunction|PlayersChanged (Utilities|Set|Length (Variables|Default|GetPlayersOnPoint))))

(event EventPlayerLeft
  (params (ID :type Integer))
  ;[0.15 0.15 0.15 0.5] Players entering and exiting point
  (if (== (Variables|Default|GetCapturerer) ID)
    (CallFunction|ResetCapturing))
  (CallFunction|PlayersChanged (Utilities|Set|Length (Variables|Default|GetPlayersOnPoint))))

(event EventActivatePoint
  ;[0.15 0.15 0.15 0.5] Activate point, perform check for players already on point and add to queue
  (CallFunction|ResetCapturing)
  (|CallParentFunction))

(event EventDeactivatePoint
  ;[0.15 0.15 0.15 0.5] Deactivate point and clear queue
  (|CallParentFunction)
  (CallFunction|ResetCapturing))

(fn ConstructionScript
  (|CallParentFunction))