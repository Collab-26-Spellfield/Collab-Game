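; BP_IncrementalCollectibleObjective is a wandering collectible objective that flees nearby players, intended to award its holder points over time.
; Move picks a random direction, or a randomized average away from players in FearRadius, then sphere-traces for a reachable target.
; A distance-scaled Timeline sweeps it there, chaining immediately when chased and otherwise setting a random-delay timer.
; Collected hides it below the level, but pickup, drop and point-timer logic are unwired.
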(event OnComponentBeginOverlap(CollectionRadius)
  (params (OverlappedComponent :type Primitive%20Component%20Object%20Reference) (OtherActor :type Actor%20Object%20Reference) (OtherComp :type Primitive%20Component%20Object%20Reference) (OtherBodyIndex :type Integer) (bFromSweep :type Boolean) (SweepResult :type Hit%20Result%20Structure%20%28by%20ref%29))
  ;[0.15 0.15 0.15 0.5] Overlaps for chasing and pickup
)

(event OnComponentBeginOverlap(FearRadius)
  (params (OverlappedComponent :type Primitive%20Component%20Object%20Reference) (OtherActor :type Actor%20Object%20Reference) (OtherComp :type Primitive%20Component%20Object%20Reference) (OtherBodyIndex :type Integer) (bFromSweep :type Boolean) (SweepResult :type Hit%20Result%20Structure%20%28by%20ref%29))
  ;[0.15 0.15 0.15 0.5] Overlaps for chasing and pickup
  (CallFunction|Move))

(event Custom|Collected
  (params (CollectedBy :type Integer))
  ;[0.15 0.15 0.15 0.5] When the pickup is collected, hide it
  (Variables|Default|SetHolder CollectedBy)
  (Audio|Components|Audio|Stop (Variables|Default|GetTimeline))
  (Transformation|SetActorLocation "0.000000,0.000000,-10000.000000" false false))

(event Custom|Move
  ;[0.15 0.15 0.15 0.5] Movement logic
  ;[0.15 0.15 0.15 0.5] Find a valid space to move to
  (bind (_direction _ischased) (CallFunction|GetMovementDirection))
  (Variables|Default|SetIs%20Chased _ischased)
  (bind _output_get (Variables|Default|SetStartPosition (Transformation|GetActorLocation)))
  (bind (_outhit _returnvalue) (Collision|SphereTraceByChannel _output_get (+ (Variables|Default|GetStartPosition) (* _direction (Math|Float|SelectFloat (Variables|Default|GetChaseTraceDistance) (Variables|Default|GetTraceDistance) (Variables|Default|GetIs%20Chased)))) (Variables|Default|GetVisualRadius) "TraceTypeQuery1" false 0 "None"))
  ;[0.15 0.15 0.15 0.5] Setup target destination and how long it will take to get there
  (Variables|Default|SetTargetPosition (Math|Vector|SelectVector (.ImpactPoint (Collision|BreakHitResult _outhit)) (.TraceEnd (Collision|BreakHitResult _outhit)) _returnvalue))
  (Components|Timeline|SetPlayRate (Variables|Default|GetTimeline) (/ (Math|Float|SelectFloat (Variables|Default|GetChasing%20Speed) (Variables|Default|GetSpeed) (Variables|Default|GetIs%20Chased)) (Math|Vector|Distance(Vector) (Variables|Default|GetStartPosition) (Variables|Default|GetTargetPosition))))
  ;[0.15 0.15 0.15 0.5] Move to target destination
  (bind _t (Timeline|Timeline PlayFromStart)
    (:Update
      (Transformation|SetActorLocation (Math|Vector|Lerp(Vector) (Variables|Default|GetStartPosition) (Variables|Default|GetTargetPosition) _t) true false))
    (:Finished
      (if (Variables|Default|GetIs%20Chased)
        (CallFunction|Move)
        (else
          (Utilities|Time|SetTimerbyEvent (EventDispatchers|CreateEvent :!event Custom|Move) (Math|Random|RandomFloatinRange 1.0 2.0)))))))

(event Custom|Drop
  ;[0.15 0.15 0.15 0.5] Drops the collectible, called when the player holding it dies.
)

(event Custom|Give%20Points
  ;[0.15 0.15 0.15 0.5] Gives points to the holder of the pickup
  (Default|CallGrantPoints (Variables|Default|GetHolder) (Variables|Default|GetPointsValue)))

(event EventBeginPlay
  ;[0.15 0.15 0.15 0.5] Probably want to set up a proper init
  (CallFunction|Move))

(fn ConstructionScript
  (|CallParentFunction))

(fn GetMovementDirection
  ;[0.15 0.15 0.15 0.5] Find nearby players
  (bind _output_get (LocalVariables|SetOverlaps (Collision|GetOverlappingActors (Variables|Default|GetFearRadius) "/Game/Design/Blueprints/Character/BP_PlayerCharacter.BP_PlayerCharacter_C" :!class /Script/Engine.PrimitiveComponent)))
  ;[0.15 0.15 0.15 0.5] If no players to avoid, just move in a random direction
  (if (> (Utilities|Array|Length _output_get) 0)
    (for _array_element (LocalVariables|GetOverlaps)
      ;[0.15 0.15 0.15 0.5] Get avoidance direction from all nearby players
      (LocalVariables|SetRunning%20Sum (+ (- (Transformation|GetActorLocation) (Transformation|GetActorLocation _array_element)) (LocalVariables|GetRunning%20Sum))))
    (return (Class|KismetMathLibrary|VectorNormal2D (+ (* (Class|KismetMathLibrary|VectorNormal2D (/ (LocalVariables|GetRunning%20Sum) (Utilities|Array|Length (LocalVariables|GetOverlaps))) 0.0001) 3.0) (Class|KismetMathLibrary|VectorNormal2D (Math|Random|RandomUnitVector) 0.0001)) 0.0001) true)
    (else
      (return (Class|KismetMathLibrary|VectorNormal2D (Math|Random|RandomUnitVector) 0.0001) false))))