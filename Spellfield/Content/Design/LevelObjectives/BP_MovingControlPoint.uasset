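; BP_MovingControlPoint is a level objective control point whose Sphere component travels continuously along a Path spline.
; BeginPlay records the start time in Birthday.
; Each Tick derives the distance from Speed and elapsed time, wraps it by the spline length to loop, and moves the Sphere to that world location with sweep enabled.
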(event EventTick
  (params (DeltaSeconds :type Float%20%28single-precision%29))
  ;[0.15 0.15 0.15 0.5] Move it along the path
  (Transformation|SetWorldLocation (Variables|Default|GetSphere) (Spline|GetLocationatDistanceAlongSpline (Variables|Default|GetPath) (Math|Float|%(Float) (* (Variables|Default|GetSpeed) (- (Utilities|Time|GetTimeSeconds) (Variables|Default|GetBirthday))) (Spline|GetSplineLength (Variables|Default|GetPath))) "World") true false))

(event EventBeginPlay
  ;[0.15 0.15 0.15 0.5] Establish a better init
  (Variables|Default|SetBirthday (Utilities|Time|GetTimeSeconds)))

(fn ConstructionScript
  (|CallParentFunction))