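; BP_KingpinCrown is a crown pickup for a Kingpin level objective that binds to the player who collects it.
; On binding it hides itself, moves to the player's XY at a fixed height, attaches to them keeping world transform, disables its collection radius and records the holder's ID.
; When the game ends, it destroys itself.
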(event Custom|BindToPlayer
  (params (Player :type BP%20Player%20Character%20Object%20Reference))
  (bind _returnvalue (Transformation|GetActorLocation Player))
  ;[0.15 0.15 0.15 0.5] When the pickup is collected, bind it to the player
  (Rendering|SetActorHiddenInGame true)
  (Transformation|SetActorLocation (Math|Vector|MakeVector (.x _returnvalue) (.y _returnvalue) 2e+02) false false)
  (Transformation|AttachActorToActor Player "None" "KeepWorld" "KeepWorld" "KeepWorld" true)
  (Components|Activation|SetActive (Variables|Default|GetCollectionRadius) false false)
  (Variables|Default|SetHolder (Variables|/Game/Design/Blueprints/Character/BP_PlayerCharacter.BP_PlayerCharacter_C|GetMy%20ID Player)))

(event EventGameEnd
  (Actor|DestroyActor))

(fn ConstructionScript
  (|CallParentFunction))