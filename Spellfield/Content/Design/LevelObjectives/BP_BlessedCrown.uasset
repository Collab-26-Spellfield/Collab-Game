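; Level objective crown that awards its holder a point every second through a looping timer.
; Once Init has run, a living character overlapping the collection radius picks it up, attaching it above the pawn and binding to that pawn's death event.
; On death it detaches at the pawn's position at movement height, stops scoring and briefly delays reactivating pickup.
; GameEnd destroys it.
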(event OnComponentBeginOverlap(CollectionRadius)
  (params (OverlappedComponent :type Primitive%20Component%20Object%20Reference) (OtherActor :type Actor%20Object%20Reference) (OtherComp :type Primitive%20Component%20Object%20Reference) (OtherBodyIndex :type Integer) (bFromSweep :type Boolean) (SweepResult :type Hit%20Result%20Structure%20%28by%20ref%29))
  ;[0.15 0.15 0.15 0.5] Overlap for pickup
  (if (and (Utilities|DoesObjectImplementInterface OtherActor "/Game/Design/Blueprints/Interfaces/BPI_Character_And_Controller.BPI_Character_And_Controller_C") (Variables|Default|GetStarted))
    (bind _player (Class|BPICharacterandController|GetPlayer(Message) OtherActor))
    (if (not (Variables|/Game/Design/Blueprints/Character/BP_PlayerCharacter.BP_PlayerCharacter_C|GetIsDead _player))
      (bind _id (Class|BPICharacterandController|GetID(Message) OtherActor))
      (CallFunction|Collected _id))))

(event Custom|Collected
  (params (CollectedBy :type Integer))
  ;[0.15 0.15 0.15 0.5] When the pickup is collected, bind it to the player
  (if (== (Variables|Default|GetHolder) -1)
    (Variables|Default|SetHolder CollectedBy)
    (CallFunction|Bind)
    (CallFunction|BeginPointsTimer)))

(event Custom|Drop
  ;[0.15 0.15 0.15 0.5] Drops the collectible, called when the player holding it dies.
  (if (!= (Variables|Default|GetHolder) -1)
    (CallFunction|Unbind)
    (CallFunction|EndPointsTimer)))

(event Custom|DeathHandler
  (params (Killer :type Integer) (Victim :type Integer))
  (CallFunction|Drop))

(event Custom|Bind
  ;[0.15 0.15 0.15 0.5] When the pickup is collected, bind it to the player
  (bind _playerconnectiondata (Class|BPIPlayerConnectionInfo|GetPlayerData(Message) (Game|GetGameInstance)))
  (Transformation|SetActorLocation (Math|Vector|MakeVector (.x (Transformation|GetActorLocation (.playerpawn (.Value (Utilities|Map|Find _playerconnectiondata (Variables|Default|GetHolder)))))) (.y (Transformation|GetActorLocation (.playerpawn (.Value (Utilities|Map|Find _playerconnectiondata (Variables|Default|GetHolder)))))) 2e+02) false false)
  (Transformation|AttachActorToActor (.playerpawn (.Value (Utilities|Map|Find _playerconnectiondata (Variables|Default|GetHolder)))) "None" "KeepWorld" "KeepWorld" "KeepWorld" true)
  (EventDispatchers|BindEventtoOnDeath (.playerpawn (.Value (Utilities|Map|Find _playerconnectiondata (Variables|Default|GetHolder)))) (EventDispatchers|CreateEvent :!event Custom|DeathHandler))
  (Components|Activation|SetActive (Variables|Default|GetCollectionRadius) false false))

(event Custom|Unbind
  ;[0.15 0.15 0.15 0.5] Drops the collectible, called when the player holding it dies.
  (bind _playerconnectiondata (Class|BPIPlayerConnectionInfo|GetPlayerData(Message) (Game|GetGameInstance)))
  (Transformation|DetachFromActor "KeepRelative" "KeepRelative" "KeepRelative")
  (Transformation|SetActorLocation (Math|Vector|MakeVector (.x (Transformation|GetActorLocation (.playerpawn (.Value (Utilities|Map|Find _playerconnectiondata (Variables|Default|GetHolder)))))) (.y (Transformation|GetActorLocation (.playerpawn (.Value (Utilities|Map|Find _playerconnectiondata (Variables|Default|GetHolder)))))) (Variables|Default|GetMovementHeight)) false false)
  (EventDispatchers|UnbindEventfromOnDeath (.playerpawn (.Value (Utilities|Map|Find _playerconnectiondata (Variables|Default|GetHolder)))) (EventDispatchers|CreateEvent :!event Custom|DeathHandler))
  (Variables|Default|SetHolder -1)
  (Components|Activation|SetActive (Variables|Default|GetCollectionRadius) false false)
  (Utilities|Time|SetTimerbyEvent (delegate Custom|Reactivate) 0.15))

(event Custom|Reactivate
  ;[0.15 0.15 0.15 0.5] Drops the collectible, called when the player holding it dies.
  (Components|Activation|SetActive (Variables|Default|GetCollectionRadius) true false))

(event Custom|BeginPointsTimer
  ;[0.15 0.15 0.15 0.5] Points timer
  (bind _returnvalue (Utilities|Time|SetTimerbyEvent (delegate Custom|GrantPoint) 1.0 true))
  (Variables|Default|SetPointsTimer _returnvalue)
  (CallFunction|GrantPoint))

(event Custom|EndPointsTimer
  ;[0.15 0.15 0.15 0.5] Points timer
  (Utilities|Time|ClearandInvalidateTimerbyHandle (Variables|Default|GetPointsTimer)))

(event Custom|GrantPoint
  ;[0.15 0.15 0.15 0.5] Points timer
  (if (> (Variables|Default|GetHolder) -1)
    (Default|CallGrantPoints (Variables|Default|GetHolder) 1)))

(event EventGameEnd
  (Actor|DestroyActor))

(event EventBeginPlay
  (bind _returnvalue (Transformation|GetActorLocation))
  (Transformation|SetActorLocation (Math|Vector|MakeVector (.x _returnvalue) (.y _returnvalue) (Variables|Default|GetMovementHeight)) false false))

(event EventInit
  (Variables|Default|SetStarted true))

(fn ConstructionScript
  (|CallParentFunction))