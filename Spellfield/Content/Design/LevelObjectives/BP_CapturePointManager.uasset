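; Capture point manager that rotates which BP_BasePoint in the level is active.
; On Init it gathers all points and binds to their deactivation events; each deactivation schedules a randomly chosen point to activate after ActivationDelay.
; Selection rerolls at random with an iteration cap of about 20; despite the name ChooseRandomInactivePoint, its loop rerolls while the pick is inactive.
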(event Custom|ChooseNewPoint
  (bind _point (CallFunction|ChooseRandomInactivePoint))
  (Default|SetActivein _point (Variables|Default|GetActivationDelay)))

(event Custom|PointDeactivated
  (CallFunction|ChooseNewPoint))

(event EventInit
  (bind _outactors (Actor|GetAllActorsOfClass "/Game/Design/LevelObjectives/BP_BasePoint.BP_BasePoint_C"))
  (bind _output_get (Variables|Default|SetPoints _outactors))
  (for _array_element _output_get
    (EventDispatchers|BindEventtoOnPointDeactivated _array_element (delegate Custom|PointDeactivated))))

(fn ConstructionScript)

(fn ChooseRandomInactivePoint
  (bind _output_get (LocalVariables|SetChoice (.OutItem (Utilities|Array|Random (Variables|Default|GetPoints)))))
  (while (not (Variables|/Game/Design/LevelObjectives/BP_BasePoint.BP_BasePoint_C|GetIsActive _output_get))
    (LocalVariables|SetChoice (.OutItem (Utilities|Array|Random (Variables|Default|GetPoints))))
    ;[0.15 0.15 0.15 0.5] Too deep, give up
    (bind _result (Math|Integer|IncrementInt (LocalVariables|GetIterations))
      (:%20%20
        (if (> _result 20)
          (return (LocalVariables|GetChoice))))))
  (return (LocalVariables|GetChoice)))