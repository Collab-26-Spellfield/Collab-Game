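; Domination objective that grants one point at a time to players standing on it until its limited point pool runs out.
; Entering players join a queue with parallel due times, and leaving removes both entries.
; A timer targets the front entry's due time; after each grant that player is requeued at the back.
; A material Fill parameter tracks remaining points, and the objective deactivates when none remain.
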(event Custom|SetTimer
  ;[0.15 0.15 0.15 0.5] Start timer if there are players in the points queue
  (if (Utilities|Array|IsNotEmpty (Variables|Default|GetPointsQueue))
    (if (<= (- (Utilities|Array|Get(acopy) (Variables|Default|GetTimeToGivePoints)) (Utilities|Time|GetTimeSeconds)) 0.0)
      (CallFunction|GrantPoint)
      (else
        (Utilities|Time|SetTimerbyEvent (EventDispatchers|CreateEvent :!event Custom|Grant%20Point) (- (Utilities|Array|Get(acopy) (Variables|Default|GetTimeToGivePoints)) (Utilities|Time|GetTimeSeconds)))))))

(event Custom|Grant%20Point
  ;[0.15 0.15 0.15 0.5] Give points to the next player in queue and move them to the end of the queue
  (if (Utilities|Array|IsNotEmpty (Variables|Default|GetPointsQueue))
    (Default|CallGrantPoints (Utilities|Array|Get(acopy) (Variables|Default|GetPointsQueue)) 1)
    (Math|Integer|DecrementInt (Variables|Default|GetPointsToDistribute)
      (:%20%20
        (if (> (Variables|Default|GetPointsToDistribute) 0)
          (Utilities|Array|Add (Variables|Default|GetPointsQueue) (Utilities|Array|Get(acopy) (Variables|Default|GetPointsQueue)))
          (Utilities|Array|Add (Variables|Default|GetTimeToGivePoints) (+ (Utilities|Time|GetTimeSeconds) (Variables|Default|GetTimeBetweenPointAssignment)))
          (Utilities|Array|RemoveIndex (Variables|Default|GetPointsQueue))
          (Utilities|Array|RemoveIndex (Variables|Default|GetTimeToGivePoints))
          (CallFunction|SetTimer)
          (Rendering|Material|SetScalarParameterValue (Variables|Default|GetMat) "Fill" (Math|Conversions|ToFloat(Integer) (Variables|Default|GetPointsToDistribute)) :!class /Script/Engine.MaterialInstanceDynamic)
          (else
            (CallFunction|DeactivatePoint)))))))

(event EventPlayerEntered
  (params (ID :type Integer))
  ;[0.15 0.15 0.15 0.5] Players entering and exiting point
  (Utilities|Array|Add (Variables|Default|GetPointsQueue) ID)
  (Utilities|Array|Add (Variables|Default|GetTimeToGivePoints) (+ (Utilities|Time|GetTimeSeconds) (Variables|Default|GetTimeBetweenPointAssignment)))
  (CallFunction|SetTimer))

(event EventPlayerLeft
  (params (ID :type Integer))
  (bind _pointsqueue (Variables|Default|GetPointsQueue))
  (bind _returnvalue (Utilities|Array|FindItem _pointsqueue ID))
  ;[0.15 0.15 0.15 0.5] Players entering and exiting point
  (Utilities|Array|RemoveIndex (Variables|Default|GetTimeToGivePoints) _returnvalue)
  (Utilities|Array|RemoveIndex (Variables|Default|GetPointsQueue) _returnvalue)
  (CallFunction|SetTimer))

(event EventActivatePoint
  ;[0.15 0.15 0.15 0.5] Activate point, perform check for players already on point and add to queue
  (Utilities|Array|Clear (Variables|Default|GetTimeToGivePoints))
  (Utilities|Array|Clear (Variables|Default|GetPointsQueue))
  (|CallParentFunction)
  (Rendering|Material|SetScalarParameterValue (Variables|Default|GetMat) "Fill" 5.0 :!class /Script/Engine.MaterialInstanceDynamic)
  (Variables|Default|SetPointsToDistribute (Variables|Default|GetMaxPoints)))

(event EventDeactivatePoint
  ;[0.15 0.15 0.15 0.5] Deactivate point and clear queue
  (Utilities|Array|Clear (Variables|Default|GetTimeToGivePoints))
  (Utilities|Array|Clear (Variables|Default|GetPointsQueue))
  (|CallParentFunction)
  (Rendering|Material|SetScalarParameterValue (Variables|Default|GetMat) "Fill" 0.0 :!class /Script/Engine.MaterialInstanceDynamic))

(fn ConstructionScript
  (|CallParentFunction))