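; Level objective spawner that creates collectible actors at random positions around itself and passes on the points they award.
; SpawnCollectible offsets a random unit vector by Radius, fixes the world height, then binds and initializes the spawned actor.
; The collectible's GrantPoints event is relayed through the spawner's own GrantPoints dispatcher with player ID and amount.
; The construction script scales the SpawnRadius component to match Radius.
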(event Custom|SpawnCollectible
  (bind _returnvalue (Math|Random|RandomUnitVector))
  (bind _returnvalue_2 (Transformation|GetActorLocation))
  (bind _radius (Variables|Default|GetRadius))
  (bind _returnvalue_3 (* _returnvalue _radius))
  (bind _returnvalue_4 (+ _returnvalue_3 _returnvalue_2))
  (bind _returnvalue_5 (Game|SpawnActorfromClass (Variables|Default|GetClass) (Math|Transform|MakeTransform (Math|Vector|MakeVector (.x _returnvalue_4) (.y _returnvalue_4) 5e+01) "0, 0, 0" "1.000000,1.000000,1.000000") "Undefined" "MultiplyWithRoot" 0 0))
  (EventDispatchers|BindEventtoGrantPoints _returnvalue_5 (delegate Custom|GrantPointsHandler))
  (Default|Init _returnvalue_5))

(event Custom|GrantPointsHandler
  (params (PlayerID :type Integer) (Points%20to%20Grant :type Integer))
  (Default|CallGrantPoints PlayerID Points%20to%20Grant))

(fn ConstructionScript
  (bind _radius (Variables|Default|GetRadius))
  (bind _returnvalue (* _radius 0.02))
  (|CallParentFunction)
  (Transformation|SetWorldScale3D (Variables|Default|GetSpawnRadius) (Math|Vector|MakeVector _returnvalue _returnvalue _returnvalue)))