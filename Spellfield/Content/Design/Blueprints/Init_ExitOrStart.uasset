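; Init_ExitOrStart is a trigger box that either removes a player from the game or starts the game, based on its Exit flag.
; It reacts only to overlapping actors that implement BPI_Character_And_Controller.
; Exit mode passes the actor's ID to the GameInstance for removal.
; Start mode checks the GameInstance for at least two players, then tells the GameMode to begin through a DoOnce, using interface-style messages.
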(event OnComponentBeginOverlap(Box)
  (params (OverlappedComponent :type Primitive%20Component%20Object%20Reference) (OtherActor :type Actor%20Object%20Reference) (OtherComp :type Primitive%20Component%20Object%20Reference) (OtherBodyIndex :type Integer) (bFromSweep :type Boolean) (SweepResult :type Hit%20Result%20Structure%20%28by%20ref%29))
  (if (Utilities|DoesObjectImplementInterface OtherActor "/Game/Design/Blueprints/Interfaces/BPI_Character_And_Controller.BPI_Character_And_Controller_C")
    (if (Variables|Default|GetExit)
      (bind _id (Class|BPICharacterandController|GetID(Message) OtherActor))
      (Class|BPIPlayerConnectionInfo|RemovePlayerfromGame(Message) (Game|GetGameInstance) _id)
      (else
        (bind _connectedplayercount (Class|BPIPlayerConnectionInfo|GetPlayerCount(Message) (Game|GetGameInstance)))
        (if (>= _connectedplayercount 2)
          (Utilities|FlowControl|DoOnce false
            (:Completed
              (Class|BPIGamemodeRequests|BeginGame(Message) (Game|GetGameMode)))))))))

(fn ConstructionScript)