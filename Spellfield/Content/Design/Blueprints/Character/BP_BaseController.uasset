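; Base player controller that routes each local player's Enhanced Input to gameplay and UI objects as input messages tagged with controller ID and trigger phase.
; Each message reaches all registered listeners plus the top stacked consumer, or the controlled pawn when none exist.
; Input flows only when connected, enabled and past a post-possess load timer; otherwise certain buttons request joining through the game instance.
; Debug keys connect players and move pawns.
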(event Custom|TryToConnect
  (if (and (Variables|Default|GetIsConnectionAllowed) (not (Variables|Default|GetIsConnected)))
    (Class|BPIPlayerConnectionInfo|AddPlayertoGame(Message) (Game|GetGameInstance) (Variables|Default|GetControllerID))))

(event Custom|SetConnected
  (params (IsConnected :type Boolean))
  (bind _output_get (Variables|Default|SetIsConnected IsConnected))
  (if _output_get
    (Utilities|FlowControl|Delay 0.2)
    (Variables|Default|SetInputEnabled true)
    (else
      (Variables|Default|SetInputEnabled false))))

(event Custom|AllowConnection
  (Variables|Default|SetIsConnectionAllowed true))

(event Custom|DisallowConnection
  (Variables|Default|SetIsConnectionAllowed false))

(event Custom|GameLoaded
  (Variables|Default|SetAfterLoad true))

(event Input|EnhancedActionEvents|EnhancedInputActionIA_Attack
  (params (ActionValue :type Float%20%28double-precision%29) (ElapsedSeconds :type Float%20%28double-precision%29) (TriggeredSeconds :type Float%20%28double-precision%29) (InputAction :type Input%20Action%20Object%20Reference :default "/Game/Design/Inputs/IA_Attack.IA_Attack"))
  (:Triggered
    (bind _type (Utilities|InputTypetoEnum :!label _label)
      (:Out
        (if (CallFunction|ShouldProcessInput)
          (if (> ActionValue 0.5)
            (Variables|Default|SetAttack%20Bool true)
            (else
              (Variables|Default|SetAttack%20Bool false)))
          (bind _array_element (Utilities|IterateOverListeners)
            (:Loop%20Body
              (Class|BPIControls|AttackInput(Message) _array_element _type (Variables|Default|GetControllerID) (Variables|Default|GetAttack%20Bool) ElapsedSeconds TriggeredSeconds InputAction)))
          (else
            (CallFunction|TrytoConnect))))))
  (:Started
    (goto _label Started))
  (:Ongoing
    (goto _label Ongoing))
  (:Canceled
    (goto _label Cancelled))
  (:Completed
    (goto _label Completed)))

(event Input|EnhancedActionEvents|EnhancedInputActionIA_Look
  (params (ActionValue :type Vector%202D%20Structure) (ElapsedSeconds :type Float%20%28double-precision%29) (TriggeredSeconds :type Float%20%28double-precision%29) (InputAction :type Input%20Action%20Object%20Reference :default "/Game/Design/Inputs/IA_Look.IA_Look"))
  (:Triggered
    (bind _type (Utilities|InputTypetoEnum :!label _label)
      (:Out
        (if (CallFunction|ShouldProcessInput)
          (bind _array_element (Utilities|IterateOverListeners)
            (:Loop%20Body
              (Class|BPIControls|LookInput(Message) _array_element _type (Variables|Default|GetControllerID) (.x ActionValue) (.y ActionValue) ElapsedSeconds TriggeredSeconds InputAction)))))))
  (:Started
    (goto _label Started))
  (:Ongoing
    (goto _label Ongoing))
  (:Canceled
    (goto _label Cancelled))
  (:Completed
    (goto _label Completed)))

(event Input|EnhancedActionEvents|EnhancedInputActionIA_Pause
  (params (ActionValue :type Boolean) (ElapsedSeconds :type Float%20%28double-precision%29) (TriggeredSeconds :type Float%20%28double-precision%29) (InputAction :type Input%20Action%20Object%20Reference :default "/Game/Design/Inputs/IA_Pause.IA_Pause"))
  (:Triggered
    (bind _type (Utilities|InputTypetoEnum :!label _label)
      (:Out
        (if (CallFunction|ShouldProcessInput)
          (bind _array_element (Utilities|IterateOverListeners)
            (:Loop%20Body
              (Class|BPIControls|PauseInput(Message) _array_element _type (Variables|Default|GetControllerID) ActionValue ElapsedSeconds TriggeredSeconds InputAction)))
          (else
            (CallFunction|TrytoConnect))))))
  (:Started
    (goto _label Started))
  (:Ongoing
    (goto _label Ongoing))
  (:Canceled
    (goto _label Cancelled))
  (:Completed
    (goto _label Completed)))

(event Input|EnhancedActionEvents|EnhancedInputActionIA_ChangeHat
  (params (ActionValue :type Boolean) (ElapsedSeconds :type Float%20%28double-precision%29) (TriggeredSeconds :type Float%20%28double-precision%29) (InputAction :type Input%20Action%20Object%20Reference :default "/Game/Design/Inputs/IA_ChangeHat.IA_ChangeHat"))
  (:Triggered
    (bind _type (Utilities|InputTypetoEnum :!label _label)
      (:Out
        (if (CallFunction|ShouldProcessInput)
          (bind _array_element (Utilities|IterateOverListeners)
            (:Loop%20Body
              (Class|BPIControls|ChangeHatInput(Message) _array_element _type (Variables|Default|GetControllerID) ActionValue ElapsedSeconds TriggeredSeconds InputAction)))
          (else
            (CallFunction|TrytoConnect))))))
  (:Started
    (goto _label Started))
  (:Ongoing
    (goto _label Ongoing))
  (:Canceled
    (goto _label Cancelled))
  (:Completed
    (goto _label Completed)))

(event Input|EnhancedActionEvents|EnhancedInputActionIA_ChangeMask
  (params (ActionValue :type Boolean) (ElapsedSeconds :type Float%20%28double-precision%29) (TriggeredSeconds :type Float%20%28double-precision%29) (InputAction :type Input%20Action%20Object%20Reference :default "/Game/Design/Inputs/IA_ChangeMask.IA_ChangeMask"))
  (:Triggered
    (Utilities|InputTypetoEnum :!label _label
      (:Out
        (if (CallFunction|ShouldProcessInput)
          (bind _array_element (Utilities|IterateOverListeners)
            (:Loop%20Body
              (Class|BPIControls|ChangeMaskInput(Message) _array_element "NewEnumerator0" (Variables|Default|GetControllerID) ActionValue ElapsedSeconds TriggeredSeconds InputAction)))
          (else
            (CallFunction|TrytoConnect))))))
  (:Started
    (goto _label Started))
  (:Ongoing
    (goto _label Ongoing))
  (:Canceled
    (goto _label Cancelled))
  (:Completed
    (goto _label Completed)))

(event Input|EnhancedActionEvents|EnhancedInputActionIA_ChangeStaff
  (params (ActionValue :type Boolean) (ElapsedSeconds :type Float%20%28double-precision%29) (TriggeredSeconds :type Float%20%28double-precision%29) (InputAction :type Input%20Action%20Object%20Reference :default "/Game/Design/Inputs/IA_ChangeStaff.IA_ChangeStaff"))
  (:Triggered
    (bind _type (Utilities|InputTypetoEnum :!label _label)
      (:Out
        (if (CallFunction|ShouldProcessInput)
          (bind _array_element (Utilities|IterateOverListeners)
            (:Loop%20Body
              (Class|BPIControls|ChangeStaffInput(Message) _array_element _type (Variables|Default|GetControllerID) ActionValue ElapsedSeconds TriggeredSeconds InputAction)))
          (else
            (CallFunction|TrytoConnect))))))
  (:Started
    (goto _label Started))
  (:Ongoing
    (goto _label Ongoing))
  (:Canceled
    (goto _label Cancelled))
  (:Completed
    (goto _label Completed)))

(event Input|EnhancedActionEvents|EnhancedInputActionIA_EmoteHappy
  (params (ActionValue :type Boolean) (ElapsedSeconds :type Float%20%28double-precision%29) (TriggeredSeconds :type Float%20%28double-precision%29) (InputAction :type Input%20Action%20Object%20Reference :default "/Game/Design/Inputs/IA_EmoteHappy.IA_EmoteHappy"))
  (:Triggered
    (bind _type (Utilities|InputTypetoEnum :!label _label)
      (:Out
        (if (CallFunction|ShouldProcessInput)
          (bind _array_element (Utilities|IterateOverListeners)
            (:Loop%20Body
              (Class|BPIControls|EmoteHappyInput(Message) _array_element _type (Variables|Default|GetControllerID) ActionValue ElapsedSeconds TriggeredSeconds InputAction)))))))
  (:Started
    (goto _label Started))
  (:Ongoing
    (goto _label Ongoing))
  (:Canceled
    (goto _label Cancelled))
  (:Completed
    (goto _label Completed)))

(event Input|EnhancedActionEvents|EnhancedInputActionIA_EmoteAngry
  (params (ActionValue :type Boolean) (ElapsedSeconds :type Float%20%28double-precision%29) (TriggeredSeconds :type Float%20%28double-precision%29) (InputAction :type Input%20Action%20Object%20Reference :default "/Game/Design/Inputs/IA_EmoteAngry.IA_EmoteAngry"))
  (:Triggered
    (bind _type (Utilities|InputTypetoEnum :!label _label)
      (:Out
        (if (CallFunction|ShouldProcessInput)
          (bind _array_element (Utilities|IterateOverListeners)
            (:Loop%20Body
              (Class|BPIControls|EmoteAngryInput(Message) _array_element _type (Variables|Default|GetControllerID) ActionValue ElapsedSeconds TriggeredSeconds InputAction)))))))
  (:Started
    (goto _label Started))
  (:Ongoing
    (goto _label Ongoing))
  (:Canceled
    (goto _label Cancelled))
  (:Completed
    (goto _label Completed)))

(event Input|EnhancedActionEvents|EnhancedInputActionIA_EmoteSad
  (params (ActionValue :type Boolean) (ElapsedSeconds :type Float%20%28double-precision%29) (TriggeredSeconds :type Float%20%28double-precision%29) (InputAction :type Input%20Action%20Object%20Reference :default "/Game/Design/Inputs/IA_EmoteSad.IA_EmoteSad"))
  (:Triggered
    (bind _type (Utilities|InputTypetoEnum :!label _label)
      (:Out
        (if (CallFunction|ShouldProcessInput)
          (bind _array_element (Utilities|IterateOverListeners)
            (:Loop%20Body
              (Class|BPIControls|EmoteSadInput(Message) _array_element _type (Variables|Default|GetControllerID) ActionValue ElapsedSeconds TriggeredSeconds InputAction)))))))
  (:Started
    (goto _label Started))
  (:Ongoing
    (goto _label Ongoing))
  (:Canceled
    (goto _label Cancelled))
  (:Completed
    (goto _label Completed)))

(event Input|EnhancedActionEvents|EnhancedInputActionIA_Movement
  (params (ActionValue :type Vector%202D%20Structure) (ElapsedSeconds :type Float%20%28double-precision%29) (TriggeredSeconds :type Float%20%28double-precision%29) (InputAction :type Input%20Action%20Object%20Reference :default "/Game/Design/Inputs/IA_Movement.IA_Movement"))
  (:Triggered
    (bind _type (Utilities|InputTypetoEnum :!label _label)
      (:Out
        (if (CallFunction|ShouldProcessInput)
          (bind _array_element (Utilities|IterateOverListeners)
            (:Loop%20Body
              (Class|BPIControls|MovementInput(Message) _array_element _type (Variables|Default|GetControllerID) (.x ActionValue) (.y ActionValue) ElapsedSeconds TriggeredSeconds InputAction)))))))
  (:Started
    (goto _label Started))
  (:Ongoing
    (goto _label Ongoing))
  (:Canceled
    (goto _label Cancelled))
  (:Completed
    (goto _label Completed)))

(event Input|EnhancedActionEvents|EnhancedInputActionIA_Dash
  (params (ActionValue :type Boolean) (ElapsedSeconds :type Float%20%28double-precision%29) (TriggeredSeconds :type Float%20%28double-precision%29) (InputAction :type Input%20Action%20Object%20Reference :default "/Game/Design/Inputs/IA_Dash.IA_Dash"))
  (:Triggered
    (bind _type (Utilities|InputTypetoEnum :!label _label)
      (:Out
        (if (CallFunction|ShouldProcessInput)
          (bind _array_element (Utilities|IterateOverListeners)
            (:Loop%20Body
              (Class|BPIControls|DashInput(Message) _array_element _type (Variables|Default|GetControllerID) ActionValue ElapsedSeconds TriggeredSeconds InputAction)))
          (else
            (CallFunction|TrytoConnect))))))
  (:Started
    (goto _label Started))
  (:Ongoing
    (goto _label Ongoing))
  (:Canceled
    (goto _label Cancelled))
  (:Completed
    (goto _label Completed)))

(event Input|EnhancedActionEvents|EnhancedInputActionIA_Block
  (params (ActionValue :type Float%20%28double-precision%29) (ElapsedSeconds :type Float%20%28double-precision%29) (TriggeredSeconds :type Float%20%28double-precision%29) (InputAction :type Input%20Action%20Object%20Reference :default "/Game/Design/Inputs/IA_Block.IA_Block"))
  (:Triggered
    (bind _type (Utilities|InputTypetoEnum :!label _label)
      (:Out
        (if (CallFunction|ShouldProcessInput)
          (if (> ActionValue 0.5)
            (Variables|Default|SetBlock%20Bool true)
            (else
              (Variables|Default|SetBlock%20Bool false)))
          (bind _array_element (Utilities|IterateOverListeners)
            (:Loop%20Body
              (Class|BPIControls|BlockInput(Message) _array_element _type (Variables|Default|GetControllerID) (Variables|Default|GetBlock%20Bool) ElapsedSeconds TriggeredSeconds InputAction)))
          (else
            (CallFunction|TrytoConnect))))))
  (:Started
    (goto _label Started))
  (:Ongoing
    (goto _label Ongoing))
  (:Canceled
    (goto _label Cancelled))
  (:Completed
    (goto _label Completed)))

(event Input|EnhancedActionEvents|EnhancedInputActionIA_UIMovement
  (params (ActionValue :type Vector%202D%20Structure) (ElapsedSeconds :type Float%20%28double-precision%29) (TriggeredSeconds :type Float%20%28double-precision%29) (InputAction :type Input%20Action%20Object%20Reference :default "/Game/Design/Inputs/IA_UIMovement.IA_UIMovement"))
  (:Triggered
    (bind _type (Utilities|InputTypetoEnum :!label _label)
      (:Out
        (if (CallFunction|ShouldProcessInput)
          (bind _array_element (Utilities|IterateOverListeners)
            (:Loop%20Body
              (Class|BPIControls|UIMovementInput(Message) _array_element _type (Variables|Default|GetControllerID) (.x ActionValue) (.y ActionValue) ElapsedSeconds TriggeredSeconds InputAction)))))))
  (:Started
    (goto _label Started))
  (:Ongoing
    (goto _label Ongoing))
  (:Canceled
    (goto _label Cancelled))
  (:Completed
    (goto _label Completed)))

(event Input|EnhancedActionEvents|EnhancedInputActionIA_Confirm
  (params (ActionValue :type Boolean) (ElapsedSeconds :type Float%20%28double-precision%29) (TriggeredSeconds :type Float%20%28double-precision%29) (InputAction :type Input%20Action%20Object%20Reference :default "/Game/Design/Inputs/IA_Confirm.IA_Confirm"))
  (:Triggered
    (bind _type (Utilities|InputTypetoEnum :!label _label)
      (:Out
        (if (CallFunction|ShouldProcessInput)
          (bind _array_element (Utilities|IterateOverListeners)
            (:Loop%20Body
              (Class|BPIControls|ConfirmInput(Message) _array_element _type (Variables|Default|GetControllerID) ActionValue ElapsedSeconds TriggeredSeconds InputAction)))))))
  (:Started
    (goto _label Started))
  (:Ongoing
    (goto _label Ongoing))
  (:Canceled
    (goto _label Cancelled))
  (:Completed
    (goto _label Completed)))

(event Input|EnhancedActionEvents|EnhancedInputActionIA_Back
  (params (ActionValue :type Boolean) (ElapsedSeconds :type Float%20%28double-precision%29) (TriggeredSeconds :type Float%20%28double-precision%29) (InputAction :type Input%20Action%20Object%20Reference :default "/Game/Design/Inputs/IA_Back.IA_Back"))
  (:Triggered
    (bind _type (Utilities|InputTypetoEnum :!label _label)
      (:Out
        (if (CallFunction|ShouldProcessInput)
          (bind _array_element (Utilities|IterateOverListeners)
            (:Loop%20Body
              (Class|BPIControls|BackInput(Message) _array_element _type (Variables|Default|GetControllerID) ActionValue ElapsedSeconds TriggeredSeconds InputAction)))))))
  (:Started
    (goto _label Started))
  (:Ongoing
    (goto _label Ongoing))
  (:Canceled
    (goto _label Cancelled))
  (:Completed
    (goto _label Completed)))

(event EventRemoveConsumer
  (params (Consumer :type Object%20Object%20Reference))
  (Utilities|Array|RemoveItem (Variables|Default|GetInputConsumers) Consumer))

(event EventPossess
  (params (PossessedPawn :type Pawn%20Object%20Reference))
  (bind _returnvalue (PlayerController|LocalPlayerSubsystems|GetEnhancedInputLocalPlayerSubsystem))
  (Utilities|IsValid _returnvalue
    (:Is%20Valid
      (Input|AddMappingContext _returnvalue "/Game/Design/Inputs/IMC_PlayerBase.IMC_PlayerBase" 0 "(bIgnoreAllPressedKeysUntilRelease=True,bForceImmediately=False,bNotifyUserSettings=False)")
      (Utilities|Time|SetTimerbyEvent (delegate Custom|GameLoaded) 3.0))))

(event EventRegisterConsumer
  (params (Consumer :type Object%20Object%20Reference))
  (Utilities|Array|Add (Variables|Default|GetInputConsumers) Consumer))

(event EventRegisterListener
  (params (Listener :type Object%20Object%20Reference))
  (Utilities|Array|Add (Variables|Default|GetInputListeners) Listener))

(event EventRemoveListener
  (params (Listener :type Object%20Object%20Reference))
  (Utilities|Array|RemoveItem (Variables|Default|GetInputListeners) Listener))

(event Input|KeyboardEvents|DebugKey6
  (params (Key :type Key%20Structure :default "None") (ActionValue :type Input%20Action%20Value%20Structure))
  (:Pressed
    (bind _playerconnectiondata (Class|BPIPlayerConnectionInfo|GetPlayerData(Message) (Game|GetGameInstance)))
    (bind _valuepin (Utilities|Map|ForEachLoop(Map) _playerconnectiondata)
      (:then
        (Transformation|SetActorLocation (.playerpawn _valuepin) "-700.000000,900.000000,100.000000" false false)))))

(event Input|KeyboardEvents|DebugKey7
  (params (Key :type Key%20Structure :default "None") (ActionValue :type Input%20Action%20Value%20Structure))
  (:Pressed
    (bind _playerconnectiondata (Class|BPIPlayerConnectionInfo|GetPlayerData(Message) (Game|GetGameInstance)))
    (bind _valuepin (Utilities|Map|ForEachLoop(Map) _playerconnectiondata)
      (:then
        (Transformation|SetActorLocation (.playerpawn _valuepin) "400.000000,900.000000,100.000000" false false)))))

(event Input|KeyboardEvents|DebugKey1
  (params (Key :type Key%20Structure :default "None") (ActionValue :type Input%20Action%20Value%20Structure))
  (:Pressed
    (CallFunction|TrytoConnect)))

(event Input|KeyboardEvents|DebugKey2
  (params (Key :type Key%20Structure :default "None") (ActionValue :type Input%20Action%20Value%20Structure))
  (:Pressed
    (bind _playerconnectiondata (Class|BPIPlayerConnectionInfo|GetAllPlayerData(Message) (Game|GetGameInstance)))
    (CallFunction|TrytoConnect (.playercontroller (.Value (Utilities|Map|Find _playerconnectiondata 1))))))

(event Input|KeyboardEvents|DebugKey3
  (params (Key :type Key%20Structure :default "None") (ActionValue :type Input%20Action%20Value%20Structure))
  (:Pressed
    (bind _playerconnectiondata (Class|BPIPlayerConnectionInfo|GetAllPlayerData(Message) (Game|GetGameInstance)))
    (CallFunction|TrytoConnect (.playercontroller (.Value (Utilities|Map|Find _playerconnectiondata 2))))))

(event Input|KeyboardEvents|DebugKey4
  (params (Key :type Key%20Structure :default "None") (ActionValue :type Input%20Action%20Value%20Structure))
  (:Pressed
    (bind _playerconnectiondata (Class|BPIPlayerConnectionInfo|GetAllPlayerData(Message) (Game|GetGameInstance)))
    (CallFunction|TrytoConnect (.playercontroller (.Value (Utilities|Map|Find _playerconnectiondata 3))))))

(fn ConstructionScript)

(fn GetSoleConsumer
  ;[0.15 0.15 0.15 0.5] Consumers on the stack do not let lower consumers recieve input (they consume it). If no consumers are on the stack, send the input to the player.
  (bind _output (CallFunction|GetConsumers))
  (if (Utilities|Array|IsEmpty _output)
    (return (Pawn|GetControlledPawn))
    (else
      (return (Utilities|Array|Get(acopy) _output (Utilities|Array|LastIndex _output))))))

(fn GetListeners
  ;[0.15 0.15 0.15 0.5] Check all listeners are still valid
  (for _array_element (Variables|Default|GetInputListeners)
    (Utilities|IsValid _array_element
      (:Is%20Valid
        (Utilities|Array|Add (LocalVariables|GetValidListeners) _array_element))))
  (bind _output_get (Variables|Default|SetInputListeners (LocalVariables|GetValidListeners)))
  (return _output_get))

(fn GetConsumers
  ;[0.15 0.15 0.15 0.5] Check all consumers are still valid
  (for _array_element (Variables|Default|GetInputConsumers)
    (Utilities|IsValid _array_element
      (:Is%20Valid
        (Utilities|Array|Add (LocalVariables|GetValidConsumers) _array_element))))
  (bind _output_get (Variables|Default|SetInputConsumers (LocalVariables|GetValidConsumers)))
  (return _output_get))

(fn ShouldProcessInput
  (return (Math|Boolean|ANDBoolean (Variables|Default|GetIsConnected) (Variables|Default|GetInputEnabled) (Variables|Default|GetAfterLoad))))

(fn GetID
  (return (Variables|Default|GetControllerID)))

(fn GetPlayer
  (bind _player (Class|BPICharacterandController|GetPlayer(Message) (Pawn|GetControlledPawn)))
  (return _player))

(fn GetPlayerController
  (return self))