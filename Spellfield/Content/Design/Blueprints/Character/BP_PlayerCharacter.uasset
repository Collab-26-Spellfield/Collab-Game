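; Player character with twin-stick movement and aim, dash, attack and block, plus death and respawn.
; BeginPlay registers with the game instance, initialises the attack component and binds health and respawn events.
; Input delegates combat to the attack component; dash line-traces to stop at obstacles, then lerps position on a timeline with cooldown and brief immunity.
; Death disables input and respawns at a random BP_RespawnPad, restoring control and health after a delay.
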(event Custom|Player%20Death
  ;[0.15 0.05938 0.07814 0.5] die
  (if (not (Variables|Default|GetIsDead))
    (Development|PrintString (Utilities|String|Append (Utilities|GetObjectName self) " has died") true true "(R=1.000000,G=0.000000,B=0.035798,A=1.000000)")
    (Input|DisableInput 0)
    (Default|CallRespawn)
    (Variables|Default|SetIsDead true)))

(event Custom|Respawn1
  (Transformation|SetWorldLocation (Variables|Collision|GetCapsuleComponent self) (Transformation|GetWorldLocation (Variables|/Game/Tech/Blueprints/BP_RespawnPad.BP_RespawnPad_C|GetBox (.OutItem (Utilities|Array|Random (Variables|Default|GetRespawnPoints))))) false false)
  (Rendering|Material|SetMaterial (Variables|Character|GetMesh) 0 "/Game/Tech/Temp_material/RespawnMaterial.RespawnMaterial")
  (Utilities|Time|SetTimerbyEvent (delegate Custom|Re-enable) 5.0))

(event Custom|Re-enable
  (bind _bp_healthcomponent (Variables|Default|GetBP_HealthComponent))
  (Input|EnableInput 0)
  (Variables|/Game/Tech/Blueprints/BP_HealthComponent.BP_HealthComponent_C|SetCurrentHealth _bp_healthcomponent (Variables|/Game/Tech/Blueprints/BP_HealthComponent.BP_HealthComponent_C|GetMaxHealth _bp_healthcomponent))
  (Rendering|Material|SetMaterial (Variables|Character|GetMesh) 0 "/Game/Art/Character/fixed_hat/default_004.default_004")
  (Variables|Default|SetIsDead false))

(event EventBeginPlay
  (bind _self self)
  ;[0.15 0.15 0.15 0.5] init components
  ;[0.3438 0 0.02987 0.5] DO NOT REMOVE
  (Utilities|FlowControl|DelayUntilNextTick)
  (Class|BPICharacterandController|InitialiseCharacter(Message) (Game|GetGameInstance) _self)
  (bind _asbp_base_controller (Utilities|Casting|CastToBP_BaseController (Pawn|GetController _self)))
  (Variables|Default|SetMy%20ID (Variables|/Game/Design/Blueprints/Character/BP_BaseController.BP_BaseController_C|GetControllerID _asbp_base_controller))
  (Default|Init (Variables|Default|GetBP_AttackComponent) (Variables|Default|GetBP_KnockbackComponent) (Variables|Default|GetFirepoint) self (Variables|Default|GetMovespeed))
  (EventDispatchers|BindEventtoDie (Variables|Default|GetBP_HealthComponent) (delegate Custom|Player%20Death))
  (bind _outactors (Actor|GetAllActorsOfClass "/Game/Tech/Blueprints/BP_RespawnPad.BP_RespawnPad_C"))
  (Variables|Default|SetRespawnPoints _outactors)
  (EventDispatchers|BindEventtoRespawn (delegate Custom|Respawn1))
  (Development|PrintString (Utilities|String|ToString(Integer) (Variables|Default|GetMy%20ID)))
  (bind _aswbp_debug_charge_display (Utilities|Casting|CastToWBP_DebugChargeDisplay (UserInterface|GetWidget (Variables|Default|GetCharges))))
  (Variables|Default|SetChargeDisplay _aswbp_debug_charge_display)
  (bind _aswbp_debug_healthbar (Utilities|Casting|CastToWBP_DebugHealthbar (UserInterface|GetWidget (Variables|Default|GetHealth%20Bar))))
  (Default|Init _aswbp_debug_healthbar self))

(event EventInitialiseCharacter
  (params (PlayerRef :type BP%20Player%20Character%20Object%20Reference))
  ;[0.15 0.15 0.15 0.5] INITIALISE
)

(event Custom|de-immune
  ;[0.15 0.15 0.15 0.5] Dash
  (Variables|/Game/Tech/Blueprints/BP_HealthComponent.BP_HealthComponent_C|SetImmune (Variables|Default|GetBP_HealthComponent) false))

(event Custom|Reset%20Dash
  ;[0.15 0.15 0.15 0.5] Dash
  (Variables|DashVariables|SetCan%20Dash true))

(event Custom|Dash
  (params (Dash%20Direction :type Vector) (Dash%20End%20Position :type Vector))
  ;[0.15 0.15 0.15 0.5] Dash
  (Variables|DashVariables|SetDash%20Start%20Location (Transformation|GetActorLocation))
  (Components|Timeline|SetPlayRate (Variables|Default|GetDash%20Timeline) (/ 1.0 (Variables|Default|GetDash%20Time)))
  (bind _newtrack_0 (Timeline|Dash%20Timeline PlayFromStart)
    (:Update
      (Transformation|SetActorLocation (Math|Vector|Lerp(Vector) (Variables|DashVariables|GetDash%20Start%20Location) Dash%20End%20Position (Math|Float|Clamp(Float) (* _newtrack_0 (/ (Variables|DashVariables|GetDash%20Distance) (Math|Vector|Distance(Vector) (Variables|DashVariables|GetDash%20Start%20Location) Dash%20End%20Position))))) false false)
      (Variables|/Game/Tech/Blueprints/BP_HealthComponent.BP_HealthComponent_C|SetImmune (Variables|Default|GetBP_HealthComponent) false))))

(event Input|EnhancedActionEvents|EnhancedInputActionIA_Attack
  (params (ActionValue :type Boolean) (ElapsedSeconds :type Float%20%28double-precision%29) (TriggeredSeconds :type Float%20%28double-precision%29) (InputAction :type Input%20Action%20Object%20Reference :default "/Game/Design/Inputs/IA_Attack.IA_Attack"))
  ;[0.15 0.15 0.15 0.5] Attack
  (Default|Attack (Variables|Default|GetBP_AttackComponent)))

(event Input|EnhancedActionEvents|EnhancedInputActionIA_Look
  (params (ActionValue :type Vector%202D%20Structure) (ElapsedSeconds :type Float%20%28double-precision%29) (TriggeredSeconds :type Float%20%28double-precision%29) (InputAction :type Input%20Action%20Object%20Reference :default "/Game/Design/Inputs/IA_Look.IA_Look"))
  ;[0.15 0.15 0.15 0.5] Right Stick Look Rotation
  (:Triggered
    (Variables|Default|SetIs%20Using%20Right%20Stick true)
    (Transformation|SetWorldRotation (Variables|Character|GetMesh) (Math|Interpolation|RInterpTo (Transformation|GetWorldRotation (Variables|Character|GetMesh)) (Math|Rotator|MakeRotfromX (Math|Vector|MakeVector (.x ActionValue) (.y ActionValue) 0.0)) (Utilities|Time|GetWorldDeltaSeconds) 15.0) false false)
    (Transformation|SetWorldRotation (Variables|Default|GetAimArrowPivot) (Math|Rotator|MakeRotfromX (Math|Vector|MakeVector (.x ActionValue) (.y ActionValue) 0.0)) false false))
  (:Canceled
    (Variables|Default|SetIs%20Using%20Right%20Stick false :!label _label))
  (:Completed
    (goto _label)))

(event Input|EnhancedActionEvents|EnhancedInputActionIA_Dash
  (params (ActionValue :type Boolean) (ElapsedSeconds :type Float%20%28double-precision%29) (TriggeredSeconds :type Float%20%28double-precision%29) (InputAction :type Input%20Action%20Object%20Reference :default "/Game/Design/Inputs/IA_Dash.IA_Dash"))
  ;[0.15 0.15 0.15 0.5] Dash
  (:Started
    (if (Variables|DashVariables|GetCan%20Dash)
      (Variables|DashVariables|SetCan%20Dash false)
      (CallFunction|DashLineTrace (select (Class|AIBlueprintHelperLibrary|IsValidAIDirection (Pawn|Components|PawnMovement|GetLastInputVector (Variables|Character|GetCharacterMovement))) (Pawn|Components|PawnMovement|GetLastInputVector (Variables|Character|GetCharacterMovement)) (Math|Vector|GetForwardVector (Variables|Default|GetAimDirectionArrow))))
      (Utilities|Time|SetTimerbyEvent (delegate Custom|Reset%20Dash) 2.0)
      (Default|StartDashCooldown (Variables|Default|GetChargeDisplay) 2.0)
      (Variables|/Game/Tech/Blueprints/BP_HealthComponent.BP_HealthComponent_C|SetImmune (Variables|Default|GetBP_HealthComponent) true)
      (Utilities|Time|SetTimerbyEvent (delegate Custom|de-immune) (Variables|Default|GetDash%20Time)))))

(event Input|EnhancedActionEvents|EnhancedInputActionIA_Charge
  (params (ActionValue :type Boolean) (ElapsedSeconds :type Float%20%28double-precision%29) (TriggeredSeconds :type Float%20%28double-precision%29) (InputAction :type Input%20Action%20Object%20Reference :default "/Game/Design/Inputs/IA_Charge.IA_Charge"))
  ;[0.15 0.15 0.15 0.5] Attack
  (Default|ChargingState (Variables|Default|GetBP_AttackComponent) TriggeredSeconds))

(event Input|EnhancedActionEvents|EnhancedInputActionIA_Block
  (params (ActionValue :type Boolean) (ElapsedSeconds :type Float%20%28double-precision%29) (TriggeredSeconds :type Float%20%28double-precision%29) (InputAction :type Input%20Action%20Object%20Reference :default "/Game/Design/Inputs/IA_Block.IA_Block"))
  ;[0.15 0.15 0.15 0.5] Block
  (:Started
    (Default|Block (Variables|Default|GetBP_AttackComponent))
    (Utilities|FlowControl|Delay 0.1)
    (Collision|SetCollisionEnabled (Variables|Default|GetBlockRadius) "NoCollision")
    (Rendering|SetVisibility (Variables|Default|GetBlockDebug) false false)))

(event Input|EnhancedActionEvents|EnhancedInputActionIA_Movement
  (params (ActionValue :type Vector%202D%20Structure) (ElapsedSeconds :type Float%20%28double-precision%29) (TriggeredSeconds :type Float%20%28double-precision%29) (InputAction :type Input%20Action%20Object%20Reference :default "/Game/Design/Inputs/IA_Movement.IA_Movement"))
  (bind _movespeed (Variables|Default|GetMovespeed))
  (bind _returnvalue (* (.y ActionValue) _movespeed))
  (bind _returnvalue_2 (* (.x ActionValue) _movespeed))
  ;[0.15 0.15 0.15 0.5] Player Movement
  ;;[0.15 0.15 0.15 0.5] Move U/D
  (Pawn|Input|AddMovementInput (Math|Vector|GetForwardVector (Math|Rotator|MakeRotator 0.0 0.0 (.yaw (Pawn|GetControlRotation (Pawn|GetController) :!class /Script/Engine.Controller)))) (* _returnvalue -1.0) false)
  ;;[0.15 0.15 0.15 0.5] Move L/R
  (Pawn|Input|AddMovementInput (Math|Vector|GetRightVector (Math|Rotator|MakeRotator 0.0 0.0 (.yaw (Pawn|GetControlRotation (Pawn|GetController) :!class /Script/Engine.Controller)))) (* _returnvalue_2 -1.0) false)
  ;;[0.15 0.15 0.15 0.5] Set Mesh Rotation
  (if (not (Variables|Default|GetIs%20Using%20Right%20Stick))
    (Transformation|SetWorldRotation (Variables|Character|GetMesh) (Math|Interpolation|RInterpTo (Transformation|GetWorldRotation (Variables|Character|GetMesh)) (Math|Rotator|MakeRotfromX (Math|Vector|MakeVector (* _returnvalue_2 1.0) (* _returnvalue -1.0) 0.0)) (Utilities|Time|GetWorldDeltaSeconds) 22.0) false false)
    (Transformation|SetWorldRotation (Variables|Default|GetAimArrowPivot) (Math|Rotator|MakeRotfromX (Math|Vector|MakeVector (* _returnvalue_2 1.0) (* _returnvalue -1.0) 0.0)) false false)))

(fn ConstructionScript)

(fn DashLineTrace
  (params (Dash%20Direction :type Vector))
  (bind _returnvalue (Transformation|GetActorLocation))
  (bind _charactermovement (Variables|Character|GetCharacterMovement))
  (bind _returnvalue_2 (Pawn|Components|PawnMovement|GetLastInputVector _charactermovement))
  (bind (_outhit _returnvalue_3) (Collision|LineTraceByChannel _returnvalue (+ _returnvalue (* Dash%20Direction (Variables|DashVariables|GetDash%20Distance))) "TraceTypeQuery1" false 0 "None"))
  (if _returnvalue_3
    (CallFunction|Dash _returnvalue_2 (+ (.Location (Collision|BreakHitResult _outhit)) (* Dash%20Direction (Variables|/Script/Engine.CapsuleComponent|GetCapsuleRadius (Variables|Collision|GetCapsuleComponent)) -1.0)))
    (else
      (CallFunction|Dash _returnvalue_2 (.TraceEnd (Collision|BreakHitResult _outhit))))))