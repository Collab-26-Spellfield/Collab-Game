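; Shared player-identity lookups that map a player ID to one of four themed colour sets and assets.
; Most functions select by ID modulo 4, returning UI-agnostic colours, VFX colours, clothing and box materials, or pole textures.
; A material helper creates a dynamic instance from a base material and sets three shade parameters for that player.
; The icon lookup instead reads the pawn's mask index through the game instance, then picks that player's icon from DT_Masks.
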(fn GetPlayerColour
  (params (Player%20Id :type Integer))
  (return (Utilities|Select :Index (Math|Integer|%(Integer) Player%20Id 4) :Option%200 "(R=0.097587,G=0.381326,B=0.723055,A=1.000000)" :Option%201 "(R=0.775822,G=0.078187,B=0.158961,A=1.000000)" :Option%202 "(R=0.147027,G=0.715694,B=0.039546,A=1.000000)" :Option%203 "(R=0.783538,G=0.396755,B=0.029557,A=1.000000)")))

(fn GetPlayerClothingColour
  (params (Player%20Id :type Integer))
  (return (Utilities|Select :Index (Math|Integer|%(Integer) Player%20Id 4) :Option%200 "/Game/Design/Dev_Textures/DebugCharacterColours/M_Player0.M_Player0" :Option%201 "/Game/Design/Dev_Textures/DebugCharacterColours/M_Player1.M_Player1" :Option%202 "/Game/Design/Dev_Textures/DebugCharacterColours/M_Player2.M_Player2" :Option%203 "/Game/Design/Dev_Textures/DebugCharacterColours/M_Player3.M_Player3")))

(fn GetPlayerVibrantColour
  (params (Player%20Id :type Integer))
  (return (Utilities|Select :Index (Math|Integer|%(Integer) Player%20Id 4) :Option%200 "(R=0.000000,G=0.334914,B=1.000000,A=1.000000)" :Option%201 "(R=1.000000,G=0.000000,B=0.115782,A=1.000000)" :Option%202 "(R=0.158960,G=1.000000,B=0.000000,A=1.000000)" :Option%203 "(R=1.000000,G=0.487012,B=0.000000,A=1.000000)")))

(fn MakePlayerDynamicMaterial
  (params (Player%20Id :type Integer) (Base%20Material :type Material%20Interface%20Object%20Reference))
  (bind _returnvalue (Math|Integer|%(Integer) Player%20Id 4))
  (bind _returnvalue_2 (Rendering|Material|CreateDynamicMaterialInstance (LocalVariables|Get__WorldContext) Base%20Material "None" :!class /Script/Engine.KismetMaterialLibrary))
  (Rendering|Material|SetVectorParameterValue _returnvalue_2 "ColourOption1" (Utilities|Select :Index _returnvalue :Option%200 "(R=0.283149,G=0.783538,B=0.871367,A=1.000000)" :Option%201 "(R=0.854993,G=0.242281,B=0.304987,A=1.000000)" :Option%202 "(R=0.520996,G=0.879623,B=0.177888,A=1.000000)" :Option%203 "(R=0.930111,G=0.854993,B=0.171441,A=1.000000)") :!class /Script/Engine.MaterialInstanceDynamic)
  (Rendering|Material|SetVectorParameterValue _returnvalue_2 "ColourOption2" (Utilities|Select :Index _returnvalue :Option%200 "(R=0.097587,G=0.381326,B=0.723055,A=1.000000)" :Option%201 "(R=0.775822,G=0.078187,B=0.158961,A=1.000000)" :Option%202 "(R=0.147027,G=0.715694,B=0.039546,A=1.000000)" :Option%203 "(R=0.783538,G=0.396755,B=0.029557,A=1.000000)") :!class /Script/Engine.MaterialInstanceDynamic)
  (Rendering|Material|SetVectorParameterValue _returnvalue_2 "ColourOption3" (Utilities|Select :Index _returnvalue :Option%200 "(R=0.034340,G=0.138432,B=0.533277,A=1.000000)" :Option%201 "(R=0.309469,G=0.018500,B=0.152926,A=1.000000)" :Option%202 "(R=0.063010,G=0.462077,B=0.042311,A=1.000000)" :Option%203 "(R=0.679543,G=0.287441,B=0.024158,A=1.000000)") :!class /Script/Engine.MaterialInstanceDynamic)
  (return _returnvalue_2))

(fn GetPlayerBox
  (params (ID :type Integer))
  (return (Utilities|Select :Index (Math|Integer|%(Integer) ID 4) :Option%200 "/Game/UI/Art/Boxes/M_PlayerBox0.M_PlayerBox0" :Option%201 "/Game/UI/Art/Boxes/M_PlayerBox1.M_PlayerBox1" :Option%202 "/Game/UI/Art/Boxes/M_PlayerBox2.M_PlayerBox2" :Option%203 "/Game/UI/Art/Boxes/M_PlayerBox3.M_PlayerBox3")))

(fn GetPlayerPole
  (params (ID :type Integer))
  (return (Utilities|Select :Index (Math|Integer|%(Integer) ID 4) :Option%200 "/Game/UI/Art/Points/T_ROD_blue.T_ROD_blue" :Option%201 "/Game/UI/Art/Points/T_ROD_PINK.T_ROD_PINK" :Option%202 "/Game/UI/Art/Points/T_ROD_GREEN.T_ROD_GREEN" :Option%203 "/Game/UI/Art/Points/T_ROD_YELLOW.T_ROD_YELLOW")))

(fn GetPlayerIcon
  (params (ID :type Integer))
  (bind _playerconnectiondata (Class|BPIPlayerConnectionInfo|GetAllPlayerData(Message) (Game|GetGameInstance (LocalVariables|Get__WorldContext))))
  (bind _outrownames (DataTable|GetDataTableRowNames "/Game/Tech/DT_Masks.DT_Masks"))
  (bind _returnvalue (Utilities|GetDataTableRow "/Game/Tech/DT_Masks.DT_Masks" (Utilities|Array|Get(acopy) _outrownames (Variables|/Game/Tech/Blueprints/BP_CustomizationComponent.BP_CustomizationComponent_C|GetMaskIndex (Variables|/Game/Design/Blueprints/Character/BP_PlayerCharacter.BP_PlayerCharacter_C|GetBP_CustomizationComponent (.playerpawn (.Value (Utilities|Map|Find _playerconnectiondata ID)))))))
    (:then
      (return (Utilities|Array|Get(acopy) (.Icons (Utilities|Struct|BreakS_Masks _returnvalue)) ID)))))

(fn GetPlayerVFXColours
  (params (ID :type Integer))
  (bind _returnvalue (Math|Integer|%(Integer) ID 4))
  (return (Utilities|Select :Index _returnvalue :Option%200 "(R=0.571125,G=0.714762,B=1.000000,A=1.000000)" :Option%201 "(R=1.000000,G=0.571125,B=0.620781,A=1.000000)" :Option%202 "(R=0.639302,G=1.000000,B=0.571125,A=1.000000)" :Option%203 "(R=1.000000,G=0.779994,B=0.571125,A=1.000000)") (Utilities|Select :Index _returnvalue :Option%200 "(R=0.000000,G=0.334917,B=1.000000,A=1.000000)" :Option%201 "(R=1.000000,G=0.000000,B=0.115783,A=1.000000)" :Option%202 "(R=0.158967,G=1.000000,B=0.000000,A=1.000000)" :Option%203 "(R=1.000000,G=0.487017,B=0.000000,A=1.000000)") (Utilities|Select :Index _returnvalue :Option%200 "(R=0.000000,G=0.334917,B=1.000000,A=1.000000)" :Option%201 "(R=1.000000,G=0.000000,B=0.115782,A=1.000000)" :Option%202 "(R=0.158967,G=1.000000,B=0.000000,A=1.000000)" :Option%203 "(R=1.000000,G=0.487017,B=0.000000,A=1.000000)") (Utilities|Select :Index _returnvalue :Option%200 "(R=0.000000,G=0.334917,B=1.000000,A=1.000000)" :Option%201 "(R=1.000000,G=0.000000,B=0.115783,A=1.000000)" :Option%202 "(R=0.158967,G=1.000000,B=0.000000,A=1.000000)" :Option%203 "(R=1.000000,G=0.487017,B=0.000000,A=1.000000)")))