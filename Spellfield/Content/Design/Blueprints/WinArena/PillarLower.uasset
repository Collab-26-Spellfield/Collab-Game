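; PillarLower is a win-arena pillar actor that sinks by a set height shortly after play begins.
; BeginPlay stores the starting location, waits through a fixed delay, then calls the Lower event.
; Lower plays a timeline whose curve lerps the actor's Z from its initial height down by the Height variable.
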(event Custom|Lower
  (bind _initial_height (Variables|Default|GetInitial%20Height))
  (bind _initial_height_2 (Variables|Default|GetInitial%20Height))
  (bind _lower_pillar (Timeline|Lower%20Pillar PlayFromStart)
    (:Update
      (Transformation|SetActorLocation (Math|Vector|MakeVector (.x _initial_height_2) (.y _initial_height_2) (Math|Float|Lerp (.z _initial_height) (- (.z _initial_height) (Variables|Default|GetHeight)) _lower_pillar)) false false))))

(event EventBeginPlay
  (Variables|Default|SetInitial%20Height (Transformation|GetActorLocation))
  (Utilities|FlowControl|Delay 5.0)
  (CallFunction|Lower))

(fn ConstructionScript)