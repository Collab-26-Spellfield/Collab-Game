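; BP_ExplosivePlant is a level hazard that explodes after a short fuse when it takes any damage, then respawns.
; Taking damage reveals a debug radius and starts a timer for the explosion, which sphere-traces nearby objects to apply damage and send knockback messages from its location.
; It then hides the explosive mesh and disables its collision, setting a respawn timer to restore both.
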(event Custom|Explosion
  (bind _returnvalue (Transformation|GetActorLocation))
  ;[0.15 0.15 0.15 0.5] Explosion
  (Rendering|Debug|DrawDebugSphere _returnvalue 4e+02 12 "(R=1.000000,G=1.000000,B=1.000000,A=1.000000)" 1.0 5.0)
  (bind (_outhits _returnvalue_2) (Collision|MultiSphereTraceForObjects _returnvalue _returnvalue 4e+02 (Variables|Default|GetObject%20Types) false 0 "None"))
  (if _returnvalue_2
    (for _array_element _outhits
      (Game|Damage|ApplyDamage (.HitActor (Collision|BreakHitResult _array_element)) 4e+01 0 0)
      (Class|BPIProjectileInterface|DealKnockback(Message) (.HitActor (Collision|BreakHitResult _array_element)) 1e+01 (Transformation|GetActorLocation)))
    (CallFunction|HideExplosive)
    (else
      (CallFunction|HideExplosive))))

(event Custom|Hide%20Explosive
  ;[0.15 0.15 0.15 0.5] Hide explosive
  (Collision|SetCollisionEnabled (Variables|Default|GetSM_PlantBombExplosive) "NoCollision")
  (Development|SetHiddeninGame (Variables|Default|Getdebug%20radius) true false)
  ;;[0.15 0.15 0.15 0.5] Respawn Timer
  (bind _returnvalue (Utilities|Time|SetTimerbyEvent (EventDispatchers|CreateEvent :!event Custom|Show%20Explosive) 5.0))
  (Variables|Default|SetExplosive%20Respawn%20Timer _returnvalue))

(event Custom|Show%20Explosive
  ;[0.15 0.15 0.15 0.5] 'Respawn' Explosive
  (Collision|SetCollisionEnabled (Variables|Default|GetSM_PlantBombExplosive) "QueryAndPhysics")
  (Development|SetHiddeninGame (Variables|Default|GetSM_PlantBombExplosive) false false))

(event Game|Damage|EventAnyDamage
  (params (Damage :type Float%20%28single-precision%29) (DamageType :type Damage%20Type%20Object%20Reference) (InstigatedBy :type Controller%20Object%20Reference) (DamageCauser :type Actor%20Object%20Reference))
  ;[0.15 0.15 0.15 0.5] Debug blast radius
  (Development|SetHiddeninGame (Variables|Default|Getdebug%20radius) false false)
  ;[0.15 0.15 0.15 0.5] Explosion timer
  (Utilities|Time|SetTimerbyEvent (delegate Custom|Explosion) 1.0))

(fn ConstructionScript)