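; Buff crystal spawner that places a crystal actor at its box on BeginPlay and cycles it between available and hidden.
; Overlap by any actor implementing BPI_modifiers hides the crystal's cone and disables that crystal's collision, then a five-second timer restores both.
; The construction script maps buff type to cone color through the crystal reference, which is only assigned at BeginPlay.
; No buff is applied in this Blueprint.
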(event OnComponentBeginOverlap(Box)
  (params (OverlappedComponent :type Primitive%20Component%20Object%20Reference) (OtherActor :type Actor%20Object%20Reference) (OtherComp :type Primitive%20Component%20Object%20Reference) (OtherBodyIndex :type Integer) (bFromSweep :type Boolean) (SweepResult :type Hit%20Result%20Structure%20%28by%20ref%29))
  (if (Utilities|DoesObjectImplementInterface OtherActor "/Game/Tech/Blueprints/Crystals/BPI_modifiers.BPI_modifiers_C")
    (CallFunction|DisableCrystal)
    (Utilities|Time|SetTimerbyEvent (delegate Custom|Rest%20Crystal) 5.0)))

(event Custom|Disable%20Crystal
  (Development|SetHiddeninGame (Variables|/Game/Tech/Blueprints/Crystals/BP_Crystal_Parent.BP_Crystal_Parent_C|GetCone (Variables|Default|Getcrystalobj)) true false)
  (Collision|SetCollisionEnabled (Variables|/Game/Tech/Blueprints/Crystals/BP_Crystal_Parent.BP_Crystal_Parent_C|GetBox (Variables|Default|Getcrystalobj)) "NoCollision"))

(event Custom|Enable%20Crystal
  (Development|SetHiddeninGame (Variables|/Game/Tech/Blueprints/Crystals/BP_Crystal_Parent.BP_Crystal_Parent_C|GetCone (Variables|Default|Getcrystalobj)) false false)
  (Collision|SetCollisionEnabled (Variables|/Game/Tech/Blueprints/Crystals/BP_Crystal_Parent.BP_Crystal_Parent_C|GetBox (Variables|Default|Getcrystalobj)) "QueryAndPhysics"))

(event Custom|Rest%20Crystal
  (CallFunction|EnableCrystal))

(event EventBeginPlay
  (bind _returnvalue (Game|SpawnActorfromClass (Variables|Default|GetCrystal) (Transformation|GetWorldTransform (Variables|Default|GetBox)) "Undefined" "MultiplyWithRoot" 0 0))
  (Variables|Default|Setcrystalobj _returnvalue))

(fn ConstructionScript
  (Rendering|Material|SetMaterial (Variables|/Game/Tech/Blueprints/Crystals/BP_Crystal_Parent.BP_Crystal_Parent_C|GetCone (Variables|Default|Getcrystalobj)) 0 (Utilities|Select :Index "NewEnumerator0" :NewEnumerator0 "/Game/Design/Dev_Textures/DevMat_Yellow.DevMat_Yellow" :NewEnumerator1 "/Game/Design/Dev_Textures/DevMat_Red.DevMat_Red" :NewEnumerator2 "/Game/Design/Dev_Textures/DevMat_Green.DevMat_Green" :NewEnumerator3 "/Game/Design/Dev_Textures/DevMat_Blue.DevMat_Blue")))