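; BP_FlameWall is a level hazard: a fire wall that periodically switches on and off and hurts actors that hit it.
; A looping timer drives a FlipFlop that toggles the wall's visibility and collision together, with collision disabled at BeginPlay.
; On component hit, BPRecentlyHitActorsComponent gates the response, which sends a knockback message to the actor, applies damage and prints a debug string.
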(event OnComponentHit(FireWall)
  (params (HitComponent :type Primitive%20Component%20Object%20Reference) (OtherActor :type Actor%20Object%20Reference) (OtherComp :type Primitive%20Component%20Object%20Reference) (NormalImpulse :type Vector :default "0, 0, 0") (Hit :type Hit%20Result%20Structure%20%28by%20ref%29))
  (bind _should_damage (Default|ActorHit (Variables|Default|GetBP_RecentlyHitActorsComponent) OtherActor))
  (if _should_damage
    ;[0.15 0.15 0.15 0.5] Knockback character here
    (Class|BPIKnockbackInterface|Knockback(Message) OtherActor 1e+01 self)
    (Game|Damage|ApplyDamage OtherActor 1e+01 0 0)
    (Development|PrintString "Hello")))

(event Custom|Wall%20Timer
  (Utilities|Time|SetTimerbyEvent (delegate Custom|Switch%20Wall%20On%20/%20Off) 3.0 true))

(event Custom|Switch%20Wall%20On%20/%20Off
  (bind _fire_wall (Variables|Default|GetFire%20Wall))
  (bind _fire_wall_2 (Variables|Default|GetFire%20Wall))
  (Utilities|FlowControl|FlipFlop
    (:A
      (Development|SetHiddeninGame _fire_wall_2 false false)
      (Collision|SetCollisionEnabled _fire_wall_2 "QueryAndPhysics"))
    (:B
      (Development|SetHiddeninGame _fire_wall true false)
      (Collision|SetCollisionEnabled _fire_wall "NoCollision"))))

(event EventBeginPlay
  (Collision|SetCollisionEnabled (Variables|Default|GetFire%20Wall) "NoCollision")
  (CallFunction|WallTimer))

(fn ConstructionScript)