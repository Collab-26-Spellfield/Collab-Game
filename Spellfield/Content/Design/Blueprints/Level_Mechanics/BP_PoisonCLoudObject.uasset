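; A level mechanic object that releases a poison cloud whenever it takes damage.
; On any damage it hides its cylinder mesh, turns off collision and spawns BP_PoisonCloud at its own transform.
; A timer then restores visibility and collision after a short delay, so the object can be triggered again.
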(event Custom|Disable%20Object
  (Development|SetHiddeninGame (Variables|Default|GetCylinder) true false)
  (Collision|SetCollisionEnabled (Variables|Default|GetCylinder) "NoCollision"))

(event Custom|Enable%20Object
  (Development|SetHiddeninGame (Variables|Default|GetCylinder) false false)
  (Collision|SetCollisionEnabled (Variables|Default|GetCylinder) "QueryAndPhysics"))

(event Custom|Reset%20Timer
  (Utilities|Time|SetTimerbyEvent (delegate Custom|Reset) 7.0))

(event Custom|Reset
  (CallFunction|EnableObject))

(event Game|Damage|EventAnyDamage
  (params (Damage :type Float%20%28single-precision%29) (DamageType :type Damage%20Type%20Object%20Reference) (InstigatedBy :type Controller%20Object%20Reference) (DamageCauser :type Actor%20Object%20Reference))
  (CallFunction|DisableObject)
  (Game|SpawnActorfromClass "/Game/Tech/Blueprints/BP_PoisonCloud.BP_PoisonCloud_C" (Transformation|GetActorTransform) "Undefined" "MultiplyWithRoot" 0 0)
  (CallFunction|ResetTimer))

(fn ConstructionScript)