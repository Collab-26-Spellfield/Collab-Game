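; Actor component that debounces hits, so the same actor is not registered as hit repeatedly in quick succession.
; ActorHit returns false for actors already in RecentlyHitActors, otherwise it adds the actor and returns true.
; A looping timer started on BeginPlay clears the whole list every quarter second, so the lockout per actor varies up to that interval.
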(event Custom|Clear%20Recently%20Hit%20Actor
  ;[0.15 0.15 0.15 0.5] Clear Array Timer
  (Utilities|Time|SetTimerbyEvent (delegate Custom|Clear%20Array) 0.25 true))

(event Custom|Clear%20Array
  ;[0.15 0.15 0.15 0.5] Clear Array Timer
  (Utilities|Array|Clear (Variables|Default|GetRecently%20Hit%20Actors)))

(event Custom|Add%20to%20Recently%20Hit%20Actors
  (params (Hit%20Actor :type Actor%20Object%20Reference))
  ;[0.15 0.15 0.15 0.5] Add To Recently Hit Actors
  (Utilities|Array|Add (Variables|Default|GetRecently%20Hit%20Actors) Hit%20Actor))

(event EventBeginPlay
  ;[0.15 0.15 0.15 0.5] Start Timer
  (CallFunction|ClearRecentlyHitActor))

(fn ActorHit
  (params (Hit%20Actor :type Actor%20Object%20Reference))
  (if (Utilities|Array|ContainsItem (Variables|Default|GetRecently%20Hit%20Actors) Hit%20Actor)
    (return false)
    (else
      (CallFunction|AddtoRecentlyHitActors Hit%20Actor)
      (return true))))