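; BP_Pillar is a destructible level pillar that topples away from its killer and hurts actors it hits.
; On death, it picks the fall point facing most away from the damage causer, then a timeline pitches and lowers that point.
; A timeline track opens a damage window in which overlaps apply damage and plane-projected knockback, filtered by a recently-hit component.
; A debug widget displays its health.
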(event Die(BP_HealthComponent)
  (params (Damage%20Causer :type Actor%20Object%20Reference))
  (if (Variables|Default|GetCan%20Fall)
    (Variables|Default|SetCan%20Fall false)
    (CallFunction|DamagingActorLocation (Transformation|GetActorLocation Damage%20Causer))
    (Variables|Default|SetStarting%20Rotation (Transformation|GetWorldRotation (Variables|Default|GetRotation%20Point)))
    (Variables|Default|SetStarting%20Location (Transformation|GetWorldLocation (Variables|Default|GetRotation%20Point)))
    (bind (_direction _newtrack_0 _newtrack_1) (Timeline|Timeline Play)
      (:Update
        (Transformation|SetWorldRotation (Variables|Default|GetRotation%20Point) (Math|Rotator|Lerp(Rotator) (Variables|Default|GetStarting%20Rotation) (Math|Rotator|MakeRotator (.roll (Variables|Default|GetStarting%20Rotation)) (+ (.pitch (Variables|Default|GetStarting%20Rotation)) -9e+01) (.yaw (Variables|Default|GetStarting%20Rotation))) _newtrack_0) false false)
        (Transformation|SetWorldLocation (Variables|Default|GetRotation%20Point) (Math|Vector|Lerp(Vector) (Variables|Default|GetStarting%20Location) (- (Variables|Default|GetStarting%20Location) "0.000000,0.000000,50.000000") _newtrack_1) false false))
      (:Finished
        (Collision|SetCollisionEnabled (Variables|Default|GetPillar%20Main2) "QueryAndPhysics")
        (Variables|Default|SetCan%20damage false))
      (:NewTrack_2
        (Variables|Default|SetCan%20damage true)))))

(event OnComponentBeginOverlap(PillarMain)
  (params (OverlappedComponent :type Primitive%20Component%20Object%20Reference) (OtherActor :type Actor%20Object%20Reference) (OtherComp :type Primitive%20Component%20Object%20Reference) (OtherBodyIndex :type Integer) (bFromSweep :type Boolean) (SweepResult :type Hit%20Result%20Structure%20%28by%20ref%29))
  (if (Variables|Default|GetCan%20damage)
    (bind _should_damage (Default|ActorHit (Variables|Default|GetBP_RecentlyHitActorsComponent) OtherActor))
    (if _should_damage
      (Game|Damage|ApplyDamage OtherActor 6e+01 0 0)
      (Class|BPIKnockbackInterface|Knockback(Message) OtherActor 1e+01 (+ (Math|Vector|ProjectVectorontoPlane (- (Transformation|GetActorLocation OtherActor) (Transformation|GetActorLocation)) (Math|Vector|GetRightVector (Variables|Default|GetRotation%20Point))) (Transformation|GetActorLocation))))))

(event Custom|Damaging%20Actor%20Location
  (params (Actor%20Location :type Vector))
  (bind _current_closest_side (CallFunction|FindFallRotation Actor%20Location))
  (Development|PrintString (Utilities|GetDisplayName _current_closest_side))
  (Variables|Default|SetRotation%20Point _current_closest_side))

(event EventBeginPlay
  (Utilities|Array|Add (Variables|Default|GetFall%20Point%20Array) (Variables|Default|GetFall%20point%201))
  (Utilities|Array|Add (Variables|Default|GetFall%20Point%20Array) (Variables|Default|GetFall%20point%202))
  (Utilities|Array|Add (Variables|Default|GetFall%20Point%20Array) (Variables|Default|GetFall%20point%203))
  (Utilities|Array|Add (Variables|Default|GetFall%20Point%20Array) (Variables|Default|GetFall%20point%204))
  (bind _aswbp_debug_pillar_health (Utilities|Casting|CastToWBP_DebugPillarHealth (UserInterface|GetWidget (Variables|Default|GetHealthBar))))
  (Default|Init _aswbp_debug_pillar_health self))

(event Game|Damage|EventAnyDamage
  (params (Damage :type Float%20%28single-precision%29) (DamageType :type Damage%20Type%20Object%20Reference) (InstigatedBy :type Controller%20Object%20Reference) (DamageCauser :type Actor%20Object%20Reference))
  (Development|PrintString (Utilities|GetDisplayName DamageCauser)))

(fn ConstructionScript)

(fn FindFallRotation
  (params (Damage%20Location :type Vector))
  (for _array_element (Variables|Default|GetFall%20Point%20Array)
    (if (< (Math|Vector|DotProduct (- Damage%20Location (Transformation|GetActorLocation)) (Math|Vector|GetForwardVector _array_element)) (LocalVariables|GetShortest%20Distance))
      (LocalVariables|SetClosest%20Side _array_element)
      (LocalVariables|SetShortest%20Distance (Math|Vector|DotProduct (- Damage%20Location (Transformation|GetActorLocation)) (Math|Vector|GetForwardVector _array_element)))))
  (return (LocalVariables|GetClosest%20Side)))