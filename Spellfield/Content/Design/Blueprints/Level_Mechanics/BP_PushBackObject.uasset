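; BP_PushBackObject is a level mechanic that, when damaged while active, emits repeated knockback pulses around itself.
; Damage deactivates it, turns its cube red and starts a looping timer that counts pulses up to MaxPushes.
; Each pulse runs a debug-drawn sphere trace and sends a knockback message to hit actors, using its location as the source.
; After the last pulse, a cooldown timer re-arms it and turns it green.
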(event Custom|Start%20Push%20Back
  ;[0.15 0.15 0.15 0.5] Push Back Timer
  (bind _returnvalue (Utilities|Time|SetTimerbyEvent (delegate Custom|Push%20Back) 0.5 true))
  (Variables|Default|SetPushBackTimer _returnvalue))

(event Custom|Push%20Back
  ;[0.15 0.15 0.15 0.5] Push Back Timer
  (Math|Integer|IncrementInt (Variables|Default|GetCurrent%20Pushes)
    (:%20%20
      (CallFunction|PushBackPlayers)
      (if (>= (Variables|Default|GetCurrent%20Pushes) (Variables|Default|GetMax%20Pushes))
        (Utilities|Time|ClearandInvalidateTimerbyHandle (Variables|Default|GetPushBackTimer))
        (Variables|Default|SetCurrent%20Pushes 0)
        (CallFunction|ObjectCooldown)))))

(event Custom|Object%20Cooldown
  ;[0.15 0.15 0.15 0.5] Object Cooldown and Reset
  (Utilities|Time|SetTimerbyEvent (delegate Custom|Reset) 5.0))

(event Custom|Push%20Back%20players
  (bind _returnvalue (Transformation|GetActorLocation))
  ;[0.15 0.15 0.15 0.5] Push Back Players
  (bind (_outhits _returnvalue_2) (Collision|MultiSphereTraceForObjects _returnvalue _returnvalue 4e+02 (Variables|Default|GetObject%20Types) false 0 "ForDuration" true "(R=1.000000,G=0.000000,B=0.000000,A=1.000000)" "(R=0.000000,G=1.000000,B=0.000000,A=1.000000)" 0.25))
  (if _returnvalue_2
    (for _array_element _outhits
      (Class|BPIKnockbackInterface|Knockback(Message) (.HitActor (Collision|BreakHitResult _array_element)) 1e+01 (Transformation|GetActorLocation)))))

(event Custom|Reset
  ;[0.15 0.15 0.15 0.5] Object Cooldown and Reset
  (Variables|Default|SetIs%20Active? true)
  (Rendering|Material|SetMaterial (Variables|Default|GetCube1) 0 "/Game/Design/Dev_Textures/DevMat_Green.DevMat_Green"))

(event Game|Damage|EventAnyDamage
  (params (Damage :type Float%20%28single-precision%29) (DamageType :type Damage%20Type%20Object%20Reference) (InstigatedBy :type Controller%20Object%20Reference) (DamageCauser :type Actor%20Object%20Reference))
  ;[0.15 0.15 0.15 0.5] Damaged
  (if (Variables|Default|GetIs%20Active?)
    (Variables|Default|SetIs%20Active? false)
    (CallFunction|StartPushBack)
    (Rendering|Material|SetMaterial (Variables|Default|GetCube1) 0 "/Game/Design/Dev_Textures/DevMat_Red.DevMat_Red")))

(fn ConstructionScript)