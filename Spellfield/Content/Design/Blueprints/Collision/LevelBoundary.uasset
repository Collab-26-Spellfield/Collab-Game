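; LevelBoundary is an actor that encloses a rectangular level area with four box collision walls, sized from a Size variable.
; Its construction script stretches each wall's extent to half the matching Size axis plus padding, so corners overlap, at a fixed height and thickness.
; It then offsets each wall outward so its inner face lies on the area's edge.
; The event graph has no active logic.
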(event EventBeginPlay)

(event Collision|EventActorBeginOverlap
  (params (OtherActor :type Actor%20Object%20Reference)))

(event EventTick
  (params (DeltaSeconds :type Float%20%28single-precision%29)))

(fn ConstructionScript
  (bind _size (Variables|Default|GetSize))
  (bind _size_2 (Variables|Default|GetSize))
  (bind (_x _y) (Math|Vector|BreakVector _size))
  (bind _returnvalue (/ _size_2 2.0))
  (bind (_x_2 _y_2) (Math|Vector|BreakVector _returnvalue))
  (Components|Box|SetBoxExtent (Variables|Default|GetLeft%20Wall) (Math|Vector|MakeVector (+ _x_2 1e+02) 5e+01 5e+02) true)
  (Components|Box|SetBoxExtent (Variables|Default|GetFront%20Wall) (Math|Vector|MakeVector 5e+01 (+ _y_2 1e+02) 5e+02) true)
  (Transformation|SetRelativeLocation (Variables|Default|GetRight%20Wall) (Math|Vector|MakeVector 0.0 (+ (/ _y 2.0) 5e+01) 0.0) false false)
  (Transformation|SetRelativeLocation (Variables|Default|GetLeft%20Wall) (Math|Vector|MakeVector 0.0 (+ (/ _y -2.0) -5e+01) 0.0) false false)
  (Transformation|SetRelativeLocation (Variables|Default|GetFront%20Wall) (Math|Vector|MakeVector (+ (/ _x 2.0) 5e+01) 0.0 0.0) false false)
  (Transformation|SetRelativeLocation (Variables|Default|GetBack%20Wall) (Math|Vector|MakeVector (+ (/ _x -2.0) -5e+01) 0.0 0.0) false false))