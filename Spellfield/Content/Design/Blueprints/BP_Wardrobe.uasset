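; BP_Wardrobe is an in-world wardrobe where a player customises hat, staff and mask cosmetics.
; Its overlap sphere claims one player through a resettable DoOnce, showing a billboard and binding menu confirm.
; Confirming teleports the player to the arrow, disables movement and maps menu axes to category and DT_CosmeticOptions row, previewing only hats immediately.
; Confirm or cancel restores walking and applies cosmetics, with cancel first assigning DefaultCosmetics.
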(event OnComponentBeginOverlap(Sphere)
  (params (OverlappedComponent :type Primitive%20Component%20Object%20Reference) (OtherActor :type Actor%20Object%20Reference) (OtherComp :type Primitive%20Component%20Object%20Reference) (OtherBodyIndex :type Integer) (bFromSweep :type Boolean) (SweepResult :type Hit%20Result%20Structure%20%28by%20ref%29))
  ;[0.15 0.15 0.15 0.5] Track Player
  (Utilities|FlowControl|DoOnce false
    (:Completed
      (bind _player (Class|BPICharacterandController|GetPlayer(Message) OtherActor))
      (Variables|Default|SetCurrentPlayer _player)
      (Rendering|SetVisibility (Variables|Default|GetBillboard) true true)
      (EventDispatchers|BindEventtoMenuConfirm (Variables|Default|GetCurrentPlayer) (delegate Custom|Begin%20Customisation)))))

(event OnComponentEndOverlap(Sphere)
  (params (OverlappedComponent :type Primitive%20Component%20Object%20Reference) (OtherActor :type Actor%20Object%20Reference) (OtherComp :type Primitive%20Component%20Object%20Reference) (OtherBodyIndex :type Integer))
  ;[0.15 0.15 0.15 0.5] Track Player
  (bind _player (Class|BPICharacterandController|GetPlayer(Message) OtherActor))
  (if (== _player (Variables|Default|GetCurrentPlayer))
    (Rendering|SetVisibility (Variables|Default|GetBillboard) false true)
    (CallFunction|Unlock)
    (EventDispatchers|UnbindallEventsfromMenuConfirm (Variables|Default|GetCurrentPlayer))))

(event Custom|Begin%20Customisation
  (bind _currentplayer (Variables|Default|GetCurrentPlayer))
  (bind _currentplayer_2 (Variables|Default|GetCurrentPlayer))
  ;[0.15 0.15 0.15 0.5] Begin Customisation
  (Pawn|Components|CharacterMovement|DisableMovement (Variables|/Script/Engine.Character|GetCharacterMovement _currentplayer_2))
  (Transformation|SetActorTransform _currentplayer_2 (Transformation|GetWorldTransform (Variables|Default|GetArrow)) false true)
  (Variables|Default|SetDefaultCosmetics "")
  (EventDispatchers|BindEventtoMenuConfirm _currentplayer (delegate Custom|Confirm%20Customisation))
  (EventDispatchers|BindEventtoMenuCancel _currentplayer (delegate Custom|Cancel%20Customisation))
  (EventDispatchers|BindEventtoMenuMove _currentplayer (delegate Custom|Menu%20Move)))

(event Custom|Confirm%20Customisation
  (bind _currentplayer (Variables|Default|GetCurrentPlayer))
  ;[0.15 0.15 0.15 0.5] Confirm/Cancel Cosmetics
  (Pawn|Components|CharacterMovement|SetMovementMode (Variables|/Script/Engine.Character|GetCharacterMovement _currentplayer) "MOVE_Walking" 0)
  (CallFunction|Unlock)
  (Default|ApplyCosmetics _currentplayer))

(event Custom|Cancel%20Customisation
  (bind _currentplayer (Variables|Default|GetCurrentPlayer))
  ;[0.15 0.15 0.15 0.5] Confirm/Cancel Cosmetics
  (Variables|/Game/Design/Blueprints/Character/BP_PlayerCharacter.BP_PlayerCharacter_C|SetCosmetics (Variables|Default|GetCurrentPlayer) (Variables|Default|GetDefaultCosmetics))
  (Pawn|Components|CharacterMovement|SetMovementMode (Variables|/Script/Engine.Character|GetCharacterMovement _currentplayer) "MOVE_Walking" 0)
  (CallFunction|Unlock)
  (Default|ApplyCosmetics _currentplayer))

(event Custom|Change%20Category
  (params (Direction :type Integer))
  ;[0.15 0.15 0.15 0.5] Change Category
  (bind _output_get (Variables|Default|SetCategory (Math|Integer|Clamp(Integer) (+ Direction (Variables|Default|GetCategory)) 0 2)))
  (Rendering|Components|TextRender|SetText (Variables|Default|GetPrompt) (Utilities|Text|ToText(Integer) _output_get)))

(event Custom|Change%20Cosmetic
  (params (Direction :type Integer))
  (bind _currentplayer (Variables|Default|GetCurrentPlayer))
  (bind _cosmetics (Variables|/Game/Design/Blueprints/Character/BP_PlayerCharacter.BP_PlayerCharacter_C|GetCosmetics _currentplayer))
  ;[0.15 0.15 0.15 0.5] Change Selected Cosmetic
  (bind _outrownames (DataTable|GetDataTableRowNames "/Game/DT_CosmeticOptions.DT_CosmeticOptions"))
  (bind _output_get (Variables|Default|SetSelection (Math|Integer|%(Integer) (+ Direction (Variables|Default|GetSelection)) (Utilities|Array|Length _outrownames))))
  (if (== (Variables|Default|GetSelection) -1)
    (Variables|Default|SetSelection (- (Utilities|Array|Length _outrownames) 1)))
  (bind _returnvalue (Utilities|GetDataTableRow "/Game/DT_CosmeticOptions.DT_CosmeticOptions" (Utilities|String|StringToName (Utilities|String|ToString(Integer) _output_get)))
    (:then
      (switch int (Variables|Default|GetCategory)
        (:0
          (Utilities|Struct|SetmembersinS_Cosmetics _cosmetics (.Hat (Utilities|Struct|BreakS_Cosmetics _returnvalue)))
          (Development|PrintString (Utilities|GetDisplayName (.Hat (Utilities|Struct|BreakS_Cosmetics _returnvalue))))
          (Default|ApplyCosmetics _currentplayer))
        (:1
          (Utilities|Struct|SetmembersinS_Cosmetics _cosmetics (.Staff (Utilities|Struct|BreakS_Cosmetics _returnvalue))))
        (:2
          (Utilities|Struct|SetmembersinS_Cosmetics _cosmetics (.Mask (Utilities|Struct|BreakS_Cosmetics _returnvalue))))))))

(event Custom|Unlock
  ;[0.15 0.15 0.15 0.5] Track Player
  (Utilities|FlowControl|DoOnce false) ; enters at Reset
)

(event Custom|Menu%20Move
  (params (NewParam :type Vector%202D%20Structure))
  ;[0.15 0.15 0.15 0.5] Begin Customisation
  (CallFunction|ChangeCosmetic (Math|Float|Round (.x NewParam)))
  (CallFunction|ChangeCategory (Math|Float|Round (.y NewParam))))

(event EventBeginPlay)

(event Collision|EventActorBeginOverlap
  (params (OtherActor :type Actor%20Object%20Reference)))

(event EventTick
  (params (DeltaSeconds :type Float%20%28single-precision%29)))

(fn ConstructionScript)