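; Poison component that damages its owner through BP_HealthComponent while its Timer is above zero.
; A looping one-second timer, started on BeginPlay, fires PoisonDamage, whose while loop applies damage and prints Timer on each iteration.
; Timer decreases only when Overlap is false, so the loop drains it within a single call, or never exits if Overlap is true.
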(event Custom|Poison%20Damage
  (while (> (Variables|Default|GetTimer) 0)
    (Default|TakeDamage (Actor|GetComponentbyClass (Components|GetOwner) "/Game/Tech/Blueprints/BP_HealthComponent.BP_HealthComponent_C") 0 (Variables|Default|GetDamage))
    (if (Variables|Default|GetOverlap)
      _
      (else
        (Variables|Default|SetTimer (- (Variables|Default|GetTimer) 1))))
    (Development|PrintString (Utilities|String|ToString(Integer) (Variables|Default|GetTimer)))))

(event EventBeginPlay
  (Utilities|Time|SetTimerbyEvent (delegate Custom|Poison%20Damage) 1.0 true true))