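; Respawn pad actor that tracks whether it is occupied and reports its distance to players for spawn selection.
; UseSpawnPad flags it in use, CheckSpawnPadUsage returns that flag, and FreeUpSpawnPad clears it after a long delay.
; FindDistToPlayers loops over the GameInstance player data map, skips the given player, and returns the distance to the farthest remaining pawn, not the nearest.
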(event Custom|FreeUpSpawnPad
  (Utilities|FlowControl|Delay 1e+03)
  (Variables|Default|SetSpawnpadInUse false))

(event Custom|UseSpawnPad
  (Variables|Default|SetSpawnpadInUse true))

(fn ConstructionScript)

(fn FindDisttoPlayers
  (params (player :type BP%20Player%20Character%20Object%20Reference))
  (Variables|Default|SetDistanceFromPlayers 0.0)
  (bind _playerconnectiondata (Class|BPIPlayerConnectionInfo|GetPlayerData(Message) (Game|GetGameInstance)))
  (bind _valuepin (Utilities|Map|ForEachLoop(Map) _playerconnectiondata)
    (:then
      (if (not (== (.playerpawn _valuepin) player))
        (if (> (Math|Vector|Distance(Vector) (Transformation|GetActorLocation (.playerpawn _valuepin)) (Transformation|GetActorLocation)) (Variables|Default|GetDistanceFromPlayers))
          (Variables|Default|SetDistanceFromPlayers (Math|Vector|Distance(Vector) (Transformation|GetActorLocation (.playerpawn _valuepin)) (Transformation|GetActorLocation))))))
    (:CompletedPin
      (return (Variables|Default|GetDistanceFromPlayers)))))

(fn CheckSpawnPadUsage
  (return (Variables|Default|GetSpawnpadInUse)))