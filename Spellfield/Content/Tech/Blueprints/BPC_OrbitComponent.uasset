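; Actor component that moves its owning actor in an orbit around a Player for a limited time.
; StartOrbit stores the angle, radius and target, then destroys the owner after OrbitTime.
; Tick advances the angle by OrbitSpeed and sets the owner's location from NewOrbitPosition, without checking ShouldOrbit.
; NewOrbitPosition contains sine/cosine circle math around the Player at the same height, though that vector appears unconnected.
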(event Custom|StartOrbit
  (params (StartingRotation :type Float%20%28double-precision%29) (Radius :type Float%20%28double-precision%29) (Player :type BP%20Player%20Character%20Object%20Reference) (OrbitTime :type Float%20%28double-precision%29))
  (Variables|Default|SetShouldOrbit true)
  (Variables|Default|SetStarting%20Rotation StartingRotation)
  (Variables|Default|SetRadius Radius)
  (Variables|Default|SetPlayer Player)
  (Utilities|FlowControl|Delay OrbitTime)
  (Actor|DestroyActor (Components|GetOwner)))

(event EventTick
  (params (DeltaSeconds :type Float%20%28single-precision%29))
  (Variables|Default|SetStarting%20Rotation (+ (Variables|Default|GetStarting%20Rotation) (* (Variables|Default|GetOrbitSpeed) (Utilities|Time|GetWorldDeltaSeconds))))
  (Transformation|SetActorLocation (Components|GetOwner) (Utilities|NewOrbitPosition) false false))