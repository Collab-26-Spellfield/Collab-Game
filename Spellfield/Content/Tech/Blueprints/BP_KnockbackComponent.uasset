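; BP_KnockbackComponent is a component that pushes an actor away from a knockback source.
; Its KnockbackCalculation event stores the amount, source and target, then finds the look-at direction from source to target.
; It drops the vertical part without renormalizing, scales by the amount times a constant, and applies it as a velocity-change impulse on the target's CharacterMovementComponent.
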(event Custom|KnockbackCalculation
  (params (KnockbackAmount :type Float%20%28double-precision%29) (KnockbackSource :type Actor%20Object%20Reference) (KnockbackedActor :type Actor%20Object%20Reference))
  (Variables|Default|SetKnockbackValue KnockbackAmount)
  (Variables|Default|SetKnockbackSource KnockbackSource)
  (Variables|Default|SetKnockbackedActor KnockbackedActor)
  (Physics|AddImpulse (Actor|GetComponentbyClass (Variables|Default|GetKnockbackedActor) "/Script/Engine.CharacterMovementComponent") (* (Math|Vector|MakeVector (.x (Math|Vector|GetForwardVector (Math|Rotator|FindLookatRotation (Transformation|GetActorLocation (Variables|Default|GetKnockbackSource)) (Transformation|GetActorLocation (Variables|Default|GetKnockbackedActor))))) (.y (Math|Vector|GetForwardVector (Math|Rotator|FindLookatRotation (Transformation|GetActorLocation (Variables|Default|GetKnockbackSource)) (Transformation|GetActorLocation (Variables|Default|GetKnockbackedActor))))) 0.0) (* (Variables|Default|GetKnockbackValue) 1e+03)) true))