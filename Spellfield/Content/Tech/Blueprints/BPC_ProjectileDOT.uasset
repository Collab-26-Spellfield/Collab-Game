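; Projectile damage-over-time component that deals poison damage to the player pawn resolved from its owner through GetPlayerMessage.
; Init stores the damage, duration, causer and instigator, applies a first tick immediately and starts a looping timer at the tick rate.
; Math expressions derive per-tick damage and tick count, and the component destroys itself when the target dies or the count is reached.
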(event Custom|Init
  (params (Damage :type Float%20%28double-precision%29) (Time :type Float%20%28double-precision%29) (DamageCauser :type Actor%20Object%20Reference) (Controller :type Controller%20Object%20Reference))
  (Variables|Default|SetFullDamage Damage)
  (Variables|Default|SetTime Time)
  (Variables|Default|SetDamageCauser DamageCauser)
  (Variables|Default|SetInstigator Controller)
  (Utilities|Time|SetTimerbyEvent (delegate Custom|Damage) (/ 1.0 (Variables|Default|GetTicksPerSecond)) true)
  (CallFunction|Damage))

(event Custom|Damage
  (bind _player (Class|BPICharacterandController|GetPlayer(Message) (Components|GetOwner)))
  (Game|Damage|ApplyDamage _player (Math|Conversions|ToFloat(Integer) (|(Floor(((Damage/{3E45A6DE-4ABA-49A4-405C-EDB6F51109BA})/{A6A6E92F-4557-E5C5-8110-749B455B3A81}))) (Variables|Default|GetFullDamage))) (Variables|Default|GetInstigator) (Variables|Default|GetDamageCauser) "/Game/Tech/DamageTypeBP_Poison.DamageTypeBP_Poison_C")
  (if (Variables|/Game/Design/Blueprints/Character/BP_PlayerCharacter.BP_PlayerCharacter_C|GetIsDead _player)
    (Components|DestroyComponent)
    (else
      (bind _result (Math|Integer|IncrementInt (Variables|Default|GetTickCounter))
        (:%20%20
          (if (>= _result (Math|Float|Truncate (|({3E45A6DE-4ABA-49A4-405C-EDB6F51109BA}/(1/{A6A6E92F-4557-E5C5-8110-749B455B3A81})))))
            (Components|DestroyComponent)))))))