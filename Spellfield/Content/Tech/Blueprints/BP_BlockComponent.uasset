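; Player block ability component that grants timed immunity and enables a radius-scaled collision sphere, then runs a cooldown shown on the spatial UI.
; Each actor entering the sphere is handled once per block.
; Projectiles get an orbit component that replaces their movement to circle the player, while other players take attack-scaled damage and knockback, both depending on upgrade multipliers.
; MirrorImage and ReflectDamage are unfinished stubs.
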(event Custom|BlockCooldown
  ;[0.1321 0.06245 0.15 0.5 40] Block Pressed
  (Variables|Default|SetBlock%20free true)
  (Utilities|Array|Clear (Variables|Default|GetHitActors)))

(event Custom|Init
  (params (Playerref :type BP%20Player%20Character%20Object%20Reference) (RadiusMultiplier :type Float%20%28double-precision%29))
  (Variables|Default|SetBlock%20Radius RadiusMultiplier)
  (Variables|Default|SetPlayerref Playerref)
  (Collision|BindEventtoOnComponentBeginOverlap (Variables|/Game/Design/Blueprints/Character/BP_PlayerCharacter.BP_PlayerCharacter_C|GetBlockRadius (Variables|Default|GetPlayerref)) (delegate Custom|Check%20What%20Hit)))

(event Custom|TurnBlockOff
  (bind _playerref (Variables|Default|GetPlayerref))
  (bind _block_cooldown (Variables|Default|GetBlock%20Cooldown))
  ;[0.1321 0.06245 0.15 0.5 40] Block Pressed
  (Default|SetImmunity (Variables|/Game/Design/Blueprints/Character/BP_PlayerCharacter.BP_PlayerCharacter_C|GetBP_HealthComponent _playerref) (not (Variables|/Game/Design/Blueprints/Character/BP_PlayerCharacter.BP_PlayerCharacter_C|GetInPregame _playerref)) false)
  (Collision|SetCollisionEnabled (Variables|/Game/Design/Blueprints/Character/BP_PlayerCharacter.BP_PlayerCharacter_C|GetBlockRadius (Variables|Default|GetPlayerref)) "NoCollision")
  (Rendering|SetVisibility (Variables|/Game/Design/Blueprints/Character/BP_PlayerCharacter.BP_PlayerCharacter_C|GetBlockDebug (Variables|Default|GetPlayerref)) false false)
  (Utilities|Time|SetTimerbyEvent (delegate Custom|BlockCooldown) _block_cooldown)
  (Default|StartCooldown (Variables|/Game/UI/SpatialUI/WBP_SpatialPlayerUI.WBP_SpatialPlayerUI_C|GetBlockCooldown (Variables|/Game/Design/Blueprints/Character/BP_PlayerCharacter.BP_PlayerCharacter_C|GetSpatialUI (Variables|Default|GetPlayerref))) _block_cooldown))

(event Custom|Block
  (bind _block_radius (Variables|Default|GetBlock%20Radius))
  (bind _playerref (Variables|Default|GetPlayerref))
  (bind _playerref_2 (Variables|Default|GetPlayerref))
  ;[0.1321 0.06245 0.15 0.5 40] Block Pressed
  (Components|Sphere|SetSphereRadius (Variables|/Game/Design/Blueprints/Character/BP_PlayerCharacter.BP_PlayerCharacter_C|GetBlockRadius (Variables|Default|GetPlayerref)) (* (Variables|Default|GetBlock%20Radius) 2e+02) true)
  (Transformation|SetRelativeScale3D (Variables|/Game/Design/Blueprints/Character/BP_PlayerCharacter.BP_PlayerCharacter_C|GetBlockDebug (Variables|Default|GetPlayerref)) (* (Math|Vector|MakeVector _block_radius _block_radius _block_radius) 4.0))
  (if (Variables|Default|GetBlock%20free)
    (Default|SetImmunity (Variables|/Game/Design/Blueprints/Character/BP_PlayerCharacter.BP_PlayerCharacter_C|GetBP_HealthComponent _playerref) (not (Variables|/Game/Design/Blueprints/Character/BP_PlayerCharacter.BP_PlayerCharacter_C|GetInPregame _playerref)) true)
    (Rendering|SetVisibility (Variables|/Game/Design/Blueprints/Character/BP_PlayerCharacter.BP_PlayerCharacter_C|GetBlockDebug _playerref_2) true false)
    (Collision|SetCollisionEnabled (Variables|/Game/Design/Blueprints/Character/BP_PlayerCharacter.BP_PlayerCharacter_C|GetBlockRadius _playerref_2) "QueryAndPhysics")
    (Development|PrintString "blocking")
    (Animation|Montage|PlayMontage (Variables|/Script/Engine.Character|GetMesh (Variables|Default|GetPlayerref)) "/Game/Art/Animations/Montages_And_BlendSpaces/AM_Block.AM_Block"
      (:then
        (Variables|Default|SetBlock%20free false)
        (Utilities|Time|SetTimerbyEvent (delegate Custom|TurnBlockOff) (Variables|Default|GetBlockDuration)))
      (:OnCompleted
        (Development|PrintString "blockdone")))))

(event Custom|Check%20What%20Hit
  (params (OverlappedComponent :type Primitive%20Component%20Object%20Reference) (OtherActor :type Actor%20Object%20Reference) (OtherComp :type Primitive%20Component%20Object%20Reference) (OtherBodyIndex :type Integer) (bFromSweep :type Boolean) (SweepResult :type Hit%20Result%20Structure%20%28by%20ref%29))
  (bind _playerref (Variables|Default|GetPlayerref))
  ;[0.117 0.06386 0.15 0.5 30] When Block is active.
  (Variables|Default|SetOtherActor OtherActor)
  (if (not (Utilities|Array|ContainsItem (Variables|Default|GetHitActors) (Variables|Default|GetOtherActor)))
    (Utilities|Array|Add (Variables|Default|GetHitActors) (Variables|Default|GetOtherActor))
    (Utilities|IsValid (Variables|Default|GetOtherActor)
      (:Is%20Valid
        (if (Actor|ActorHasTag (Variables|Default|GetOtherActor) "Projectile")
          (if (> (Variables|Default|GetOrbitMultiplier) 0.0)
            (CallFunction|Orbit))
          (elif (Math|Boolean|ANDBoolean (Actor|ActorHasTag (Variables|Default|GetOtherActor) "Player") (!= (Variables|Default|GetOtherActor) (Variables|Default|GetPlayerref)) (> (Variables|Default|GetBlockMultiplier) 1.0))
            (Game|Damage|ApplyDamage (Variables|Default|GetOtherActor) (* (Variables|Default|GetBlockMultiplier) (Variables|/Game/Tech/Blueprints/BP_AttackComponent.BP_AttackComponent_C|GetAttackDamage (Variables|/Game/Design/Blueprints/Character/BP_PlayerCharacter.BP_PlayerCharacter_C|GetBP_AttackComponent (Variables|Default|GetPlayerref)))) 0 0)
            (Class|BPIKnockbackInterface|Knockback(Message) (Variables|Default|GetOtherActor) (* 1e+01 (Variables|/Game/Tech/Blueprints/BP_AttackComponent.BP_AttackComponent_C|GetKnockbackMultiplier (Variables|/Game/Design/Blueprints/Character/BP_PlayerCharacter.BP_PlayerCharacter_C|GetBP_AttackComponent _playerref))) (Transformation|GetActorLocation _playerref))))))))

(fn MirrorImage
  (for _index (range 1 (Math|Float|Truncate (Variables|/Game/Tech/Blueprints/BP_AttackComponent.BP_AttackComponent_C|GetReflectDuplication (Variables|/Game/Design/Blueprints/Character/BP_PlayerCharacter.BP_PlayerCharacter_C|GetBP_AttackComponent (Variables|Default|GetPlayerref)))))
    (if (LocalVariables|GetIsPositive)
      _))
  (LocalVariables|SetIsPositive true)
  (LocalVariables|SetRotation 5.0))

(fn Orbit
  (bind _playerref (Variables|Default|GetPlayerref))
  (bind _otheractor (Variables|Default|GetOtherActor))
  (bind _returnvalue (Transformation|GetActorLocation _playerref))
  (bind _returnvalue_2 (Transformation|GetActorLocation _otheractor))
  (bind _returnvalue_3 (- _returnvalue_2 _returnvalue))
  (bind _returnvalue_4 (Game|AddComponentbyClass (Variables|Default|GetOtherActor) "/Game/Tech/Blueprints/BPC_OrbitComponent.BPC_OrbitComponent_C"))
  (LocalVariables|SetOrbitComp _returnvalue_4)
  (Components|Activation|SetActive (Actor|GetComponentbyClass (Variables|Default|GetOtherActor) "/Script/Engine.ProjectileMovementComponent") false false)
  (bind _output_get (LocalVariables|SetOrbitPoint _returnvalue))
  (Development|PrintString "Hello")
  (Default|StartOrbit (LocalVariables|GetOrbitComp) (Class|KismetMathLibrary|DegAtan2 (.x _returnvalue_3) (.y _returnvalue_3)) (Math|Vector|Distance(Vector) _returnvalue_2 _output_get) _playerref (* (Variables|Default|GetOrbitMultiplier) 3.0)))

(fn ReflectDamage)