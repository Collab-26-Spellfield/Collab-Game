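; BP_Crystal_Parent is the base crystal Blueprint, which hands a modifier to actors that overlap it.
; On overlap it constructs an object from its Modifier class, with the other actor as outer.
; If that actor implements BPI_modifiers, it receives the object through RecievedModifierMessage.
; The modifier is constructed before the interface check, and the construction script is empty.
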(event Collision|EventActorBeginOverlap
  (params (OtherActor :type Actor%20Object%20Reference))
  (Variables|Default|SetOther%20Actor OtherActor)
  (Utilities|IsValid (Variables|Default|GetOther%20Actor)
    (:Is%20Valid
      (if true
        (bind _returnvalue (Game|ConstructObjectfromClass (Variables|Default|GetOther%20Actor) (Variables|Default|GetModifier)))
        (if (Utilities|DoesObjectImplementInterface (Variables|Default|GetOther%20Actor) "/Game/Tech/Blueprints/Crystals/BPI_modifiers.BPI_modifiers_C")
          (Class|BPIModifiers|RecievedModifier(Message) (Variables|Default|GetOther%20Actor) _returnvalue))))))

(fn ConstructionScript)