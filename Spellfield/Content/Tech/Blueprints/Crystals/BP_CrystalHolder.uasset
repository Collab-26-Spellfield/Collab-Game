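; BP_CrystalHolder is a spawner actor that keeps a crystal in place and respawns it after it is destroyed.
; On BeginPlay it spawns the configured crystal class at its Cone component's world transform and binds to that actor's OnDestroyed event.
; When the crystal is destroyed, a five-second timer triggers a new spawn, which rebinds the same event so the cycle repeats.
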(event Custom|spawn%20crystal
  (bind _returnvalue (Game|SpawnActorfromClass (Variables|Default|GetCrystaltospawn) (Transformation|GetWorldTransform (Variables|Default|GetCone)) "Undefined" "MultiplyWithRoot" 0 0))
  (Game|BindEventtoOnDestroyed _returnvalue (delegate Custom|respawn%20crystal)))

(event Custom|respawn%20crystal
  (params (DestroyedActor :type Actor%20Object%20Reference))
  (Utilities|Time|SetTimerbyEvent (delegate Custom|r) 5.0))

(event Custom|r
  (CallFunction|SpawnCrystal))

(event EventBeginPlay
  (CallFunction|SpawnCrystal))

(event Collision|EventActorBeginOverlap
  (params (OtherActor :type Actor%20Object%20Reference)))

(event EventTick
  (params (DeltaSeconds :type Float%20%28single-precision%29)))

(fn ConstructionScript)