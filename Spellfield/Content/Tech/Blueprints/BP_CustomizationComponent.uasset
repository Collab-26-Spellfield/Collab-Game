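; Player customization component that cycles hat, staff and mask cosmetics during pregame.
; On BeginPlay in Lvl_Main, it caches the player reference and row names from the cosmetic DataTables.
; Input actions step through rows: staff and mask wrap and swap meshes, while hat increments without wrapping and assigns HatMesh directly.
; Masks also get a per-player dynamic material; the emissive tint step is disconnected.
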(event Input|EnhancedActionEvents|EnhancedInputActionIA_ChangeStaff
  (params (ActionValue :type Boolean) (ElapsedSeconds :type Float%20%28double-precision%29) (TriggeredSeconds :type Float%20%28double-precision%29) (InputAction :type Input%20Action%20Object%20Reference :default "/Game/Design/Inputs/IA_ChangeStaff.IA_ChangeStaff"))
  (:Started
    (if (Variables|/Game/Design/Blueprints/Character/BP_PlayerCharacter.BP_PlayerCharacter_C|GetInPregame (Variables|Default|GetPlayer%20ref))
      (if (== (Variables|Default|GetStaffIndex) (- (Utilities|Array|Length (Variables|Default|Getstaff%20table)) 1))
        (Variables|Default|SetStaffIndex 0)
        (else
          (Math|Integer|IncrementInt (Variables|Default|GetStaffIndex)
            (:%20%20
              _))))
      (bind _returnvalue (Utilities|GetDataTableRow "/Game/Tech/DT_Staffs.DT_Staffs" (Utilities|Array|Get(acopy) (Variables|Default|Getstaff%20table) (Variables|Default|GetStaffIndex)))
        (:then
          (Components|StaticMesh|SetStaticMesh (Variables|/Game/Design/Blueprints/Character/BP_PlayerCharacter.BP_PlayerCharacter_C|GetStaff%20Mesh (Variables|Default|GetPlayer%20ref)) (.mesh _returnvalue)))))))

(event Input|EnhancedActionEvents|EnhancedInputActionIA_ChangeMask
  (params (ActionValue :type Boolean) (ElapsedSeconds :type Float%20%28double-precision%29) (TriggeredSeconds :type Float%20%28double-precision%29) (InputAction :type Input%20Action%20Object%20Reference :default "/Game/Design/Inputs/IA_ChangeMask.IA_ChangeMask"))
  (bind _player_ref (Variables|Default|GetPlayer%20ref))
  (bind _mask_mesh (Variables|/Game/Design/Blueprints/Character/BP_PlayerCharacter.BP_PlayerCharacter_C|GetMask%20Mesh _player_ref))
  (:Started
    (if (Variables|/Game/Design/Blueprints/Character/BP_PlayerCharacter.BP_PlayerCharacter_C|GetInPregame (Variables|Default|GetPlayer%20ref))
      (if (== (Variables|Default|GetMaskIndex) (- (Utilities|Array|Length (Variables|Default|GetMask%20table)) 1))
        (Variables|Default|SetMaskIndex 0)
        (else
          (Math|Integer|IncrementInt (Variables|Default|GetMaskIndex)
            (:%20%20
              _))))
      (bind _returnvalue (Utilities|GetDataTableRow "/Game/Tech/DT_Masks.DT_Masks" (Utilities|Array|Get(acopy) (Variables|Default|GetMask%20table) (Variables|Default|GetMaskIndex)))
        (:then
          (Components|StaticMesh|SetStaticMesh _mask_mesh (.mesh _returnvalue))
          (Rendering|Material|SetMaterial (Variables|/Game/Design/Blueprints/Character/BP_PlayerCharacter.BP_PlayerCharacter_C|GetMask%20Mesh (Variables|Default|GetPlayer%20ref)) 0 (CallFunction|MakePlayerDynamicMaterial (Variables|/Game/Design/Blueprints/Character/BP_PlayerCharacter.BP_PlayerCharacter_C|GetMy%20ID (Variables|Default|GetPlayer%20ref)) (Rendering|Material|GetMaterial _mask_mesh 0))))))))

(event Input|EnhancedActionEvents|EnhancedInputActionIA_ChangeHat
  (params (ActionValue :type Boolean) (ElapsedSeconds :type Float%20%28double-precision%29) (TriggeredSeconds :type Float%20%28double-precision%29) (InputAction :type Input%20Action%20Object%20Reference :default "/Game/Design/Inputs/IA_ChangeHat.IA_ChangeHat"))
  (:Started
    (if (Variables|/Game/Design/Blueprints/Character/BP_PlayerCharacter.BP_PlayerCharacter_C|GetInPregame (Variables|Default|GetPlayer%20ref))
      (bind _result (Math|Integer|IncrementInt (Variables|Default|GetHatIndex))
        (:%20%20
          (bind _returnvalue (Utilities|GetDataTableRow "/Game/Tech/DT_Hats.DT_Hats" (Utilities|Array|Get(acopy) (Variables|Default|GetHatTable) _result))
            (:then
              (Variables|/Game/Design/Blueprints/Character/BP_PlayerCharacter.BP_PlayerCharacter_C|SetHat%20Mesh (Variables|Default|GetPlayer%20ref) (.mesh _returnvalue)))))))))

(event EventBeginPlay
  (bind _returnvalue (Game|GetCurrentLevelName true))
  (if (Utilities|Enum|Equal(Enum) _returnvalue "Lvl_Main")
    (Variables|Default|Setin%20main true)
    (bind _player (Class|BPICharacterandController|GetPlayer(Message) (Components|GetOwner)))
    (Variables|Default|SetPlayer%20ref _player)
    (bind _outrownames (DataTable|GetDataTableRowNames "/Game/Tech/DT_Hats.DT_Hats"))
    (Variables|Default|SetHatTable _outrownames)
    (bind _outrownames_2 (DataTable|GetDataTableRowNames "/Game/Tech/DT_Staffs.DT_Staffs"))
    (Variables|Default|Setstaff%20table _outrownames_2)
    (bind _outrownames_3 (DataTable|GetDataTableRowNames "/Game/Tech/DT_Masks.DT_Masks"))
    (Variables|Default|SetMask%20table _outrownames_3)))