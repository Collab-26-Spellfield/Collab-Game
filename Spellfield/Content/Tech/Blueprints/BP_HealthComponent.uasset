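; Actor component that tracks health, damage immunity and death for its owner, whether player or non-player.
; BeginPlay binds the owner's any-damage event and starts a looping timer, presumably for regeneration.
; Health changes broadcast updates, with healing clamped to max only after broadcasting, and immunity is forced on outside the game.
; At zero health it broadcasts death, first registering deaths and kills through message calls for player owners.
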(event Custom|Take%20Damage
  (params (DamagedActor :type Actor%20Object%20Reference) (Damage :type Float%20%28single-precision%29) (DamageType :type Damage%20Type%20Object%20Reference) (InstigatedBy :type Controller%20Object%20Reference) (DamageCauser :type Actor%20Object%20Reference))
  (if (not (Variables|Default|GetImmune))
    (bind _output_get (Variables|Default|SetCurrentHealth (- (Variables|Default|GetCurrentHealth) Damage)))
    (Default|CallHealthUpdated _output_get)
    (if (<= _output_get 0.0)
      (Utilities|FlowControl|Sequence
        (:then_0
          (if (not (Variables|Default|GetIsForNonPlayer))
            (bind _player (Class|BPICharacterandController|GetPlayer(Message) (Components|GetOwner)))
            (Utilities|IsValid InstigatedBy
              (:Is%20Valid
                (bind _id (Class|BPICharacterandController|GetID(Message) InstigatedBy))
                (Default|RegisterDeath _player _id)
                (bind _player_2 (Class|BPICharacterandController|GetPlayer(Message) InstigatedBy))
                (bind _id_2 (Class|BPICharacterandController|GetID(Message) (Components|GetOwner)))
                (Default|RegisterKill _player_2 _id_2))
              (:Is%20Not%20Valid
                (Default|RegisterDeath _player -1)))))
        (:then_1
          (Default|CallDie DamageCauser))))))

(event Custom|GainHealth
  (params (AmountGained :type Float%20%28double-precision%29))
  (bind _output_get (Variables|Default|SetCurrentHealth (+ (Variables|Default|GetCurrentHealth) AmountGained)))
  (Default|CallHealthUpdated _output_get)
  (if (> _output_get (Variables|Default|GetMaxHealth))
    (Variables|Default|SetCurrentHealth (Variables|Default|GetMaxHealth))))

(event Custom|HealthRegen
  (CallFunction|GainHealth (* (Variables|Default|GetHealthRegeneration) 1e+01)))

(event EventBeginPlay
  (EventDispatchers|BindEventtoOnTakeAnyDamage (Components|GetOwner) (delegate Custom|Take%20Damage))
  (Utilities|Time|SetTimerbyEvent (EventDispatchers|CreateEvent :!event Custom|HealthRegen) 0.1 true))

(fn SetImmunity
  (params (InGame :type Boolean) (Immunity :type Boolean))
  (if InGame
    (Variables|Default|SetImmune Immunity)
    (else
      (Variables|Default|SetImmune true))))