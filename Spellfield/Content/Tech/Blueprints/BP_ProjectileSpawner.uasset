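; BP_ProjectileSpawner is an actor that automatically fires BP_BaseProjectile instances on a looping one-second timer.
; Each tick of the timer spawns a projectile at the Arrow1 transform with itself as instigator, then initializes it with hardcoded stats including damage, ricochets and speed.
; After each shot, a FlipFlop teleports the spawner back and forth along world X, so consecutive shots alternate between two positions.
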(event Custom|CustomEvent
  (bind _arrow1 (Variables|Default|GetArrow1))
  (bind _returnvalue (Transformation|GetWorldTransform _arrow1))
  (bind _returnvalue_2 (Game|SpawnActorfromClass "/Game/Tech/Blueprints/BP_BaseProjectile.BP_BaseProjectile_C" (Math|Transform|MakeTransform (.location _returnvalue) (.rotation _returnvalue) "1.000000,1.000000,1.000000") "Undefined" "MultiplyWithRoot" 0 false self))
  (Default|Initialize _returnvalue_2 25.0 0.0 5.0 2.0 1.0 0.0 1.0 3e+03 1e+01)
  (Utilities|FlowControl|FlipFlop
    (:A
      (Transformation|SetActorLocation (+ (Transformation|GetActorLocation) "1200.000000,0.000000,0.000000") false true))
    (:B
      (Transformation|SetActorLocation (+ (Transformation|GetActorLocation) "-1200.000000,0.000000,0.000000") false true))))

(event EventBeginPlay
  (Utilities|Time|SetTimerbyEvent (delegate Custom|CustomEvent) 1.0 true))

(fn ConstructionScript)