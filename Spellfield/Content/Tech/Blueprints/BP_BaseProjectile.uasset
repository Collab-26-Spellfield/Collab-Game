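; Base spell projectile whose Initialize sets damage, size, speed, range and modifiers, scaling and tinting its Niagara effect per player.
; Overlaps reflect off shields, switching owner and colour, or ricochet off non-player surfaces until bounces run out.
; Final hits check lifesteal and slow, then deal direct, explosive or over-time damage with knockback before destroying it.
; Traces gate DamageSphere hits by line of sight and supply ricochet normals.
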(event OnComponentBeginOverlap(Physical)
  (params (OverlappedComponent :type Primitive%20Component%20Object%20Reference) (OtherActor :type Actor%20Object%20Reference) (OtherComp :type Primitive%20Component%20Object%20Reference) (OtherBodyIndex :type Integer) (bFromSweep :type Boolean) (SweepResult :type Hit%20Result%20Structure%20%28by%20ref%29))
  (bind _explosionradius (Variables|Default|GetExplosionRadius))
  (bind _output_get (Variables|Default|SetOther%20Actor OtherActor))
  (Variables|Default|SetOther%20Comp OtherComp)
  (if (not (== _output_get (Variables|Actor|GetInstigator)))
    (if (Components|ComponentHasTag (Variables|Default|GetOther%20Comp) "Shield")
      (CallFunction|ReflectVelocity (Variables|Actor|GetInstigator) "0, 0, 0")
      (bind _aspawn (Utilities|Casting|CastToPawn (Variables|Default|GetOther%20Actor)))
      (Variables|Actor|SetInstigator _aspawn)
      (CallFunction|UpdatetoInstigatorColour)
      (else
        (bind _controller (Class|BPICharacterandController|GetPlayerController(Message) (Variables|Actor|GetInstigator)))
        (Variables|Default|SetController _controller)
        (if (Actor|ActorHasTag (Variables|Default|GetOther%20Actor) "Player")
          (if (>= _explosionradius 1.0) :!label _label
            ;[0.7826 0.306 0.04561 0.5] Explode
            (CallFunction|Explosion (* _explosionradius 2.5e+02) (Variables|Default|GetController)))
          ;[1 0 0.04524 0.5] Lifesteal
          (CallFunction|CheckLifesteal)
          ;[0.1252 0.4176 0.5521 0.5] Slowonhit
          (CallFunction|CheckSlow)
          (if (>= (Variables|Default|GetDamageOverTime) 1.0)
            (if (>= (Variables|Default|GetExplosionRadius) 1.0)
              _
              (else
                (bind _returnvalue (AddComponent|AddBPCProjectileDOT (Variables|Default|GetOther%20Actor)))
                (Default|Init _returnvalue (Variables|Default|GetDamage) (* (Variables|Default|GetDamageOverTime) 3.0) self (Variables|Default|GetController))
                (Development|PrintString "Has DoT")
                (Class|BPIProjectileInterface|DealKnockback(Message) (Variables|Default|GetOther%20Actor) (* 1e+01 (Variables|Default|GetKnockbackMultiplier)) (- (Transformation|GetActorLocation (Variables|Default|GetOther%20Actor)) (Math|Vector|Normalize (Variables|/Script/Engine.MovementComponent|GetVelocity (Variables|Default|GetProjectileMovement)))))
                (CallFunction|OnDestroyProjectileEffects)))
            (Actor|DestroyActor)
            (else
              (if (>= (Variables|Default|GetExplosionRadius) 1.0)
                _
                (else
                  (CallFunction|ApplyNormalDamage)
                  (CallFunction|OnDestroyProjectileEffects)))
              (Actor|DestroyActor)))
          (else
            ;[0.8542 0.8542 0.8542 0.5] Ricochet
            (if (>= (Variables|Default|GetTimesBounced) (Variables|Default|GetRicochetCount))
              (goto _label)
              (else
                (CallFunction|Barrier)
                (CallFunction|Ricochet)))))))))

(event OnComponentBeginOverlap(DamageSphere)
  (params (OverlappedComponent :type Primitive%20Component%20Object%20Reference) (OtherActor :type Actor%20Object%20Reference) (OtherComp :type Primitive%20Component%20Object%20Reference) (OtherBodyIndex :type Integer) (bFromSweep :type Boolean) (SweepResult :type Hit%20Result%20Structure%20%28by%20ref%29))
  (bind _explosionradius (Variables|Default|GetExplosionRadius))
  (bind _output_get (Variables|Default|SetOther%20Actor OtherActor))
  (Variables|Default|SetOther%20Comp OtherComp)
  (bind _returnvalue (CallFunction|CanSeeTarget))
  (if _returnvalue
    (if (not (== _output_get (Variables|Actor|GetInstigator)))
      (if (Components|ComponentHasTag (Variables|Default|GetOther%20Comp) "Shield")
        (CallFunction|ReflectVelocity (Variables|Actor|GetInstigator) "0, 0, 0")
        (bind _aspawn (Utilities|Casting|CastToPawn (Variables|Default|GetOther%20Actor)))
        (Variables|Actor|SetInstigator _aspawn)
        (CallFunction|UpdatetoInstigatorColour)
        (else
          (bind _controller (Class|BPICharacterandController|GetPlayerController(Message) (Variables|Actor|GetInstigator)))
          (Variables|Default|SetController _controller)
          (if (Actor|ActorHasTag (Variables|Default|GetOther%20Actor) "Player")
            (if (>= _explosionradius 1.0) :!label _label
              ;[0.7826 0.306 0.04561 0.5] Explode
              (CallFunction|Explosion (* _explosionradius 2.5e+02) (Variables|Default|GetController)))
            ;[1 0 0.04524 0.5] Lifesteal
            (CallFunction|CheckLifesteal)
            ;[0.1252 0.4176 0.5521 0.5] Slowonhit
            (CallFunction|CheckSlow)
            (if (>= (Variables|Default|GetDamageOverTime) 1.0)
              (if (>= (Variables|Default|GetExplosionRadius) 1.0)
                _
                (else
                  (bind _returnvalue_2 (AddComponent|AddBPCProjectileDOT (Variables|Default|GetOther%20Actor)))
                  (Default|Init _returnvalue_2 (Variables|Default|GetDamage) (* (Variables|Default|GetDamageOverTime) 3.0) self (Variables|Default|GetController))
                  (Development|PrintString "Has DoT")
                  (Class|BPIProjectileInterface|DealKnockback(Message) (Variables|Default|GetOther%20Actor) (* 1e+01 (Variables|Default|GetKnockbackMultiplier)) (- (Transformation|GetActorLocation (Variables|Default|GetOther%20Actor)) (Math|Vector|Normalize (Variables|/Script/Engine.MovementComponent|GetVelocity (Variables|Default|GetProjectileMovement)))))
                  (CallFunction|OnDestroyProjectileEffects)))
              (Actor|DestroyActor)
              (else
                (if (>= (Variables|Default|GetExplosionRadius) 1.0)
                  _
                  (else
                    (CallFunction|ApplyNormalDamage)
                    (CallFunction|OnDestroyProjectileEffects)))
                (Actor|DestroyActor)))
            (else
              ;[0.8542 0.8542 0.8542 0.5] Ricochet
              (if (>= (Variables|Default|GetTimesBounced) (Variables|Default|GetRicochetCount))
                (goto _label)
                (else
                  (CallFunction|Barrier)
                  (CallFunction|Ricochet))))))))))

(event Custom|Initialize
  (params (Damage :type Float%20%28double-precision%29) (DamageOverTime :type Float%20%28double-precision%29) (Knockback :type Float%20%28double-precision%29) (RicochetCount :type Float%20%28double-precision%29) (ExplosionRadiusMulti :type Float%20%28double-precision%29) (ReflectMultiplier :type Float%20%28double-precision%29) (ProjectileSize :type Float%20%28double-precision%29) (Speed :type Float%20%28double-precision%29) (Range :type Float%20%28double-precision%29))
  (bind _returnvalue (/ Speed 3e+03))
  (bind _returnvalue_2 (* _returnvalue _returnvalue))
  (bind _output_get (Variables|Default|SetFirstInstigator (Variables|Actor|GetInstigator)))
  (bind _id (Class|BPICharacterandController|GetID(Message) _output_get))
  (Variables|Default|SetInstigatorID _id)
  (Variables|Default|SetDamage Damage)
  (Variables|Default|SetDamageOverTime DamageOverTime)
  (Variables|Default|SetKnockbackMultiplier Knockback)
  (Variables|Default|SetRicochetCount RicochetCount)
  (Variables|Default|SetExplosionRadius ExplosionRadiusMulti)
  (Variables|Default|SetReflectMultiplier ReflectMultiplier)
  (bind _output_get_2 (Variables|Default|SetProjectileSize ProjectileSize))
  (Utilities|SetSpeed Speed)
  (Utilities|SetProjectileSize _output_get_2)
  (Variables|Default|SetRange Range)
  (Actor|SetLifeSpan Range)
  (Utilities|NormalizeVelocity Speed)
  (Collision|SetCollisionEnabled (Variables|Default|GetDamageSphere) "QueryOnly")
  (Utilities|IsValid (Variables|Default|GetNiagara)
    (:Is%20Valid
      (Niagara|SetNiagaraVariable(Float) (Variables|Default|GetNiagara) "Trail Max Furiosity" (/ (Variables|Default|GetDamage) 25.0))
      (Niagara|SetNiagaraVariable(Float) (Variables|Default|GetNiagara) "Electricity Length" (* _returnvalue_2 1e+02))
      (Niagara|SetNiagaraVariable(Float) (Variables|Default|GetNiagara) "Trail Max Length" (* _returnvalue_2 3e+02))
      (Niagara|SetNiagaraVariable(Float) (Variables|Default|GetNiagara) "Helix Length" (* _returnvalue_2 0.75))
      (Niagara|SetNiagaraVariable(Float) (Variables|Default|GetNiagara) "Luminance" (* (/ (Variables|Default|GetDamage) 25.0) 1e+01))
      (CallFunction|UpdatetoInstigatorColour))))

(event Custom|UpdateToInstigatorColour
  (bind _id (Class|BPICharacterandController|GetID(Message) (Variables|Actor|GetInstigator)))
  (Niagara|SetNiagaraVariable(LinearColor) (Variables|Default|GetNiagara) "Orb Colour" (.Orb%20Colour (CallFunction|GetPlayerVFXColours _id)))
  (Niagara|SetNiagaraVariable(LinearColor) (Variables|Default|GetNiagara) "Friction Colour" (.Friction%20Colour (CallFunction|GetPlayerVFXColours _id)))
  (Niagara|SetNiagaraVariable(LinearColor) (Variables|Default|GetNiagara) "Primary Colour" (.Primary%20Colour (CallFunction|GetPlayerVFXColours _id)))
  (Niagara|SetNiagaraVariable(LinearColor) (Variables|Default|GetNiagara) "Secondary Colour" (.Secondary%20Colour (CallFunction|GetPlayerVFXColours _id))))

(event Custom|OnDestroyProjectileEffects
  (Audio|SpawnSound2D "/Game/Audio/SFX/MetaSounds/MS_SpellHit.MS_SpellHit" 1.0 1.0 0.0 0)
  (bind _returnvalue (Niagara|SpawnSystematLocation "/Game/Tech/Effects/VFX/Explosions/Spell/NS_SpellHit.NS_SpellHit" (Transformation|GetActorLocation) (Transformation|GetActorRotation) (Transformation|GetActorScale3D)))
  (CallFunction|HitCloudColour _returnvalue)
  (CallFunction|Barrier))

(event Custom|Hit%20Cloud%20Colour
  (params (Target :type Niagara%20Component%20Object%20Reference))
  (bind _id (Class|BPICharacterandController|GetID(Message) (Variables|Actor|GetInstigator)))
  (Niagara|SetNiagaraVariable(LinearColor) Target "Highlight Secondary Colour" (.Secondary%20Colour (CallFunction|GetPlayerVFXColours _id)))
  (Niagara|SetNiagaraVariable(LinearColor) Target "Fog Colour" (.Primary%20Colour (CallFunction|GetPlayerVFXColours _id))))

(event EventDamageMultiplier
  (params (Multiplier :type Float%20%28double-precision%29))
  (Variables|Default|SetDamage (* (Variables|Default|GetDamage) Multiplier)))

(fn ConstructionScript)

(fn ReflectDuplication)

(fn ReflectVelocity
  (params (Target :type Actor%20Object%20Reference) (AddRotation :type Rotator))
  (bind _projectilemovement (Variables|Default|GetProjectileMovement))
  (Utilities|IsValid Target
    (:Is%20Valid
      (bind _returnvalue (Collision|LineTraceByChannel (Transformation|GetActorLocation Target) (Transformation|GetActorLocation self) "TraceTypeQuery1" false 0 "None"))
      (if _returnvalue
        (Variables|/Script/Engine.MovementComponent|SetVelocity _projectilemovement (* (Variables|/Script/Engine.MovementComponent|GetVelocity _projectilemovement) -1.0) :!label _label)
        (else
          (Variables|/Script/Engine.MovementComponent|SetVelocity (Variables|Default|GetProjectileMovement) (* (Math|Vector|GetForwardVector (Math|Rotator|CombineRotators (Math|Rotator|FindLookatRotation (Transformation|GetActorLocation self) (Transformation|GetActorLocation Target)) AddRotation)) (Class|MovementComponent|GetMaxSpeed (Variables|Default|GetProjectileMovement))))
          (Development|PrintString "REFLECT"))))
    (:Is%20Not%20Valid
      (goto _label))))

(fn CheckLifesteal
  (bind _instigator (Variables|Actor|GetInstigator))
  (bind _returnvalue (Actor|GetComponentbyClass _instigator "/Game/Tech/Blueprints/BP_AttackComponent.BP_AttackComponent_C"))
  ;[0.15 0.025 0.025 0.5] Lifesteal
  (Utilities|IsValid _returnvalue
    (:Is%20Valid
      (if (> (Variables|/Game/Tech/Blueprints/BP_AttackComponent.BP_AttackComponent_C|GetLifestealPercentage _returnvalue) 0.0)
        (Default|ProvideLifesteal _returnvalue (Variables|Default|GetDamage))
        (Development|PrintString "Has Lifesteal")))))

(fn Ricochet
  (bind _returnvalue (Transformation|GetActorLocation))
  (bind _projectilemovement (Variables|Default|GetProjectileMovement))
  (bind _projectilemovement_2 (Variables|Default|GetProjectileMovement))
  (bind (_outhit _returnvalue_2) (Collision|SphereTraceByChannel (- _returnvalue (* (Transformation|GetActorForwardVector) 2e+01)) _returnvalue 75.0 "TraceTypeQuery1" true 0 "ForDuration" true "(R=1.000000,G=0.000000,B=0.000000,A=1.000000)" "(R=0.134144,G=0.000000,B=1.000000,A=1.000000)" 0.3))
  (if _returnvalue_2
    (Variables|/Script/Engine.MovementComponent|SetVelocity _projectilemovement_2 (Math|Vector|SelectVector (* (Variables|/Script/Engine.MovementComponent|GetVelocity _projectilemovement_2) -1.0) (* (Math|Vector|VectorLength (Math|Vector|MirrorVectorbyNormal (Variables|/Script/Engine.MovementComponent|GetVelocity _projectilemovement_2) (.impactnormal _outhit))) (Class|KismetMathLibrary|VectorNormal2D (Math|Vector|MirrorVectorbyNormal (Variables|/Script/Engine.MovementComponent|GetVelocity _projectilemovement_2) (.impactnormal _outhit)) 0.0001)) (Utilities|Operators|EqualEqual :A (Class|KismetMathLibrary|VectorNormal2D (Math|Vector|MirrorVectorbyNormal (Variables|/Script/Engine.MovementComponent|GetVelocity _projectilemovement_2) (.impactnormal _outhit)) 0.0001))))
    (if (Utilities|Operators|EqualEqual (Variables|Default|GetPrevVelocity) (Variables|/Script/Engine.MovementComponent|GetVelocity _projectilemovement_2) 0.1)
      (Variables|/Script/Engine.MovementComponent|SetVelocity _projectilemovement (* (Variables|/Script/Engine.MovementComponent|GetVelocity _projectilemovement) -1.0))
      (else
        (Variables|Default|SetPrevVelocity (Variables|/Script/Engine.MovementComponent|GetVelocity _projectilemovement))))
    (Transformation|SetActorLocation (- (.location _outhit) (* (Math|Vector|Normalize (.location _outhit)) (LocalVariables|GetOffsetAmount))) false false)
    (Math|Float|IncrementFloat (Variables|Default|GetTimesBounced))))

(fn Explosion
  (params (Radius :type Float%20%28double-precision%29) (EventInstigator :type Controller%20Object%20Reference))
  (bind _returnvalue (Transformation|GetActorLocation))
  (bind _instigatorid (Variables|Default|GetInstigatorID))
  (bind _player_colour (CallFunction|GetPlayerVibrantColour _instigatorid))
  (bind _outhits (Collision|MultiSphereTraceForObjects _returnvalue _returnvalue Radius (Utilities|Array|MakeArray (Utilities|Enum|LiteralenumEObjectTypeQuery "ObjectTypeQuery3")) false 0 "None" true "(R=1.000000,G=0.000000,B=0.000000,A=1.000000)" "(R=0.000000,G=1.000000,B=0.000000,A=1.000000)" 0.2))
  (Audio|SpawnSound2D "/Game/Audio/SFX/SoundFile/SW_Explosion.SW_Explosion" 1.0 1.0 0.0 0)
  (bind _returnvalue_2 (Niagara|SpawnSystematLocation "/Game/Tech/Effects/VFX/Explosions/Spell/NS_SpellExplosionExample.NS_SpellExplosionExample" (Transformation|GetActorLocation) "0, 0, 0" (Math|Conversions|ToVector(Float) (Variables|Default|GetExplosionRadius))))
  (Niagara|SetNiagaraVariable(LinearColor) _returnvalue_2 "Highlight Secondary Colour" _player_colour)
  (Niagara|SetNiagaraVariable(LinearColor) _returnvalue_2 "Highlight Primary Colour" _player_colour)
  (Niagara|SetNiagaraVariable(LinearColor) _returnvalue_2 "Fog Colour" (CallFunction|GetPlayerColour _instigatorid))
  (bind _array_element (Utilities|Array|ForEachLoopwithBreak _outhits)
    (:LoopBody
      (if (not (== (.HitActor (Collision|BreakHitResult _array_element)) (Variables|Actor|GetInstigator)))
        (Class|BPIProjectileInterface|DealKnockback(Message) (.HitActor (Collision|BreakHitResult _array_element)) (* 1e+01 (Variables|Default|GetKnockbackMultiplier)) (Transformation|GetActorLocation))
        (if (>= (Variables|Default|GetDamageOverTime) 1.0)
          (bind _returnvalue_3 (AddComponent|AddBPCProjectileDOT (Variables|Default|GetOther%20Actor)))
          (Default|Init _returnvalue_3 (Variables|Default|GetDamage) (* (Variables|Default|GetDamageOverTime) 3.0) self (Variables|Default|GetController))
          (else
            (Game|Damage|ApplyDamage (.HitActor (Collision|BreakHitResult _array_element)) (Variables|Default|GetDamage) EventInstigator self)
            (Development|PrintString "Hello")))))))

(fn ApplyNormalDamage
  (bind _other_actor (Variables|Default|GetOther%20Actor))
  (Game|Damage|ApplyDamage (Variables|Default|GetOther%20Actor) (Variables|Default|GetDamage) (Variables|Default|GetController) self)
  (Class|BPIProjectileInterface|DealKnockback(Message) _other_actor (* 1e+01 (Variables|Default|GetKnockbackMultiplier)) (- (Transformation|GetActorLocation _other_actor) (Math|Vector|Normalize (Variables|/Script/Engine.MovementComponent|GetVelocity (Variables|Default|GetProjectileMovement))))))

(fn CheckSlow
  (bind _other_actor (Variables|Default|GetOther%20Actor))
  (bind _instigator (Variables|Actor|GetInstigator))
  (bind _returnvalue (Actor|GetComponentbyClass _instigator "/Game/Tech/Blueprints/BP_AttackComponent.BP_AttackComponent_C"))
  (bind _returnvalue_2 (Actor|GetComponentbyClass _other_actor "/Game/Tech/Blueprints/BP_AttackComponent.BP_AttackComponent_C"))
  (bind _slowonhit (Variables|/Game/Tech/Blueprints/BP_AttackComponent.BP_AttackComponent_C|GetSlowOnHit _returnvalue))
  ;[0.05445 0.15 0.1497 0.5] Slow On HIT
  (if (> _slowonhit 0.0)
    (Utilities|IsValid _returnvalue_2
      (:Is%20Valid
        (Default|HitSlow _returnvalue_2 _slowonhit)
        (Development|PrintString "Has Slow")))))

(fn Barrier
  (bind _physical (Variables|Default|GetPhysical))
  (bind _returnvalue (Transformation|GetWorldLocation _physical))
  (if (Actor|ActorHasTag (Variables|Default|GetOther%20Actor) "Barrier")
    (bind _outhit (Collision|SphereTraceByChannel _returnvalue (+ _returnvalue (* (Class|KismetMathLibrary|VectorNormal2D (Variables|/Script/Engine.MovementComponent|GetVelocity (Variables|Default|GetProjectileMovement)) 0.0001) 5e+01)) (Variables|/Script/Engine.SphereComponent|GetSphereRadius (Variables|Default|GetDamageSphere)) "TraceTypeQuery1" false 0 "None" true "(R=1.000000,G=0.000000,B=0.000000,A=1.000000)" "(R=0.000000,G=1.000000,B=0.000000,A=1.000000)" 0.3))
    (Niagara|SpawnSystematLocation "/Game/Tech/VFX/NS_ProjectileBarrier.NS_ProjectileBarrier" (- (Transformation|GetActorLocation self) (* (.impactnormal _outhit) 5e+01)) (Math|Conversions|RotationFromXVector (.impactnormal _outhit)))))

(fn CanSeeTarget
  (bind _returnvalue (Collision|LineTraceByChannel (Transformation|GetActorLocation) (Transformation|GetActorLocation (Variables|Default|GetOther%20Actor)) "TraceTypeQuery1" false (Utilities|Array|MakeArray (Variables|Actor|GetInstigator) (Variables|Default|GetOther%20Actor)) "None"))
  (Development|PrintString (Utilities|String|ToString(Boolean) (not _returnvalue)))
  (return (not _returnvalue)))

(fn GetProjectileRef
  (return self))

(fn GetVariables
  (return (Utilities|Struct|MakeS_ProjectileID (Variables|Default|GetDamage) (Variables|Default|GetDamageOverTime) (Variables|Default|GetKnockbackMultiplier) (Variables|Default|GetRicochetCount) (Variables|Default|GetExplosionRadius) (Variables|Default|GetReflectMultiplier) (Variables|Default|GetProjectileSize) (Variables|Default|GetSpeed) (Variables|Default|GetRange))))

(fn IsClone
  (return (Variables|Default|GetIsClone_)))