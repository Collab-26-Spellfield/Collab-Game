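; Player attack component that fires light and charged projectiles from a firepoint, using references and owner ID set in Init.
; Light shots fire only at zero MultishotCount; both shot types pass combat stats to the projectile and share a timer cooldown shown on the player's spatial UI.
; Charging slows movement and disables block and dash until release, which fires a larger, stronger shot if charged long enough.
; Also provides a timed hit slow and damage-based lifesteal.
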(event Custom|Charging%20state
  (params (timecharged :type Float%20%28double-precision%29))
  (bind _playerref (Variables|Default|GetPlayerref))
  ;[0.06076 0.05806 0.15 0.5 30] Hold down charged shot
  (Variables|Default|SetCanBlock false)
  (Variables|/Game/Design/Blueprints/Character/BP_PlayerCharacter.BP_PlayerCharacter_C|SetCan%20Dash _playerref false)
  (Utilities|FlowControl|Sequence
    (:then_0
      (Utilities|FlowControl|DoOnce false
        (:Completed
          (Variables|/Game/Design/Blueprints/Character/BP_PlayerCharacter.BP_PlayerCharacter_C|SetMovespeed _playerref (Variables|Default|GetMoveSpeedWhileCharging)))))
    (:then_1
      (if (> timecharged 0.75)
        (Variables|Default|SetChargeReady true)))))

(event Custom|Init
  (params (Knockback%20Component :type BP%20Knockback%20Component%20Object%20Reference) (firepoint :type Arrow%20Component%20Object%20Reference) (player :type BP%20Player%20Character%20Object%20Reference) (Base%20movespeed :type Float%20%28double-precision%29))
  (Variables|Default|SetKnockback%20Component Knockback%20Component)
  (Variables|Default|SetFirepoint firepoint)
  (bind _output_get (Variables|Default|SetPlayerref player))
  (Variables|Default|SetBase%20Movespeed Base%20movespeed)
  (Variables|Default|SetOwnerId (Variables|/Game/Design/Blueprints/Character/BP_PlayerCharacter.BP_PlayerCharacter_C|GetMy%20ID _output_get)))

(event Custom|HitSlow
  (params (TimeSlowed :type Float%20%28double-precision%29))
  (bind _playerref (Variables|Default|GetPlayerref))
  (Variables|/Script/Engine.CharacterMovementComponent|SetMaxWalkSpeed (Variables|/Script/Engine.Character|GetCharacterMovement _playerref) (* (.MovementSpeed (Utilities|Struct|BreakMovementStats (Variables|/Game/Design/Blueprints/Character/BP_PlayerCharacter.BP_PlayerCharacter_C|GetBaseMovementStats _playerref))) 0.5))
  (Utilities|Time|SetTimerbyEvent (delegate Custom|SlowHit) TimeSlowed))

(event Custom|ResetCooldown
  ;[0.15 0.15 0.15 0.5] AttackCooldown
  (Variables|Default|SetCanShoot true))

(event Custom|Attack
  ;[0.02603 0.000177 0.15 0.5 30] Single shots
  (if (Variables|Default|GetCanShoot)
    (CallFunction|CooldownonAttack)
    (if (== (Variables|Default|GetMultishotCount) 0.0)
      (CallFunction|LightAttack))))

(event Custom|SlowHit
  (bind _playerref (Variables|Default|GetPlayerref))
  (Variables|/Script/Engine.CharacterMovementComponent|SetMaxWalkSpeed (Variables|/Script/Engine.Character|GetCharacterMovement _playerref) (.MovementSpeed (Utilities|Struct|BreakMovementStats (Variables|/Game/Design/Blueprints/Character/BP_PlayerCharacter.BP_PlayerCharacter_C|GetBaseMovementStats _playerref))))
  (Development|PrintString "Hello"))

(event Custom|Charged%20Shot
  (bind _playerref (Variables|Default|GetPlayerref))
  (bind _firepoint (Variables|Default|GetFirepoint))
  (bind _returnvalue (Transformation|GetWorldTransform _firepoint))
  (Utilities|FlowControl|Sequence
    (:then_0
      ;[0.06076 0.05806 0.15 0.5 30] Hold down charged shot
      (Variables|Default|SetCanBlock true)
      ;[0.03679 0.04058 0.15 0.5 30] release charged shot
      (if (Variables|Default|GetChargeReady)
        (Variables|Default|SetChargeReady false)
        (bind _returnvalue_2 (Game|SpawnActorfromClass (Variables|Default|GetProjectile) (Math|Transform|MakeTransform (.location _returnvalue) (.rotation _returnvalue) "2.000000,2.000000,2.000000") "Undefined" "MultiplyWithRoot" 0 (Game|Player|GetPlayerPawn (- (Variables|Default|GetOwnerId) 1))))
        (Utilities|IsValid _returnvalue_2
          (:Is%20Valid
            (Variables|/Game/Tech/Blueprints/BP_BaseProjectile.BP_BaseProjectile_C|Setdamage _returnvalue_2 (* (Variables|Default|GetAttackDamage) (Variables|Default|GetHeavyAttackMultiplier)))
            (CallFunction|CooldownonAttack)
            (Default|Initialize _returnvalue_2 (Variables|Default|GetProjectileSpeed) (Variables|Default|GetProjectileRange) (Variables|Default|GetProjectileSize) (Variables|Default|GetKnockbackMultiplier) (Variables|Default|GetRicochetCount))))))
    (:then_1
      (Variables|/Game/Design/Blueprints/Character/BP_PlayerCharacter.BP_PlayerCharacter_C|SetCan%20Dash _playerref true)
      (Variables|/Game/Design/Blueprints/Character/BP_PlayerCharacter.BP_PlayerCharacter_C|SetMovespeed _playerref (Variables|Default|GetBase%20Movespeed))
      (Utilities|FlowControl|DoOnce false) ; enters at Reset
    )))

(event Custom|CooldownOnAttack
  (bind _attackcooldown (Variables|Default|GetAttackCooldown))
  ;[0.15 0.15 0.15 0.5] AttackCooldown
  (Variables|Default|SetCanShoot false)
  (Utilities|Time|SetTimerbyEvent (delegate Custom|ResetCooldown) _attackcooldown)
  (Default|StartCooldown (Variables|/Game/UI/SpatialUI/WBP_SpatialPlayerUI.WBP_SpatialPlayerUI_C|GetAttackCooldown (Variables|/Game/Design/Blueprints/Character/BP_PlayerCharacter.BP_PlayerCharacter_C|GetSpatialUI (Variables|Default|GetPlayerref))) _attackcooldown))

(fn LightAttack
  (bind _firepoint (Variables|Default|GetFirepoint))
  (bind _returnvalue (Transformation|GetWorldTransform _firepoint))
  (bind _returnvalue_2 (Game|SpawnActorfromClass (Variables|Default|GetProjectile) (Math|Transform|MakeTransform (.location _returnvalue) (.rotation _returnvalue) "1.000000,1.000000,1.000000") "Undefined" "MultiplyWithRoot" 0 (Game|Player|GetPlayerPawn (Variables|Default|GetOwnerId))))
  (Utilities|IsValid _returnvalue_2
    (:Is%20Valid
      (Variables|/Game/Tech/Blueprints/BP_BaseProjectile.BP_BaseProjectile_C|Setdamage _returnvalue_2 (Variables|Default|GetAttackDamage))
      (Default|Initialize _returnvalue_2 (Variables|Default|GetProjectileSpeed) (Variables|Default|GetProjectileRange) (Variables|Default|GetProjectileSize) (Variables|Default|GetKnockbackMultiplier) (Variables|Default|GetRicochetCount)))))

(fn ProvideLifesteal
  (params (Damage :type Float%20%28double-precision%29))
  (Default|GainHealth (Variables|/Game/Design/Blueprints/Character/BP_PlayerCharacter.BP_PlayerCharacter_C|GetBP_HealthComponent (Variables|Default|GetPlayerref)) (* Damage (Variables|Default|GetLifestealPercentage))))