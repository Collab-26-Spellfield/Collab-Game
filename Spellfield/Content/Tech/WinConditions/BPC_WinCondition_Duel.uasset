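; BPC_WinCondition_Duel is a win condition component for a duel mode that ranks players by the order in which they die.
; Each death stores a descending DeathCounter as that player's position, then conditionally ends the game.
; EndGame stops the running state and calls GetWinners on the positions with lowest value winning.
; Setup only calls the parent implementation.
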(event Custom|OnPlayerDied
  (params (PlayerID :type Integer))
  ;[0.15 0.15 0.15 0.5] When a player dies, mark down their position
  (if (Variables|Default|GetIsGameRunning)
    (Utilities|Array|SetArrayElem (Variables|Default|GetPositions) PlayerID (Variables|Default|GetDeathCounter) true)
    (Math|Integer|DecrementInt (Variables|Default|GetDeathCounter)
      (:%20%20
        ;[0.15 0.15 0.15 0.5] Try and end the game
        (if true
          (CallFunction|EndGame))))))

(event Custom|EndGame
  ;[0.15 0.15 0.15 0.5] End game and distribute points
  (if (Variables|Default|GetIsGameRunning)
    (Variables|Default|SetIsGameRunning false)
    (CallFunction|GetWinners (Variables|Default|GetPositions) true)))

(fn SetupWinCondition
  (|CallParentFunction))