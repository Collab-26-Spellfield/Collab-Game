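; Timed win condition component that ranks players by generic points earned from the level's BP_BaseObjective actors.
; Setup binds each objective to GrantPoints and starts the game timer, whose expiry ends the game or enters overtime if leaders are tied.
; In overtime, GrantPoints calls EndGame when the tie check returns true, as wired.
; Final ranking breaks ties with an incrementing countback stamp, favoring whoever reached their score first.
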(event Custom|Grant%20Points
  (params (Player%20ID :type Integer) (Points%20to%20Grant :type Integer))
  ;[0.15 0.15 0.15 0.5] Called to grant points
  (if (Variables|Default|GetIsGameRunning)
    (Utilities|Array|SetArrayElem (Variables|Default|GetPoints) Player%20ID (+ (Utilities|Array|Get(acopy) (Variables|Default|GetPoints) Player%20ID) Points%20to%20Grant) true)
    ;[0.15 0.15 0.15 0.5] Countback records when the player took their last point, meaning if players are tied on points by the end, whomever has the lowest countback value got their current point value before the other player, making them win the tie.
    (Utilities|Array|SetArrayElem (Variables|Default|GetCountback) Player%20ID (Variables|Default|GetCountbackValue) true)
    (Math|Integer|IncrementInt (Variables|Default|GetCountbackValue)
      (:%20%20
        ;[0.15 0.15 0.15 0.5] Try and end the game if we're in overtime
        (if (Variables|Default|GetIsInOvertime)
          (bind _istied (CallFunction|AreWinnersTied (Variables|Default|GetPoints) false))
          (if _istied
            (CallFunction|EndGame)))))))

(event Custom|EndGame
  ;[0.15 0.15 0.15 0.5] End game and distribute points
  (if (Variables|Default|GetIsGameRunning)
    (Variables|Default|SetIsGameRunning false)
    (bind _winners (CallFunction|GetWinnerswithTiebreaker (Variables|Default|GetPoints) false (Variables|Default|GetCountback) true))
    (Default|CallDonConditionTrue (Utilities|Struct|MakeF_Ranking _winners))))

(event Custom|Start%20Game
  ;[0.15 0.15 0.15 0.5] Game timer
  (Utilities|Time|SetTimerbyEvent (delegate Custom|TryToEndGame) (Variables|Default|GetGame%20Time)))

(event Custom|TryToEndGame
  ;[0.15 0.15 0.15 0.5] If top 2 points are equal, go to overtime
  (bind _istied (CallFunction|AreWinnersTied (Variables|Default|GetPoints) false))
  (if _istied
    (Variables|Default|SetIsInOvertime true)
    (else
      (CallFunction|EndGame))))

(fn SetupWinCondition
  (|CallParentFunction)
  ;[0.15 0.15 0.15 0.5] Get all point assigning items in level and bind to them
  (bind _outactors (Actor|GetAllActorsOfClass "/Game/Design/LevelObjectives/BP_BaseObjective.BP_BaseObjective_C"))
  (for _array_element _outactors
    (EventDispatchers|BindEventtoGrantPoints _array_element (EventDispatchers|CreateEvent :!event Custom|Grant%20Points))
    (Default|Init _array_element))
  (CallFunction|StartGame))