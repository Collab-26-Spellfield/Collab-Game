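; Deathmatch win condition component that scores players on kills.
; Setup runs the parent logic, then loops over the game instance's player data map to bind an event to each player pawn's OnKill dispatcher.
; The kill handler grants the killer a point for killing another player while the game is running, and deducts one otherwise, including for self-kills.
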(event Custom|OnPlayerKilled
  (params (Killer%20ID :type Integer) (Killed%20ID :type Integer))
  (if (and (!= Killer%20ID Killed%20ID) (Variables|Default|GetIsGameRunning))
    (CallFunction|GrantPoints Killer%20ID 1)
    (else
      (CallFunction|GrantPoints Killer%20ID -1))))

(fn SetupWinCondition
  (|CallParentFunction)
  ;[0.15 0.15 0.15 0.5] Bind to handle kill
  (bind _playerconnectiondata (Class|BPIPlayerConnectionInfo|GetPlayerData(Message) (Game|GetGameInstance)))
  (bind _valuepin (Utilities|Map|ForEachLoop(Map) _playerconnectiondata)
    (:then
      (EventDispatchers|BindEventtoOnKill (.playerpawn _valuepin) (EventDispatchers|CreateEvent :!event Custom|OnPlayerKilled)))))