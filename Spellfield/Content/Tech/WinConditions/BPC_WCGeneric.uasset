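; Generic points-based win condition component for a timed game, with overridable GameStart and GameEnd events.
; It seeds points and a shuffled ranking from player data, creates the HUD, and binds every BP_BaseObjective to grant points, re-sorting the ranking incrementally.
; A modifier-dependent timer ends play, or enters sudden-death overtime while first place is tied.
; Ending notifies objectives, shows the end widget, then passes on the ranking after a delay.
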(event Custom|Grant%20Points
  (params (Player%20ID :type Integer) (Points%20to%20Grant :type Integer))
  ;[0.15 0.15 0.15 0.5] Called to grant points
  (if (Variables|Default|GetIsGameRunning)
    (Utilities|Map|Add (Variables|Default|GetGamePoints) Player%20ID (+ (.Value (Utilities|Map|Find (Variables|Default|GetGamePoints) Player%20ID)) Points%20to%20Grant))
    (CallFunction|UpdateRanking Player%20ID)
    (Default|OrderChanged (Variables|Default|GetUI) (Utilities|Struct|MakeS_ArrayOfInts (Variables|Default|GetRanking)))
    (Default|PointsChanged (Variables|Default|GetUI) (Variables|Default|GetGamePoints))
    ;[0.15 0.15 0.15 0.5] Try and end the game if we're in overtime
    (if (Variables|Default|GetIsOvertime)
      (bind _istied (CallFunction|AreWinnersTied (Variables|Default|GetGamePoints) false))
      (if (not _istied)
        (CallFunction|EndGame)))))

(event Custom|EndGame
  ;[0.15 0.15 0.15 0.5] End game and distribute points
  (if (Variables|Default|GetIsGameRunning)
    (Variables|Default|SetIsGameRunning false)
    (CallFunction|GameEnd)
    (bind _outactors (Actor|GetAllActorsOfClass "/Game/Design/LevelObjectives/BP_BaseObjective.BP_BaseObjective_C"))
    (for _array_element _outactors
      (Default|GameEnd _array_element))
    (Utilities|Time|SetTimerbyEvent (delegate Custom|Continue) 2.0)
    (bind _returnvalue (UserInterface|CreateWidget "/Game/UI/Player_HUD/WBP_GameEnd.WBP_GameEnd_C"))
    (UserInterface|Viewport|AddtoViewport _returnvalue 0)))

(event Custom|StartGameTimer
  (Utilities|Time|SetTimerbyEvent (delegate Custom|TryEndGame) (Variables|Default|GetGameLength))
  (Default|SetTimer (Variables|Default|GetUI) (Math|Float|Truncate (Variables|Default|GetGameLength))))

(event Custom|TryEndGame
  (bind _istied (CallFunction|AreWinnersTied (Variables|Default|GetGamePoints) false))
  (if _istied
    (Variables|Default|SetIsOvertime true)
    (Default|EnterOvertime (Variables|Default|GetUI))
    (else
      (CallFunction|EndGame))))

(event Custom|Game%20Start
  ;[0.15 0.15 0.15 0.5] Overridable
)

(event Custom|Game%20End
  ;[0.15 0.15 0.15 0.5] Overridable
)

(event Custom|Continue
  ;[0.15 0.15 0.15 0.5] End game and distribute points
  (Default|CallDonConditionTrue (Utilities|Struct|MakeF_Ranking (Variables|Default|GetRanking))))

(fn SetupWinCondition
  ;[0.15 0.15 0.15 0.5] SetupPoints
  (bind _playerconnectiondata (Class|BPIPlayerConnectionInfo|GetPlayerData(Message) (Game|GetGameInstance)))
  (bind _keypin (Utilities|Map|ForEachLoop(Map) _playerconnectiondata)
    (:then
      (Utilities|Map|Add (Variables|Default|GetGamePoints) _keypin 0)
      (Utilities|Array|Add (Variables|Default|GetRanking) _keypin))
    (:CompletedPin
      (Utilities|Array|Shuffle (Variables|Default|GetRanking))
      ;[0.15 0.15 0.15 0.5] Setup UI
      (bind _returnvalue (UserInterface|CreateWidget "/Game/UI/Player_HUD/WBP_HUDUI.WBP_HUDUI_C"))
      (UserInterface|Viewport|AddtoViewport _returnvalue -1)
      (Default|Init _returnvalue (Variables|Default|GetRanking))
      (Variables|Default|SetUI _returnvalue)
      (bind _isenabled (Class|BPIGameModifiers|IsModifierEnabled(Message) (Game|GetGameInstance) "NewEnumerator5"))
      (if _isenabled
        (Variables|Default|SetGameLength 4e+01)
        (else
          (Variables|Default|SetGameLength 6e+01)))
      (Default|ShowTimer (Variables|Default|GetUI) (Math|Float|Truncate (Variables|Default|GetGameLength))))))

(fn BeginGame
  (Variables|Default|SetIsGameRunning true)
  ;[0.15 0.15 0.15 0.5] Setup level objects
  (bind _outactors (Actor|GetAllActorsOfClass "/Game/Design/LevelObjectives/BP_BaseObjective.BP_BaseObjective_C"))
  (for _array_element _outactors
    (EventDispatchers|BindEventtoGrantPoints _array_element (EventDispatchers|CreateEvent :!event Custom|Grant%20Points))
    (Default|Init _array_element))
  (CallFunction|StartGameTimer)
  (CallFunction|GameStart))

(fn UnloadWinCondition
  (Widget|RemovefromParent (Variables|Default|GetUI)))

(fn GetWinnerswithTiebreaker
  (params (Points :type Map%20of%20Integers%20to%20Integers) (Lowest%20Wins :type Boolean) (Tiebreaker :type Map%20of%20Integers%20to%20Integers) (Lowest%20Breaks :type Boolean))
  (bind (_keypin _valuepin) (Utilities|Map|ForEachLoop(Map) Points)
    (:then
      (bind _index (Utilities|FlowControl|ForLoopwithBreak 0 (Utilities|Array|Length (LocalVariables|GetOrder)) :!label _label)
        (:LoopBody
          (if (< (Utilities|Array|LastIndex (LocalVariables|GetOrder)) _index)
            (Utilities|Array|Add (LocalVariables|GetOrder) _keypin)
            (goto _label Break)
            (elif (or (Class|KismetMathLibrary|XORBoolean (< (.Value (Utilities|Map|Find Points (Utilities|Array|Get(acopy) (LocalVariables|GetOrder) _index))) _valuepin) Lowest%20Wins) (and (== (.Value (Utilities|Map|Find Points (Utilities|Array|Get(acopy) (LocalVariables|GetOrder) _index))) _valuepin) (or (Class|KismetMathLibrary|XORBoolean (< (.Value (Utilities|Map|Find Tiebreaker (Utilities|Array|Get(acopy) (LocalVariables|GetOrder) _index))) (.Value (Utilities|Map|Find Tiebreaker _keypin))) Lowest%20Breaks) (and (== (.Value (Utilities|Map|Find Tiebreaker (Utilities|Array|Get(acopy) (LocalVariables|GetOrder) _index))) (.Value (Utilities|Map|Find Tiebreaker _keypin))) (Math|Random|RandomBool)))))
              (Utilities|Array|Insert (LocalVariables|GetOrder) _keypin _index)
              (goto _label Break))))))
    (:CompletedPin
      (return (LocalVariables|GetOrder)))))

(fn GetWinners
  (params (Points :type Map%20of%20Integers%20to%20Integers) (Lowest%20Wins :type Boolean))
  ;[0.15 0.15 0.15 0.5] With an array of points with index = player ID, return an ordererd list of player IDs. Ties resolved randomly.
  (bind (_keypin _valuepin) (Utilities|Map|ForEachLoop(Map) Points)
    (:then
      (bind _index (Utilities|FlowControl|ForLoopwithBreak 0 (Utilities|Array|Length (LocalVariables|GetOrder)) :!label _label)
        (:LoopBody
          (if (< (Utilities|Array|LastIndex (LocalVariables|GetOrder)) _index)
            (Utilities|Array|Add (LocalVariables|GetOrder) _keypin)
            (goto _label Break)
            (elif (or (Class|KismetMathLibrary|XORBoolean (< (.Value (Utilities|Map|Find Points (Utilities|Array|Get(acopy) (LocalVariables|GetOrder) _index))) _valuepin) Lowest%20Wins) (and (== (.Value (Utilities|Map|Find Points (Utilities|Array|Get(acopy) (LocalVariables|GetOrder) _index))) _valuepin) (Math|Random|RandomBool)))
              (Utilities|Array|Insert (LocalVariables|GetOrder) _keypin _index)
              (goto _label Break))))))
    (:CompletedPin
      (return (LocalVariables|GetOrder)))))

(fn AreWinnersTied
  (params (Points :type Map%20of%20Integers%20to%20Integers) (Lowest%20Wins :type Boolean))
  ;[0.15 0.15 0.15 0.5] Find winner
  (bind _winner (CallFunction|GetCurrentWinner Points Lowest%20Wins))
  (LocalVariables|SetWinner _winner)
  ;[0.15 0.15 0.15 0.5] Check if anyone is tied with winner
  (bind (_keypin _valuepin) (Utilities|Map|ForEachLoop(Map) Points)
    (:then
      (if (and (!= (LocalVariables|GetWinner) _keypin) (== (.Value (Utilities|Map|Find Points (LocalVariables|GetWinner))) _valuepin))
        (return true)))
    (:CompletedPin
      (return false))))

(fn GetCurrentWinner
  (params (Points :type Map%20of%20Integers%20to%20Integers) (Lowest%20Wins :type Boolean))
  (LocalVariables|SetCurrentWinner (.Key (Utilities|Map|GetKeyValueByIndex Points 0)))
  (bind (_keypin _valuepin) (Utilities|Map|ForEachLoop(Map) Points)
    (:then
      (if (Class|KismetMathLibrary|XORBoolean (< (.Value (Utilities|Map|Find Points (LocalVariables|GetCurrentWinner))) _valuepin) Lowest%20Wins)
        (LocalVariables|SetCurrentWinner _keypin)))
    (:CompletedPin
      (return (LocalVariables|GetCurrentWinner)))))

(fn UpdateRanking
  (params (IDToCheck :type Integer))
  (LocalVariables|SetMyIndex (Utilities|Array|FindItem (Variables|Default|GetRanking) IDToCheck))
  (if (< (LocalVariables|GetMyIndex) (Utilities|Array|LastIndex (Variables|Default|GetRanking)))
    (if (< (.Value (Utilities|Map|Find (Variables|Default|GetGamePoints) IDToCheck)) (.Value (Utilities|Map|Find (Variables|Default|GetGamePoints) (Utilities|Array|Get(acopy) (Variables|Default|GetRanking) (+ (LocalVariables|GetMyIndex) 1)))))
      (Utilities|Array|RemoveIndex (Variables|Default|GetRanking) (LocalVariables|GetMyIndex))
      (Utilities|Array|Insert (Variables|Default|GetRanking) IDToCheck (+ (LocalVariables|GetMyIndex) 1))
      (CallFunction|UpdateRanking IDToCheck)
      (else
        (if (> (LocalVariables|GetMyIndex) 0) :!label _label
          (if (> (.Value (Utilities|Map|Find (Variables|Default|GetGamePoints) IDToCheck)) (.Value (Utilities|Map|Find (Variables|Default|GetGamePoints) (Utilities|Array|Get(acopy) (Variables|Default|GetRanking) (- (LocalVariables|GetMyIndex) 1)))))
            (Utilities|Array|RemoveIndex (Variables|Default|GetRanking) (LocalVariables|GetMyIndex))
            (Utilities|Array|Insert (Variables|Default|GetRanking) IDToCheck (- (LocalVariables|GetMyIndex) 1))
            (CallFunction|UpdateRanking IDToCheck)))))
    (else
      (goto _label))))