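; Deathmatch win condition component that awards a point per non-suicide kill and ranks players when the match ends.
; Setup binds each player pawn's kill event, then starts the game timer, score maps and debug UI.
; A tie for the lead at time-up triggers overtime until a kill breaks it.
; Final ranking breaks ties by countback, an incrementing kill-order stamp favouring whoever reached their score first.
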(event Custom|OnPlayerKilled
  (params (Killer%20ID :type Integer) (Killed%20ID :type Integer))
  ;[0.15 0.15 0.15 0.5] If it wasn't a suicide, give the killer a point
  (if (!= Killer%20ID Killed%20ID)
    (if (Variables|Default|GetIsGameRunning)
      (Utilities|Map|Add (Variables|Default|GetPoints) Killer%20ID (+ (.Value (Utilities|Map|Find (Variables|Default|GetPoints) Killer%20ID)) 1))
      ;[0.15 0.15 0.15 0.5] Countback records when the player took their last kill, meaning if players are tied on kills by the end, whomever has the lowest countback value got their last before the other player, making them win the tie.
      (Utilities|Map|Add (Variables|Default|GetCountback) Killer%20ID (Variables|Default|GetCountbackValue))
      (Math|Integer|IncrementInt (Variables|Default|GetCountbackValue)
        (:%20%20
          (Default|PointsChanged (Variables|Default|GetUI) (Variables|Default|GetPoints))
          ;[0.15 0.15 0.15 0.5] Try and end the game if we're in overtime
          (if (Variables|Default|GetIsInOvertime)
            (bind _istied (CallFunction|AreWinnersTied (Variables|Default|GetPoints) false))
            (if (not _istied)
              (CallFunction|EndGame))))))))

(event Custom|EndGame
  ;[0.15 0.15 0.15 0.5] End game and distribute points
  (if (Variables|Default|GetIsGameRunning)
    (Variables|Default|SetIsGameRunning false)
    (bind _winners (CallFunction|GetWinnerswithTiebreaker (Variables|Default|GetPoints) false (Variables|Default|GetCountback) true))
    (Default|CallDonConditionTrue (Utilities|Struct|MakeF_Ranking _winners))))

(event Custom|Start%20Game
  ;[0.15 0.15 0.15 0.5] Game timer
  (Utilities|Time|SetTimerbyEvent (delegate Custom|TryToEndGame) (Variables|Default|GetGame%20Time))
  ;[0.15 0.15 0.15 0.5] Set up initial points
  (bind _playerconnectiondata (Class|BPIPlayerConnectionInfo|GetPlayerData(Message) (Game|GetGameInstance)))
  (bind _keypin (Utilities|Map|ForEachLoop(Map) _playerconnectiondata)
    (:then
      (Utilities|Map|Add (Variables|Default|GetPoints) _keypin 0)
      (Utilities|Map|Add (Variables|Default|GetCountback) _keypin 0)
      (bind _returnvalue (UserInterface|CreateWidget "/Game/UI/Player_HUD/Debug/WBP_DebugUI.WBP_DebugUI_C"))
      (UserInterface|Viewport|AddtoViewport _returnvalue 0)
      (Default|Init _returnvalue true)
      (Default|SetTimer _returnvalue (Math|Float|Truncate (Variables|Default|GetGame%20Time)))
      (Variables|Default|SetUI _returnvalue))))

(event Custom|TryToEndGame
  ;[0.15 0.15 0.15 0.5] If top 2 points are equal, go to overtime
  (bind _istied (CallFunction|AreWinnersTied (Variables|Default|GetPoints) false))
  (if _istied
    (Variables|Default|SetIsInOvertime true)
    (Default|EnterOvertime (Variables|Default|GetUI))
    (else
      (CallFunction|EndGame))))

(event Custom|HandleKill
  (params (Killer :type Integer) (Victim :type Integer))
  (CallFunction|OnPlayerKilled Killer Victim))

(fn SetupWinCondition
  (|CallParentFunction)
  (bind _playerconnectiondata (Class|BPIPlayerConnectionInfo|GetPlayerData(Message) (Game|GetGameInstance)))
  (bind _valuepin (Utilities|Map|ForEachLoop(Map) _playerconnectiondata)
    (:then
      (EventDispatchers|BindEventtoOnKill (.playerpawn _valuepin) (EventDispatchers|CreateEvent :!event Custom|HandleKill)))
    (:CompletedPin
      (CallFunction|StartGame))))

(fn UnloadWinCondition
  (|CallParentFunction)
  (Widget|RemovefromParent (Variables|Default|GetUI)))