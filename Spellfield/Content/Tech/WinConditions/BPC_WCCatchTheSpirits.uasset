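; Win condition component for a Catch the Spirits mode, where players earn points from collectible spirits.
; On game start it spawns three spirits per player at random spawner actors, then keeps spawning on a looping timer whose interval scales with player count.
; It binds to each pawn's death event; a death drops up to SpiritsLostOnDeath of the victim's points as new collectibles at that position and deducts them from their score.
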(event Custom|SpiritTimer
  (bind _spawnrate (Variables|Default|GetSpawnRate))
  (bind _returnvalue (* _spawnrate 1.3333))
  (if (Variables|Default|GetIsGameRunning)
    (CallFunction|SpawnSpirit)
    (Utilities|Time|SetTimerbyEvent (delegate Custom|SpiritTimer) (Math|Random|RandomFloatinRange _returnvalue _returnvalue))))

(event Custom|SpawnSpirit
  (Default|SpawnCollectible (.OutItem (Utilities|Array|Random (Variables|Default|GetSpawnLocations)))))

(event Custom|OnPlayerDied
  (params (Killer :type Integer) (Victim :type Integer))
  (bind _gamepoints (Variables|Default|GetGamePoints))
  (bind _spiritslostondeath (Variables|Default|GetSpiritsLostOnDeath))
  (bind _value (Utilities|Map|Find _gamepoints Victim))
  (bind _returnvalue (Math|Integer|Min(Integer) _value _spiritslostondeath))
  ;[0.15 0.15 0.15 0.5] Release up to 3 spirits on player death
  (if (Variables|Default|GetIsGameRunning)
    (bind _playerconnectiondata (Class|BPIPlayerConnectionInfo|GetPlayerData(Message) (Game|GetGameInstance)))
    (for _index (range 1 _returnvalue)
      (bind _returnvalue_2 (Game|SpawnActorfromClass "/Game/Design/LevelObjectives/BP_CollectibleObjective.BP_CollectibleObjective_C" (Math|Transform|MakeTransform (Math|Vector|MakeVector (.x (Transformation|GetActorLocation (.playerpawn (.Value (Utilities|Map|Find _playerconnectiondata Victim))))) (.y (Transformation|GetActorLocation (.playerpawn (.Value (Utilities|Map|Find _playerconnectiondata Victim))))) 5e+01) "0, 0, 0" "1.000000,1.000000,1.000000") "Undefined" "MultiplyWithRoot" 0 0))
      (EventDispatchers|BindEventtoGrantPoints _returnvalue_2 (EventDispatchers|CreateEvent :!event GrantPoints))
      (Default|Init _returnvalue_2))
    (CallFunction|GrantPoints Victim (* _returnvalue -1))))

(event EventGameStart
  (bind _spawnrate (Variables|Default|GetSpawnRate))
  (bind _returnvalue (* _spawnrate 1.3333))
  (bind _connectedplayercount (Class|BPIPlayerConnectionInfo|GetPlayerCount(Message) (Game|GetGameInstance)))
  (for _index (range 1 (* _connectedplayercount 3))
    (CallFunction|SpawnSpirit))
  (Utilities|Time|SetTimerbyEvent (delegate Custom|SpiritTimer) (Math|Random|RandomFloatinRange _returnvalue _returnvalue)))

(fn SetupWinCondition
  (|CallParentFunction)
  (bind _connectedplayercount (Class|BPIPlayerConnectionInfo|GetPlayerCount(Message) (Game|GetGameInstance)))
  (Variables|Default|SetSpawnRate (/ _connectedplayercount 1.5))
  ;[0.15 0.15 0.15 0.5] Bind to handle kill
  (bind _playerconnectiondata (Class|BPIPlayerConnectionInfo|GetPlayerData(Message) (Game|GetGameInstance)))
  (bind _valuepin (Utilities|Map|ForEachLoop(Map) _playerconnectiondata)
    (:then
      (EventDispatchers|BindEventtoOnDeath (.playerpawn _valuepin) (EventDispatchers|CreateEvent :!event Custom|OnPlayerDied)))
    (:CompletedPin
      (bind _outactors (Actor|GetAllActorsOfClass "/Game/Design/LevelObjectives/BP_CollectibleObjectiveSpawner.BP_CollectibleObjectiveSpawner_C"))
      (Variables|Default|SetSpawnLocations _outactors))))