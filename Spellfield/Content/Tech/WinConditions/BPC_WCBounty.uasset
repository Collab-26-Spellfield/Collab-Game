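; Bounty win condition component that scores players on survival and kills during a match.
; A looping one-second timer, started at game start and cleared at game end, grants a point to every living player.
; Setup extends the parent win condition and binds to each pawn's kill event.
; While the game runs, kills transfer half the victim's points to the killer, and suicides lose half, with a one-point minimum.
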(event Custom|OnPlayerKilled
  (params (Killer%20ID :type Integer) (Killed%20ID :type Integer))
  (bind _gamepoints (Variables|Default|GetGamePoints))
  (bind _value (Utilities|Map|Find _gamepoints Killed%20ID))
  (bind _returnvalue (/ _value 2))
  (bind _returnvalue_2 (Math|Integer|Max(Integer) _returnvalue 1))
  ;[0.15 0.15 0.15 0.5] Killer takes half the victim's points. On suicide, lose half points.
  (if (Variables|Default|GetIsGameRunning)
    (if (or (!= Killer%20ID Killed%20ID) (== Killer%20ID -1))
      (CallFunction|GrantPoints Killer%20ID _returnvalue_2)
      (CallFunction|GrantPoints Killed%20ID (* _returnvalue_2 -1))
      (else
        (CallFunction|GrantPoints Killed%20ID (Math|Integer|Min(Integer) (/ (.Value (Utilities|Map|Find (Variables|Default|GetGamePoints) Killed%20ID)) -2) -1))))))

(event Custom|StartPointsTimer
  (bind _returnvalue (Utilities|Time|SetTimerbyEvent (delegate Custom|GrantPoints) 1.0 true))
  (Variables|Default|SetPointsTimer _returnvalue))

(event Custom|GrantPoints
  (bind _playerconnectiondata (Class|BPIPlayerConnectionInfo|GetPlayerData(Message) (Game|GetGameInstance)))
  (bind (_keypin _valuepin) (Utilities|Map|ForEachLoop(Map) _playerconnectiondata)
    (:then
      (if (not (Variables|/Game/Design/Blueprints/Character/BP_PlayerCharacter.BP_PlayerCharacter_C|GetIsDead (.playerpawn _valuepin)))
        (CallFunction|GrantPoints _keypin 1)))))

(event Custom|EndPointsTimer
  (Utilities|Time|ClearandInvalidateTimerbyHandle (Variables|Default|GetPointsTimer)))

(event EventGameStart
  (CallFunction|StartPointsTimer))

(event EventGameEnd
  (CallFunction|EndPointsTimer))

(fn SetupWinCondition
  (|CallParentFunction)
  ;[0.15 0.15 0.15 0.5] Bind to handle kill
  (bind _playerconnectiondata (Class|BPIPlayerConnectionInfo|GetPlayerData(Message) (Game|GetGameInstance)))
  (bind _valuepin (Utilities|Map|ForEachLoop(Map) _playerconnectiondata)
    (:then
      (EventDispatchers|BindEventtoOnKill (.playerpawn _valuepin) (EventDispatchers|CreateEvent :!event Custom|OnPlayerKilled)))))