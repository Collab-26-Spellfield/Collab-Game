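; Base win condition component that provides setup and unload hooks plus shared helpers for ranking players from score maps.
; Setup only flags the game as running, and Unload is an empty stub.
; GetWinners functions insertion-sort player IDs by points, high or low, breaking ties randomly or by a secondary map first.
; GetCurrentWinner scans for the leader, which AreWinnersTied uses to check for a shared top score.
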(fn SetupWinCondition
  (Variables|Default|SetIsGameRunning true))

(fn UnloadWinCondition)

(fn GetWinnerswithTiebreaker
  (params (Points :type Map%20of%20Integers%20to%20Integers) (Lowest%20Wins :type Boolean) (Tiebreaker :type Map%20of%20Integers%20to%20Integers) (Lowest%20Breaks :type Boolean))
  (bind (_keypin _valuepin) (Utilities|Map|ForEachLoop(Map) Points)
    (:then
      (bind _index (Utilities|FlowControl|ForLoopwithBreak 0 (Utilities|Array|Length (LocalVariables|GetOrder)) :!label _label)
        (:LoopBody
          (if (< (Utilities|Array|LastIndex (LocalVariables|GetOrder)) _index)
            (Utilities|Array|Add (LocalVariables|GetOrder) _keypin)
            (goto _label Break)
            (elif (or (Class|KismetMathLibrary|XORBoolean (< (.Value (Utilities|Map|Find Points (Utilities|Array|Get(acopy) (LocalVariables|GetOrder) _index))) _valuepin) Lowest%20Wins) (and (== (.Value (Utilities|Map|Find Points (Utilities|Array|Get(acopy) (LocalVariables|GetOrder) _index))) _valuepin) (or (Class|KismetMathLibrary|XORBoolean (< (.Value (Utilities|Map|Find Tiebreaker (Utilities|Array|Get(acopy) (LocalVariables|GetOrder) _index))) (.Value (Utilities|Map|Find Tiebreaker _keypin))) Lowest%20Breaks) (and (== (.Value (Utilities|Map|Find Tiebreaker (Utilities|Array|Get(acopy) (LocalVariables|GetOrder) _index))) (.Value (Utilities|Map|Find Tiebreaker _keypin))) (Math|Random|RandomBool)))))
              (Utilities|Array|Insert (LocalVariables|GetOrder) _keypin _index)
              (goto _label Break))))))
    (:CompletedPin
      (return (LocalVariables|GetOrder)))))

(fn GetWinners
  (params (Points :type Map%20of%20Integers%20to%20Integers) (Lowest%20Wins :type Boolean))
  ;[0.15 0.15 0.15 0.5] With an array of points with index = player ID, return an ordererd list of player IDs. Ties resolved randomly.
  (bind (_keypin _valuepin) (Utilities|Map|ForEachLoop(Map) Points)
    (:then
      (bind _index (Utilities|FlowControl|ForLoopwithBreak 0 (Utilities|Array|Length (LocalVariables|GetOrder)) :!label _label)
        (:LoopBody
          (if (< (Utilities|Array|LastIndex (LocalVariables|GetOrder)) _index)
            (Utilities|Array|Add (LocalVariables|GetOrder) _keypin)
            (goto _label Break)
            (elif (or (Class|KismetMathLibrary|XORBoolean (< (.Value (Utilities|Map|Find Points (Utilities|Array|Get(acopy) (LocalVariables|GetOrder) _index))) _valuepin) Lowest%20Wins) (and (== (.Value (Utilities|Map|Find Points (Utilities|Array|Get(acopy) (LocalVariables|GetOrder) _index))) _valuepin) (Math|Random|RandomBool)))
              (Utilities|Array|Insert (LocalVariables|GetOrder) _keypin _index)
              (goto _label Break))))))
    (:CompletedPin
      (return (LocalVariables|GetOrder)))))

(fn AreWinnersTied
  (params (Points :type Map%20of%20Integers%20to%20Integers) (Lowest%20Wins :type Boolean))
  ;[0.15 0.15 0.15 0.5] Find winner
  (bind _winner (CallFunction|GetCurrentWinner Points Lowest%20Wins))
  (LocalVariables|SetWinner _winner)
  ;[0.15 0.15 0.15 0.5] Check if anyone is tied with winner
  (bind _valuepin (Utilities|Map|ForEachLoop(Map) Points)
    (:then
      (if (and (!= (LocalVariables|GetWinner) _valuepin) (== (.Value (Utilities|Map|Find Points (LocalVariables|GetWinner))) _valuepin))
        (return true)))
    (:CompletedPin
      (return false))))

(fn GetCurrentWinner
  (params (Points :type Map%20of%20Integers%20to%20Integers) (Lowest%20Wins :type Boolean))
  (LocalVariables|SetCurrentWinner (.Key (Utilities|Map|GetKeyValueByIndex Points 0)))
  (bind (_keypin _valuepin) (Utilities|Map|ForEachLoop(Map) Points)
    (:then
      (if (Class|KismetMathLibrary|XORBoolean (< (.Value (Utilities|Map|Find Points (LocalVariables|GetCurrentWinner))) _valuepin) Lowest%20Wins)
        (LocalVariables|SetCurrentWinner _keypin)))
    (:CompletedPin
      (return (LocalVariables|GetCurrentWinner)))))