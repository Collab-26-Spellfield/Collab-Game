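; Win condition component for a points race, ending the game when the leading player reaches the target score.
; Setup binds every BP_BaseObjective in the level to point granting, then zeroes each player's score and creates debug UI.
; Each grant updates the score and UI, and stamps the player with an incrementing countback.
; At game end it broadcasts a ranking, breaking ties in favour of whoever reached their score first.
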(event Custom|Grant%20Points
  (params (Player%20ID :type Integer) (Points%20to%20Grant :type Integer))
  ;[0.15 0.15 0.15 0.5] Called to grant points
  (if (Variables|Default|GetIsGameRunning)
    (Utilities|Map|Add (Variables|Default|GetPoints) Player%20ID (+ (.Value (Utilities|Map|Find (Variables|Default|GetPoints) Player%20ID)) Points%20to%20Grant))
    ;[0.15 0.15 0.15 0.5] Countback records when the player took their last point, meaning if players are tied on points by the end, whomever has the lowest countback value got their current point value before the other player, making them win the tie.
    (Utilities|Map|Add (Variables|Default|GetCountback) Player%20ID (Variables|Default|GetCountbackValue))
    (Math|Integer|IncrementInt (Variables|Default|GetCountbackValue)
      (:%20%20
        (Default|PointsChanged (Variables|Default|GetUI) (Variables|Default|GetPoints))
        ;[0.15 0.15 0.15 0.5] Try and end the game
        (bind _winner (CallFunction|GetCurrentWinner (Variables|Default|GetPoints) false))
        (if (>= (.Value (Utilities|Map|Find (Variables|Default|GetPoints) _winner)) (Variables|Default|GetPoints%20Needed%20To%20Win))
          (CallFunction|EndGame))))))

(event Custom|EndGame
  ;[0.15 0.15 0.15 0.5] End game and distribute points
  (if (Variables|Default|GetIsGameRunning)
    (Variables|Default|SetIsGameRunning false)
    (bind _winners (CallFunction|GetWinnerswithTiebreaker (Variables|Default|GetPoints) false (Variables|Default|GetCountback) true))
    (Default|CallDonConditionTrue (Utilities|Struct|MakeF_Ranking _winners))))

(event Custom|StartGame
  ;[0.15 0.15 0.15 0.5] Set up initial points
  (bind _playerconnectiondata (Class|BPIPlayerConnectionInfo|GetPlayerData(Message) (Game|GetGameInstance)))
  (bind _keypin (Utilities|Map|ForEachLoop(Map) _playerconnectiondata)
    (:then
      (Utilities|Map|Add (Variables|Default|GetPoints) _keypin 0)
      (Utilities|Map|Add (Variables|Default|GetCountback) _keypin 0)
      (bind _returnvalue (UserInterface|CreateWidget "/Game/UI/Player_HUD/Debug/WBP_DebugUI.WBP_DebugUI_C"))
      (UserInterface|Viewport|AddtoViewport _returnvalue 0)
      (Default|Init _returnvalue true)
      (Variables|Default|SetUI _returnvalue))))

(fn SetupWinCondition
  (|CallParentFunction)
  ;[0.15 0.15 0.15 0.5] Get all point assigning items in level and bind to them
  (bind _outactors (Actor|GetAllActorsOfClass "/Game/Design/LevelObjectives/BP_BaseObjective.BP_BaseObjective_C"))
  (for _array_element _outactors
    (EventDispatchers|BindEventtoGrantPoints _array_element (EventDispatchers|CreateEvent :!event Custom|Grant%20Points))
    (Default|Init _array_element))
  (CallFunction|StartGame))