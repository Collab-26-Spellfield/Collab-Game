(event Custom|OnPlayerKilled
  (params (Killer :type Integer) (Victim :type Integer))
  (bind _currentkingpin (Variables|Default|GetCurrentKingpin))
  ;[0.15 0.15 0.15 0.5] Handle player kills
  (if (and (!= Killer Victim) (Variables|Default|GetIsGameRunning))
    (if (or (== _currentkingpin Victim) (== _currentkingpin -1))
      (CallFunction|SetKingpin Killer)
      (CallFunction|GrantPoints Killer 3)
      (else
        (CallFunction|GrantPoints Killer 1)))
    (else
      (CallFunction|GrantPoints Killer (Math|Integer|SelectInt -3 -1 (== (Variables|Default|GetCurrentKingpin) Victim))))))

(event Custom|SetKingpin
  (params (PlayerID :type Integer))
  ;[0.15 0.15 0.15 0.5] Give the new kingpin the crown
  (Variables|Default|SetCurrentKingpin PlayerID)
  (Utilities|IsValid (Variables|Default|GetKingpin)
    (:Is%20Valid
      _)
    (:Is%20Not%20Valid
      (bind _returnvalue (Game|SpawnActorfromClass "/Game/Design/LevelObjectives/BP_KingpinCrown.BP_KingpinCrown_C" (Math|Transform|MakeTransform "0, 0, 0" "0, 0, 0" "1.000000,1.000000,1.000000") "Undefined" "MultiplyWithRoot" 0 0))
      (Variables|Default|SetKingpin _returnvalue)))
  (bind _playerconnectiondata (Class|BPIPlayerConnectionInfo|GetPlayerData(Message) (Game|GetGameInstance)))
  (Default|BindtoPlayer (Variables|Default|GetKingpin) (.playerpawn (.Value (Utilities|Map|Find _playerconnectiondata (Variables|Default|GetCurrentKingpin))))))

(fn SetupWinCondition
  (|CallParentFunction)
  ;[0.15 0.15 0.15 0.5] Bind to handle kill
  (bind _playerconnectiondata (Class|BPIPlayerConnectionInfo|GetPlayerData(Message) (Game|GetGameInstance)))
  (bind _valuepin (Utilities|Map|ForEachLoop(Map) _playerconnectiondata)
    (:then
      (EventDispatchers|BindEventtoOnKill (.playerpawn _valuepin) (EventDispatchers|CreateEvent :!event Custom|OnPlayerKilled)))))