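; BP_TestGamemode is a test game mode that boots a two-player session as soon as play begins.
; On BeginPlay it has the BPCPregame component load characters, then registers two players with the GameInstance.
; It then runs ResetPlayers and StartPlayers, which loop over the GameInstance's player data map and call ResetPlayer and StartGame on each player pawn.
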(event Custom|ResetPlayers
  (bind _playerconnectiondata (Class|BPIPlayerConnectionInfo|GetPlayerData(Message) (Game|GetGameInstance)))
  (bind _valuepin (Utilities|Map|ForEachLoop(Map) _playerconnectiondata)
    (:then
      (Default|ResetPlayer (.playerpawn _valuepin)))))

(event Custom|StartPlayers
  (bind _playerconnectiondata (Class|BPIPlayerConnectionInfo|GetPlayerData(Message) (Game|GetGameInstance)))
  (bind _valuepin (Utilities|Map|ForEachLoop(Map) _playerconnectiondata)
    (:then
      (Default|StartGame (.playerpawn _valuepin)))))

(event EventBeginPlay
  (bind _returnvalue (Game|GetGameInstance))
  (Default|LoadCharacters (Variables|Default|GetBPC_Pregame))
  (Class|BPIPlayerConnectionInfo|AddPlayertoGame(Message) _returnvalue)
  (Class|BPIPlayerConnectionInfo|AddPlayertoGame(Message) _returnvalue 1)
  (CallFunction|ResetPlayers)
  (CallFunction|StartPlayers))

(fn ConstructionScript)