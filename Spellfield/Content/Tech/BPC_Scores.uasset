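; Score-tracking component that keeps current and previous score objects for each player in the game instance's player data.
; IncreaseScores snapshots previous scores, then awards ranking points from a player-count table, scaled by a modifier that grows in later rounds.
; With three or more players, last round's last-place player earns an underdog bonus for finishing first.
; GetOldAndNewPoints returns old, new and difference maps; the points-to-win check does nothing yet.
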(event Custom|Increase%20Scores
  (params (Rankings :type Array%20of%20Integers))
  (bind _output (Utilities|Array|Get(acopy) Rankings))
  (bind _scores (Variables|Default|GetScores))
  (bind _value (Utilities|Map|Find _scores _output))
  (Utilities|FlowControl|Sequence
    (:then_0
      ;[0.15 0.15 0.15 0.5] Previous Score Update
      (bind (_keypin _valuepin) (Utilities|Map|ForEachLoop(Map) (Variables|Default|GetScores))
        (:then
          (Variables|/Game/Tech/BP_ScoreObject.BP_ScoreObject_C|SetScore (.Value (Utilities|Map|Find (Variables|Default|GetPrevious) _keypin)) (Variables|/Game/Tech/BP_ScoreObject.BP_ScoreObject_C|GetScore _valuepin)))))
    (:then_1
      ;[0.15 0.15 0.15 0.5] Underdog
      (if (and (> (Utilities|Array|Length Rankings) 2) (== _output (Variables|Default|GetUnderdog%20ID)))
        (Variables|/Game/Tech/BP_ScoreObject.BP_ScoreObject_C|SetScore _value (+ (Variables|/Game/Tech/BP_ScoreObject.BP_ScoreObject_C|GetScore _value) (Variables|Default|GetUnderdog%20Bonus)))))
    (:then_2
      ;[0.15 0.15 0.15 0.5] Modifier (Past 4 rounds and modifier increases)
      (if (> (Variables|Default|GetRound) 4)
        (Variables|Default|SetModifier (+ (Math|Float|Floor (/ (Math|Conversions|ToFloat(Integer) (- (Variables|Default|GetRound) 3)) 2.0)) 1))))
    (:then_3
      ;[0.15 0.15 0.15 0.5] Increase by rankings
      (for (_array_element _array_index) Rankings
        (bind _output_get (Variables|/Game/Tech/BP_ScoreObject.BP_ScoreObject_C|SetScore (.Value (Utilities|Map|Find (Variables|Default|GetScores) _array_element)) (+ (* (Utilities|Array|Get(acopy) (.array (.Value (Utilities|Map|Find (Variables|Default|GetScore%20Increases) (Utilities|Array|Length Rankings)))) _array_index) (Variables|Default|GetModifier)) (Variables|/Game/Tech/BP_ScoreObject.BP_ScoreObject_C|GetScore (.Value (Utilities|Map|Find (Variables|Default|GetScores) _array_element))))))
        ;;[0.15 0 0 0.5] Disconnected for now!
        (if (>= _output_get (Variables|Default|GetPoints%20To%20Win))
          _))
      (if (not (Variables|Default|GetEnd%20Loop?))
        (Math|Integer|IncrementInt (Variables|Default|GetRound)
          (:%20%20
            (Variables|Default|SetUnderdog%20ID (Utilities|Array|Get(acopy) Rankings (- (Utilities|Array|Length Rankings) 1)))))))))

(event EventBeginPlay
  (Utilities|FlowControl|DelayUntilNextTick)
  (bind _playerconnectiondata (Class|BPIPlayerConnectionInfo|GetPlayerData(Message) (Game|GetGameInstance)))
  (bind _keypin (Utilities|Map|ForEachLoop(Map) _playerconnectiondata)
    (:then
      (bind _returnvalue (Game|ConstructObjectfromClass "/Game/Tech/BP_ScoreObject.BP_ScoreObject_C"))
      (Utilities|Map|Add (Variables|Default|GetScores) _keypin _returnvalue)
      (bind _returnvalue_2 (Game|ConstructObjectfromClass "/Game/Tech/BP_ScoreObject.BP_ScoreObject_C"))
      (Utilities|Map|Add (Variables|Default|GetPrevious) _keypin _returnvalue_2))))

(fn GetOldandNewPoints
  (bind (_keypin _valuepin) (Utilities|Map|ForEachLoop(Map) (Variables|Default|GetScores))
    (:then
      (Utilities|Map|Add (LocalVariables|GetLocal%20New%20Points) _keypin (Variables|/Game/Tech/BP_ScoreObject.BP_ScoreObject_C|GetScore _valuepin)))
    (:CompletedPin
      (bind (_keypin_2 _valuepin_2) (Utilities|Map|ForEachLoop(Map) (Variables|Default|GetPrevious))
        (:then
          (Utilities|Map|Add (LocalVariables|GetLocal%20Old%20Points) _keypin_2 (Variables|/Game/Tech/BP_ScoreObject.BP_ScoreObject_C|GetScore _valuepin_2)))
        (:CompletedPin
          (bind (_keypin_3 _valuepin_3) (Utilities|Map|ForEachLoop(Map) (LocalVariables|GetLocal%20New%20Points))
            (:then
              (Utilities|Map|Add (LocalVariables|GetLocal%20Difference) _keypin_3 (- _valuepin_3 (.Value (Utilities|Map|Find (LocalVariables|GetLocal%20Old%20Points) _keypin_3)))))
            (:CompletedPin
              (return (LocalVariables|GetLocal%20Old%20Points) (LocalVariables|GetLocal%20New%20Points) (LocalVariables|GetLocal%20Difference)))))))))