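; Upgrade manager that draws random card upgrades and applies their stat modifiers to players.
; After a few ticks' delay at BeginPlay, it sorts data table cards into Common, Uncommon and Rare pools for rarity-weighted draws.
; AddCard stores cards per player ID, triggers stat recalculation and logs to the debug data grabber.
; Recalculation converts stat maps to structs, sums them field by field, then pushes the result to the pawn.
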(event Custom|LoadUpgrades
  ;[0.15 0.15 0.15 0.5] Init
  (bind _outrownames (DataTable|GetDataTableRowNames "/Game/Tech/UpgradeSystem/DT_CardStatsRevamped.DT_CardStatsRevamped"))
  (for _array_element _outrownames
    (bind _returnvalue (Utilities|GetDataTableRow "/Game/Tech/UpgradeSystem/DT_CardStatsRevamped.DT_CardStatsRevamped" _array_element)
      (:then
        (switch Utilities|FlowControl|Switch|SwitchonEUpgradeRarity (.rarity (.UpgradeDetails (Utilities|Struct|BreakS_CardStruct _returnvalue)))
          (:Common
            (Utilities|Array|Add (Variables|Default|GetCommonCards) _returnvalue))
          (:Uncommon
            (Utilities|Array|Add (Variables|Default|GetUncommonCards) _returnvalue))
          (:Rare
            (Utilities|Array|Add (Variables|Default|GetRareCards) _returnvalue)))))))

(event Custom|Init
  ;[0.15 0.15 0.15 0.5] BeginPlay
)

(event EventOnBecomeViewTarget
  (params (PC :type Player%20Controller%20Object%20Reference))
  ;[1 0.009212 0 1 185] DO NOT TOUCH
  (bind _outgoals (Class|IKGoalCreatorInterface|AddIKGoals(Message) PC))
  (if (Utilities|Map|Contains _outgoals "Alex Smith")
    (Class|GameplayStatics|AnnounceAccessibleString "ALEX SMITH")))

(event EventBeginPlay
  (Utilities|FlowControl|DelayUntilNextTick)
  (Utilities|FlowControl|DelayUntilNextTick)
  (Utilities|FlowControl|DelayUntilNextTick)
  (Utilities|FlowControl|DelayUntilNextTick)
  ;[0.15 0.15 0.15 0.5] BeginPlay
  (bind _asgi_game_instance_test (Utilities|Casting|CastToGI_GameInstanceTest (Game|GetGameInstance)))
  (Variables|Default|SetPlayer%20Connection%20Data (Variables|/Game/Tech/GI_GameInstanceTest.GI_GameInstanceTest_C|GetPlayerConnectionData _asgi_game_instance_test))
  (CallFunction|LoadUpgrades))

(fn ConstructionScript)

(fn AddStats
  (params (Player :type Character%20Stats%20Structure) (Card :type Character%20Stats%20Structure))
  (bind (_healthparameters _attackparameters _blockparameters _dashparameters _movementparameters _projectileparameters) (Utilities|Struct|BreakCharacterStats Player))
  (bind (_healthparameters_2 _attackparameters_2 _blockparameters_2 _dashparameters_2 _movementparameters_2 _projectileparameters_2) (Utilities|Struct|BreakCharacterStats Card))
  (bind _healthstats (Additive|HealthAddParams _healthparameters _healthparameters_2))
  (bind _attackstats (Additive|AttackAddParams _attackparameters _attackparameters_2))
  (bind _blockstats (Additive|BlockAddParams _blockparameters _blockparameters_2))
  (bind _dashstats (Additive|DashAddParams _dashparameters _dashparameters_2))
  (bind _movementstats (Additive|MovementAddParams _movementparameters _movementparameters_2))
  (bind _projectilestats (Additive|ProjectileAddParams _projectileparameters _projectileparameters_2))
  (return (Utilities|Struct|MakeCharacterStats _healthstats _attackstats _blockstats _dashstats _movementstats _projectilestats)))

(fn Renormalised)

(fn DashAddParams
  (params (Player :type Dash%20Stats%20Structure) (Card :type Dash%20Stats%20Structure))
  (bind (_dashspeed _dashcount _dashdistance _dashcooldownlength) (Utilities|Struct|BreakDashStats Player))
  (bind (_dashspeed_2 _dashcount_2 _dashdistance_2 _dashcooldownlength_2) (Utilities|Struct|BreakDashStats Card))
  (return (Utilities|Struct|MakeDashStats (+ _dashspeed _dashspeed_2) (+ _dashcount _dashcount_2) (+ _dashdistance _dashdistance_2) (+ _dashcooldownlength _dashcooldownlength_2))))

(fn ProjectileAddParams
  (params (Player :type Projectile%20Stats%20Structure) (Card :type Projectile%20Stats%20Structure))
  (bind (_projectiledamageparameters _projectilespeedmultiplier _projectilerangemultiplier _projectilesizemultiplier _projectilespreadbonus _explosionradiusmultiplier _knockbackgivenmultiplier _lifestealpercentage _slowonhit _lifesteal _penetration _ricochetcount _multishotbonus) (Utilities|Struct|BreakProjectileStats Card))
  (bind (_projectiledamageparameters_2 _projectilespeedmultiplier_2 _projectilerangemultiplier_2 _projectilesizemultiplier_2 _projectilespreadbonus_2 _explosionradiusmultiplier_2 _knockbackgivenmultiplier_2 _lifestealpercentage_2 _slowonhit_2 _lifesteal_2 _penetration_2 _ricochetcount_2 _multishotbonus_2) (Utilities|Struct|BreakProjectileStats Player))
  (return (Utilities|Struct|MakeProjectileStats (Utilities|Struct|MakeProjectileDamageStats (+ (.damagebonus _projectiledamageparameters_2) (.damagebonus _projectiledamageparameters)) (+ (.heavydamagebonus _projectiledamageparameters_2) (.heavydamagebonus _projectiledamageparameters)) (+ (.damageovertime _projectiledamageparameters_2) (.damageovertime _projectiledamageparameters))) (+ _projectilespeedmultiplier_2 _projectilespeedmultiplier) (+ _projectilerangemultiplier_2 _projectilerangemultiplier) (+ _projectilesizemultiplier_2 _projectilesizemultiplier) (+ _projectilespreadbonus_2 _projectilespreadbonus) (+ _explosionradiusmultiplier_2 _explosionradiusmultiplier) (+ _knockbackgivenmultiplier_2 _knockbackgivenmultiplier) (+ _lifestealpercentage_2 _lifestealpercentage) (+ _slowonhit_2 _slowonhit) (+ _lifesteal_2 _lifesteal) (+ _penetration_2 _penetration) (+ _ricochetcount_2 _ricochetcount) (+ _multishotbonus_2 _multishotbonus))))

(fn MovementAddParams
  (params (Player :type Movement%20Stats%20Structure) (Card :type Movement%20Stats%20Structure))
  (bind (_movementspeed _knockbackrecieved) (Utilities|Struct|BreakMovementStats Card))
  (bind (_movementspeed_2 _knockbackrecieved_2) (Utilities|Struct|BreakMovementStats Player))
  (return (Utilities|Struct|MakeMovementStats (+ _movementspeed_2 _movementspeed) (+ _knockbackrecieved_2 _knockbackrecieved))))

(fn AttackAddParams
  (params (Player :type Attack%20Stats%20Structure) (Card :type Attack%20Stats%20Structure))
  (bind (_attackcooldown _movementspeedwhilecharging) (Utilities|Struct|BreakAttackStats Card))
  (bind (_attackcooldown_2 _movementspeedwhilecharging_2) (Utilities|Struct|BreakAttackStats Player))
  (return (Utilities|Struct|MakeAttackStats (+ _attackcooldown_2 _attackcooldown) (+ _movementspeedwhilecharging_2 _movementspeedwhilecharging))))

(fn BlockAddParams
  (params (Player :type Block%20Stats%20Structure) (Card :type Block%20Stats%20Structure))
  (bind (_blockcooldownlength _blockradius _blockduration _lifestealpercentageonblock _blockdamage _reflecteddamagemultiplier) (Utilities|Struct|BreakBlockStats Card))
  (bind (_blockcooldownlength_2 _blockradius_2 _blockduration_2 _lifestealpercentageonblock_2 _blockdamage_2 _reflecteddamagemultiplier_2) (Utilities|Struct|BreakBlockStats Player))
  (return (Utilities|Struct|MakeBlockStats (+ _blockcooldownlength_2 _blockcooldownlength) (+ _blockradius_2 _blockradius) (+ _blockduration_2 _blockduration) (+ _lifestealpercentageonblock_2 _lifestealpercentageonblock) (+ _blockdamage_2 _blockdamage) (+ _reflecteddamagemultiplier_2 _reflecteddamagemultiplier))))

(fn HealthAddParams
  (params (Player :type Health%20Stats%20Structure) (Card :type Health%20Stats%20Structure))
  (bind (_maxhealth _healthregeneration) (Utilities|Struct|BreakHealthStats Player))
  (bind (_maxhealth_2 _healthregeneration_2) (Utilities|Struct|BreakHealthStats Card))
  (bind _returnvalue (+ _maxhealth _maxhealth_2))
  (Development|PrintString (Utilities|String|ToString(Float) _returnvalue))
  (return (Utilities|Struct|MakeHealthStats _returnvalue (+ _healthregeneration _healthregeneration_2))))

(fn AddCard
  (params (NewCard :type S%20Card%20Struct%20Structure%20%28by%20ref%29) (ID :type Integer))
  (bind _playercards (Variables|Default|GetPlayerCards))
  (bind _value (Utilities|Map|Find _playercards ID))
  (bind _cardsheld (Utilities|Struct|BreakS_PlayerCards _value))
  (bind _returnvalue (Utilities|Array|LastIndex _cardsheld))
  (bind _output (Utilities|Array|Get(acopy) _cardsheld _returnvalue))
  (bind _output_get (LocalVariables|SetNewUpgradeList (.cardsheld (.Value (Utilities|Map|Find (Variables|Default|GetPlayerCards) ID)))))
  (Utilities|Array|Add _output_get NewCard)
  (Utilities|Map|Add _playercards ID (Utilities|Struct|MakeS_PlayerCards (LocalVariables|GetNewUpgradeList)))
  (CallFunction|RecaulculateStats ID)
  (Class|DebugDataGrabber|UpdateCardDataforPlayeronRoundBasis (Subsystems|GetDebugDataGrabber) (Utilities|Struct|MakeCardStats (Utilities|Struct|MakeUpgrade (.rarity (.upgradedetails _output)) (.weighting (.upgradedetails _output)) (.upgradename (.upgradedetails _output)) (.flavortext (.upgradedetails _output))) "(MaxHealth=0.000000,HealthRegeneration=0.000000)" "(AttackCooldown=0.000000,MovementSpeedWhileCharging=0.000000)" "(BlockCooldownLength=0.000000,BlockRadius=0.000000,BlockDuration=0.000000,LifestealPercentageOnBlock=0.000000,BlockDamage=0.000000,ReflectedDamageMultiplier=0.000000)" "(DashSpeed=0.000000,DashCount=0.000000,DashDistance=0.000000,DashCooldownLength=0.000000)" "(MovementSpeed=0.000000,KnockbackRecieved=0.000000)" "(ProjectileDamageParameters=(DamageBonus=0.000000,HeavyDamageBonus=0.000000,DamageOverTime=0.000000),ProjectileSpeedMultiplier=0.000000,ProjectileRangeMultiplier=0.000000,ProjectileSizeMultiplier=0.000000,ProjectileSpreadBonus=0.000000,ExplosionRadiusMultiplier=0.000000,KnockbackGivenMultiplier=0.000000,LifeStealPercentage=0.000000,SlowOnHit=0.000000,Lifesteal=0.000000,Penetration=0.000000,RicochetCount=0.000000,MultishotBonus=0.000000)") ID true))

(fn RecaulculateStats
  (params (PlayerID :type Integer))
  (bind _player_connection_data (Variables|Default|GetPlayer%20Connection%20Data))
  (bind _value (Utilities|Map|Find _player_connection_data PlayerID))
  (for _array_element (.cardsheld (.Value (Utilities|Map|Find (Variables|Default|GetPlayerCards) PlayerID)))
    (bind _playerstats (CallFunction|AddStats (LocalVariables|GetPlayerStats) (CallFunction|CardtoCharacterStats _array_element)))
    (LocalVariables|SetPlayerStats _playerstats))
  (Variables|/Game/Design/Blueprints/Character/BP_PlayerCharacter.BP_PlayerCharacter_C|SetStatModifers (.playerpawn _value) (LocalVariables|GetPlayerStats))
  (Default|CallEDUpgradeAcquired (.playerpawn _value))
  (Default|SetVariablesfromStats (.playerpawn _value)))

(fn CardtoCharacterStats
  (params (CardStats :type S%20Card%20Struct%20Structure))
  (bind _statmap (Utilities|Struct|BreakS_CardStruct CardStats))
  (return (Utilities|Struct|MakeCharacterStats (Utilities|Struct|MakeHealthStats (.Value (Utilities|Map|Find (.statmap _statmap) "NewEnumerator0")) (.Value (Utilities|Map|Find (.statmap _statmap) "NewEnumerator20"))) (Utilities|Struct|MakeAttackStats (.Value (Utilities|Map|Find (.statmap _statmap) "NewEnumerator12")) 0.0) (Utilities|Struct|MakeBlockStats 0.0 (.Value (Utilities|Map|Find (.statmap _statmap) "NewEnumerator22")) 0.0 0.0 (.Value (Utilities|Map|Find (.statmap _statmap) "NewEnumerator19")) 0.0) (Utilities|Struct|MakeDashStats 0.0 (.Value (Utilities|Map|Find (.statmap _statmap) "NewEnumerator17")) 0.0 0.0) (Utilities|Struct|MakeMovementStats (.Value (Utilities|Map|Find (.statmap _statmap) "NewEnumerator10")) 0.0) (Utilities|Struct|MakeProjectileStats (Utilities|Struct|MakeProjectileDamageStats (.Value (Utilities|Map|Find (.statmap _statmap) "NewEnumerator9")) 0.0 0.0) (.Value (Utilities|Map|Find (.statmap _statmap) "NewEnumerator11")) 0.0 (.Value (Utilities|Map|Find (.statmap _statmap) "NewEnumerator18")) 0.0 0.0 (.Value (Utilities|Map|Find (.statmap _statmap) "NewEnumerator16")) (.Value (Utilities|Map|Find (.statmap _statmap) "NewEnumerator15")) (.Value (Utilities|Map|Find (.statmap _statmap) "NewEnumerator21")) 0.0 0.0 (.Value (Utilities|Map|Find (.statmap _statmap) "NewEnumerator13")) (.Value (Utilities|Map|Find (.statmap _statmap) "NewEnumerator14"))))))

(fn DrawRandomCards
  (params (CardsToDraw :type Integer))
  (bind _returnvalue (Math|Random|RandomFloatinRange 0.0 1.0))
  ;[0.15 0.15 0.15 0.5] Add in logic for other rarities and guaranteeing at least one rare and uncommon later...
  (Utilities|Array|Clear (LocalVariables|GetCardSelection))
  (for _index (range 1 CardsToDraw)
    (if (<= _returnvalue 0.15)
      (Variables|Default|SetTargetRarity "Rare")
      (elif (<= _returnvalue 0.45)
        (Variables|Default|SetTargetRarity "Uncommon")
        (else
          (Variables|Default|SetTargetRarity "Common"))))
    (switch Utilities|FlowControl|Switch|SwitchonEUpgradeRarity (Variables|Default|GetTargetRarity)
      (:Common
        (Utilities|Array|Add (LocalVariables|GetCardSelection) (.OutItem (Utilities|Array|Random (Variables|Default|GetCommonCards)))))
      (:Uncommon
        (Utilities|Array|Add (LocalVariables|GetCardSelection) (.OutItem (Utilities|Array|Random (Variables|Default|GetUncommonCards)))))
      (:Rare
        (Utilities|Array|Add (LocalVariables|GetCardSelection) (.OutItem (Utilities|Array|Random (Variables|Default|GetRareCards)))))))
  (Utilities|Array|Shuffle (LocalVariables|GetCardSelection))
  (return (LocalVariables|GetCardSelection)))