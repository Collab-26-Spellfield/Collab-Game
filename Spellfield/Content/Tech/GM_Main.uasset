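; Main game mode for a multiplayer party game, running the training-grounds lobby, a loop of minigame rounds and the return to the lobby.
; Rounds start with Death Match, then draw a random different, enabled mode and level from the Modes DataTable, with transition screens showing scores between them.
; Each mode adds its win-condition component at runtime, whose result updates BPCScores.
; Components handle level loading and music, and the final seconds trigger a blood moon.
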(event Custom|Load%20Gamemode
  (params (Level :type World%20Soft%20Object%20Reference) (Mode :type S%20Mode%20Data%20Structure))
  ;[0.15 0.15 0.15 0.5] Load new gamemode
  (bind _output_get (Variables|Default|SetCurrent%20Mode Mode))
  (Class|DebugDataGrabber|SetGameModeName (Subsystems|GetDebugDataGrabber) (Utilities|String|ToString(Name) (Utilities|Struct|BreakS_ModeData _output_get)))
  (Utilities|FlowControl|Sequence
    (:then_0
      ;;[0.15 0.15 0.15 0.5] Clear Previous
      (Utilities|IsValid (Variables|Default|GetCurrent%20Win%20Condition)
        (:Is%20Valid
          (Default|UnloadWinCondition (Variables|Default|GetCurrent%20Win%20Condition))
          (Components|DestroyComponent (Variables|Default|GetCurrent%20Win%20Condition)))))
    (:then_1
      (EventDispatchers|BindEventtoOnLevelLoadingComplete (Variables|Default|GetBPC_Level) (delegate Custom|OnLevelLoaded))
      (Default|LoadLevel (Variables|Default|GetBPC_Level) Level))))

(event Custom|OnLevelLoaded
  ;[0.15 0.15 0.15 0.5] Load new gamemode
  (EventDispatchers|UnbindEventfromOnLevelLoadingComplete (Variables|Default|GetBPC_Level) (delegate Custom|OnLevelLoaded))
  (CallFunction|AutoAssignSpawnPoints)
  (CallFunction|DefaultMoon)
  (bind _returnvalue (Game|AddComponentbyClass (Utilities|Struct|BreakS_ModeData (Variables|Default|GetCurrent%20Mode))))
  (Default|SetupWinCondition _returnvalue)
  (EventDispatchers|BindEventtoOnTimerTicked (Variables|/Game/UI/Player_HUD/WBP_HUDUI.WBP_HUDUI_C|GetWBP_Clock (Variables|/Game/Tech/WinConditions/BPC_WCGeneric.BPC_WCGeneric_C|GetUI _returnvalue)) (EventDispatchers|CreateEvent :!event Custom|TimerTicked))
  (EventDispatchers|BindEventtoDonConditionTrue _returnvalue (EventDispatchers|CreateEvent :!event Custom|Win%20Condition%20Returns%20True))
  (Variables|Default|SetCurrent%20Win%20Condition _returnvalue)
  (CallFunction|StopPlayers)
  (CallFunction|ResetPlayers)
  (Utilities|Time|SetTimerbyEvent (delegate Custom|Start%20Gamemode) 0.5))

(event Custom|AllowPlayerConnections
  ;[0.15 0.15 0.15 0.5] Player Handling
  (bind _playerconnectiondata (Class|BPIPlayerConnectionInfo|GetAllPlayerData(Message) (Game|GetGameInstance)))
  (bind _valuepin (Utilities|Map|ForEachLoop(Map) _playerconnectiondata)
    (:then
      (Default|AllowConnection (.playercontroller _valuepin))
      (Variables|/Game/Design/Blueprints/Character/BP_PlayerCharacter.BP_PlayerCharacter_C|SetHasGameStarted (.playerpawn _valuepin) false))))

(event Custom|GoToNewGamemode
  ;[0.15 0.15 0.15 0.5] Load the next gamemode
  (CallFunction|LoadGamemode (Variables|Default|GetNext%20Level) (Variables|Default|GetNext%20Mode))
  (Default|CombatMusic (Variables|Default|GetBPC_SoundtrackManager))
  (CallFunction|DefaultMoon))

(event Custom|BloodMoon
  (Default|CallSetMoon true))

(event Custom|DisallowPlayerConnections
  ;[0.15 0.15 0.15 0.5] Player Handling
  (bind _playerconnectiondata (Class|BPIPlayerConnectionInfo|GetAllPlayerData(Message) (Game|GetGameInstance)))
  (bind _valuepin (Utilities|Map|ForEachLoop(Map) _playerconnectiondata)
    (:then
      (Default|DisallowConnection (.playercontroller _valuepin)))))

(event Custom|Spawn%20Last%20Transition%20Screen
  (params (F_Ranking :type F%20Ranking%20Structure%20%28by%20ref%29))
  (bind _bpc_scores (Variables|Default|GetBPC_Scores))
  ;[0.15 0.15 0.15 0.5] Spawn First Transition Screen
  (bind _returnvalue (UserInterface|CreateWidget "/Game/UI/TransitionScreenUI/WBP_TransitionScreen.WBP_TransitionScreen_C"))
  (UserInterface|Viewport|AddtoViewport _returnvalue 0)
  (EventDispatchers|BindEventtoEContinueLoopProc _returnvalue (EventDispatchers|CreateEvent :!event Custom|GoToVictoryScene))
  (bind (_old_points _new_points _difference) (Default|GetOldandNewPoints (Variables|Default|GetBPC_Scores)))
  (Default|InitforFinalScores _returnvalue _old_points _difference (Variables|/Game/Tech/BPC_Scores.BPC_Scores_C|GetPoints%20To%20Win _bpc_scores) (Utilities|Struct|BreakF_Ranking F_Ranking) self (Variables|/Game/Tech/BPC_Scores.BPC_Scores_C|GetGrantedUnderdogTo _bpc_scores) (Variables|/Game/Tech/BPC_Scores.BPC_Scores_C|GetModifier _bpc_scores) _new_points)
  (Default|TransitionScreenMusic (Variables|Default|GetBPC_SoundtrackManager)))

(event Custom|DefaultMoon
  (Default|CallSetMoon false))

(event Custom|EnterTrainingGrounds
  ;[0.15 0.15 0.15 0.5] Enter the training grounds (main menu area)
  (Default|LobbyMusic (Variables|Default|GetBPC_SoundtrackManager))
  (CallFunction|AllowPlayerConnections)
  (bind _returnvalue (UserInterface|CreateWidget "/Game/UI/Player_HUD/WBP_TrainingGroundsHUD.WBP_TrainingGroundsHUD_C"))
  (UserInterface|Viewport|AddtoViewport _returnvalue 0)
  (Default|Init _returnvalue self)
  (Default|LoadLevel (Variables|Default|GetBPC_Level) (Variables|Default|GetStartMap))
  (EventDispatchers|BindEventtoOnLevelLoadingComplete (Variables|Default|GetBPC_Level) (delegate Custom|AfterLoadedTrainingGrounds))
  (CallFunction|PlayersGametoLobbySetVars)
  (CallFunction|DefaultMoon))

(event Custom|SpawnTransitionScreen
  (params (F_Ranking :type F%20Ranking%20Structure%20%28by%20ref%29))
  (bind _next_mode (Variables|Default|GetNext%20Mode))
  (bind _bpc_scores (Variables|Default|GetBPC_Scores))
  (bind (_displayname _description) (Utilities|Struct|BreakS_ModeData _next_mode))
  ;[0.15 0.15 0.15 0.5] Spawn Standard Transition Screen
  (bind _returnvalue (UserInterface|CreateWidget "/Game/UI/TransitionScreenUI/WBP_TransitionScreen.WBP_TransitionScreen_C"))
  (UserInterface|Viewport|AddtoViewport _returnvalue 0)
  (EventDispatchers|BindEventtoEContinueLoopProc _returnvalue (EventDispatchers|CreateEvent :!event Custom|GoToNewGamemode))
  (bind (_old_points _new_points _difference) (Default|GetOldandNewPoints (Variables|Default|GetBPC_Scores)))
  (Default|InitforScores _returnvalue _old_points _difference (Variables|/Game/Tech/BPC_Scores.BPC_Scores_C|GetPoints%20To%20Win _bpc_scores) _description (Utilities|Text|ToText(Name) _displayname) (Utilities|Struct|BreakF_Ranking F_Ranking) self (Variables|/Game/Tech/BPC_Scores.BPC_Scores_C|GetGrantedUnderdogTo _bpc_scores) (Variables|/Game/Tech/BPC_Scores.BPC_Scores_C|GetModifier _bpc_scores) (Variables|/Game/Tech/BPC_Scores.BPC_Scores_C|GetNextRoundModifier _bpc_scores) (Variables|/Game/Tech/BPC_Scores.BPC_Scores_C|GetRound _bpc_scores))
  (Default|TransitionScreenMusic (Variables|Default|GetBPC_SoundtrackManager)))

(event Custom|CompleteWinscreenTransition
  ;[0.15 0.15 0.15 0.5] Leave victory screen
  (EventDispatchers|UnbindEventfromOnLevelLoadingComplete (Variables|Default|GetBPC_Level) (delegate Custom|CompleteWinscreenTransition))
  (Widget|RemovefromParent (stale Custom|Leave%20Victory%20Screen _returnvalue))
  (bind _returnvalue (UserInterface|CreateWidget "/Game/UI/TransitionScreenUI/WBP_FadeFromBlack.WBP_FadeFromBlack_C"))
  (UserInterface|Viewport|AddtoViewport _returnvalue 0))

(event Custom|Spawn%20First%20Transition%20Screen
  (bind _next_mode (Variables|Default|GetNext%20Mode))
  (bind (_displayname _description) (Utilities|Struct|BreakS_ModeData _next_mode))
  ;[0.15 0.15 0.15 0.5] Spawn First Transition Screen
  (bind _returnvalue (UserInterface|CreateWidget "/Game/UI/TransitionScreenUI/WBP_TransitionScreen.WBP_TransitionScreen_C"))
  (UserInterface|Viewport|AddtoViewport _returnvalue 0)
  (EventDispatchers|BindEventtoEContinueLoopProc _returnvalue (EventDispatchers|CreateEvent :!event Custom|GoToNewGamemode))
  (Default|InitforNoScores _returnvalue _description (Utilities|Text|ToText(Name) _displayname) self)
  (Default|TransitionScreenMusic (Variables|Default|GetBPC_SoundtrackManager)))

(event Custom|After%20Countdown
  ;[0.15 0.15 0.15 0.5] Load new gamemode
  (CallFunction|StartPlayers)
  (Default|BeginGame (Variables|Default|GetCurrent%20Win%20Condition)))

(event Custom|InitPauseMenu
  (Utilities|IsValid (Variables|Default|GetPauseMenu)
    (:Is%20Not%20Valid
      (bind _returnvalue (UserInterface|CreateWidget "/Game/UI/PauseMenu/WBP_PauseMenu.WBP_PauseMenu_C"))
      (bind _output_get (Variables|Default|SetPauseMenu _returnvalue))
      (UserInterface|Viewport|AddtoViewport _output_get 0))))

(event Custom|GoToVictoryScene
  ;[0.15 0.15 0.15 0.5] Go to the podium area
  (Default|LobbyMusic (Variables|Default|GetBPC_SoundtrackManager))
  (Utilities|IsValid (Variables|Default|GetCurrent%20Win%20Condition)
    (:Is%20Valid
      (Default|UnloadWinCondition (Variables|Default|GetCurrent%20Win%20Condition))
      (Components|DestroyComponent (Variables|Default|GetCurrent%20Win%20Condition)))
    (:Is%20Not%20Valid
      _))
  (bind _returnvalue (Actor|GetActorOfClass "/Game/Tech/UpgradeSystem/BP_UpgradeManager.BP_UpgradeManager_C"))
  (Default|ClearUpgrades _returnvalue)
  (CallFunction|EnterTrainingGrounds))

(event Custom|ResetPlayers
  ;[0.15 0.15 0.15 0.5] Player Handling
  (bind _playerconnectiondata (Class|BPIPlayerConnectionInfo|GetPlayerData(Message) (Game|GetGameInstance)))
  (bind _valuepin (Utilities|Map|ForEachLoop(Map) _playerconnectiondata)
    (:then
      (Default|ResetPlayer (.playerpawn _valuepin)))))

(event Custom|TimerTicked
  (params (SecondsRemaining :type Integer))
  (if (<= SecondsRemaining 3)
    (CallFunction|BloodMoon)))

(event Custom|Leave%20Victory%20Screen
  ;[0.15 0.15 0.15 0.5] Leave victory screen
  (bind _returnvalue (UserInterface|CreateWidget "/Game/UI/TransitionScreenUI/WBP_FadeToBlack.WBP_FadeToBlack_C"))
  (EventDispatchers|BindEventtoOnComplete _returnvalue (delegate Custom|AfterVictoryScreenFade))
  (Variables|/Game/UI/TransitionScreenUI/WBP_FadeToBlack.WBP_FadeToBlack_C|SetAutoDestroy _returnvalue false)
  (UserInterface|Viewport|AddtoViewport _returnvalue 0))

(event Custom|AfterVictoryScreenFade
  ;[0.15 0.15 0.15 0.5] Leave victory screen
  (EventDispatchers|UnbindEventfromOnComplete (stale Custom|Leave%20Victory%20Screen _returnvalue) (delegate Custom|AfterVictoryScreenFade))
  (CallFunction|EnterTrainingGrounds)
  (EventDispatchers|BindEventtoOnLevelLoadingComplete (Variables|Default|GetBPC_Level) (delegate Custom|CompleteWinscreenTransition)))

(event Custom|AfterLoadedTrainingGrounds
  ;[0.15 0.15 0.15 0.5] Enter the training grounds (main menu area)
  (EventDispatchers|UnbindEventfromOnLevelLoadingComplete (Variables|Default|GetBPC_Level) (delegate Custom|AfterLoadedTrainingGrounds))
  (CallFunction|ResetPlayers)
  (CallFunction|InitPauseMenu))

(event Custom|MovePlayersToPodiums
  ;[0.15 0.15 0.15 0.5] Player Handling
  (bind _rankings (Default|GetRankings (Variables|Default|GetBPC_Scores)))
  (bind _playerconnectiondata (Class|BPIPlayerConnectionInfo|GetPlayerData(Message) (Game|GetGameInstance)))
  (bind (_keypin _valuepin) (Utilities|Map|ForEachLoop(Map) _playerconnectiondata)
    (:then
      (Default|SetupPlayerforWinscreen (.playerpawn _valuepin) (Utilities|Array|FindItem _rankings _keypin)))))

(event Custom|StopPlayers
  ;[0.15 0.15 0.15 0.5] Player Handling
  (bind _playerconnectiondata (Class|BPIPlayerConnectionInfo|GetPlayerData(Message) (Game|GetGameInstance)))
  (bind _valuepin (Utilities|Map|ForEachLoop(Map) _playerconnectiondata)
    (:then
      (Default|EndGame (.playerpawn _valuepin)))))

(event Custom|Win%20Condition%20Returns%20True
  (params (Rankings :type F%20Ranking%20Structure))
  ;[0.15 0.15 0.15 0.5] On winner found / level ended
  (CallFunction|StopPlayers)
  (Default|IncreaseScores (Variables|Default|GetBPC_Scores) (Utilities|Struct|BreakF_Ranking Rankings))
  (if (Variables|/Game/Tech/BPC_Scores.BPC_Scores_C|GetEnd%20Loop? (Variables|Default|GetBPC_Scores))
    (CallFunction|SpawnLastTransitionScreen Rankings)
    (else
      (CallFunction|DrawNewLevelandMode)
      (CallFunction|SpawnTransitionScreen Rankings))))

(event Custom|Start%20Gamemode
  ;[0.15 0.15 0.15 0.5] Load new gamemode
  (Utilities|Time|SetTimerbyEvent (delegate Custom|After%20Countdown) 3.0)
  (bind _returnvalue (UserInterface|CreateWidget "/Game/UI/Player_HUD/WBP_321Go.WBP_321Go_C"))
  (UserInterface|Viewport|AddtoViewport _returnvalue 0))

(event Custom|StartPlayers
  ;[0.15 0.15 0.15 0.5] Player Handling
  (bind _playerconnectiondata (Class|BPIPlayerConnectionInfo|GetPlayerData(Message) (Game|GetGameInstance)))
  (bind _valuepin (Utilities|Map|ForEachLoop(Map) _playerconnectiondata)
    (:then
      (Default|StartGame (.playerpawn _valuepin)))))

(event Custom|PlayersLobbyToGameSetVars
  ;[0.15 0.15 0.15 0.5] Player Handling
  (bind _playerconnectiondata (Class|BPIPlayerConnectionInfo|GetAllPlayerData(Message) (Game|GetGameInstance)))
  (bind _valuepin (Utilities|Map|ForEachLoop(Map) _playerconnectiondata)
    (:then
      (Default|SetPregame (.playerpawn _valuepin) false))))

(event Custom|PlayersGameToLobbySetVars
  ;[0.15 0.15 0.15 0.5] Player Handling
  (bind _playerconnectiondata (Class|BPIPlayerConnectionInfo|GetAllPlayerData(Message) (Game|GetGameInstance)))
  (bind _valuepin (Utilities|Map|ForEachLoop(Map) _playerconnectiondata)
    (:then
      (Default|SetPregame (.playerpawn _valuepin) true))))

(event EventBeginPlay
  ;[0.15 0.15 0.15 0.5] Begin initialisation chain
  (Default|Init (Variables|Default|GetBPC_SoundtrackManager) (Variables|Default|GetSoundtrack))
  (Default|LoadCharacters (Variables|Default|GetBPC_Pregame))
  (Class|GameplayStatics|LoadStreamLevelbySoftObjectPtr (Variables|Default|GetBackground) true false)
  (CallFunction|EnterTrainingGrounds))

(event EventBeginGame
  ;[0.15 0.15 0.15 0.5] Start the gameloop
  (CallFunction|DisallowPlayerConnections)
  (Default|InitScores (Variables|Default|GetBPC_Scores))
  (CallFunction|PlayersLobbytoGameSetVars)
  (bind _returnvalue (Utilities|GetDataTableRow (Variables|Default|GetModes) "Death_Match")
    (:then
      (CallFunction|DrawLevelforSpecificMode _returnvalue)
      (CallFunction|SpawnFirstTransitionScreen)
      (Default|CallLeftTrainingArea))))

(event EventSetScoretoWin
  (params (ScoreToWin :type Integer))
  ;[0.15 0.15 0.15 0.5] Player Handling
  (Variables|/Game/Tech/BPC_Scores.BPC_Scores_C|SetPoints%20To%20Win (Variables|Default|GetBPC_Scores) ScoreToWin))

(fn ConstructionScript)

(fn DrawNewLevelandMode
  (Variables|Default|SetNext%20Mode (Variables|Default|GetCurrent%20Mode))
  (while (or (== (.DisplayName (Utilities|Struct|BreakS_ModeData (Variables|Default|GetCurrent%20Mode))) (.DisplayName (Utilities|Struct|BreakS_ModeData (Variables|Default|GetNext%20Mode)))) (.IsDisabled (Utilities|Struct|BreakS_ModeData (Variables|Default|GetNext%20Mode))))
    (bind _outrownames (DataTable|GetDataTableRowNames (Variables|Default|GetModes)))
    (bind _returnvalue (Utilities|GetDataTableRow (Variables|Default|GetModes) (.OutItem (Utilities|Array|Random _outrownames)))
      (:then
        (Variables|Default|SetNext%20Mode _returnvalue)
        (bind _result (Math|Integer|IncrementInt (LocalVariables|GetDepth))
          (:%20%20
            (if (> _result 100)
              (Utilities|Debugging|RaiseScriptError "Couldn't draw a new gamemode!")
              (return 0 "")))))))
  (bind _output_get (Variables|Default|SetNext%20Level (.worldasset (.OutItem (Utilities|Array|Random (.Levels (Utilities|Struct|BreakS_ModeData (Variables|Default|GetNext%20Mode))))))))
  (return _output_get (Variables|Default|GetNext%20Mode)))

(fn DrawLevelforSpecificMode
  (params (NewMode :type S%20Mode%20Data%20Structure))
  (Variables|Default|SetNext%20Mode NewMode)
  (bind _output_get (Variables|Default|SetNext%20Level (.worldasset (.OutItem (Utilities|Array|Random (.Levels (Utilities|Struct|BreakS_ModeData (Variables|Default|GetNext%20Mode))))))))
  (return _output_get (Variables|Default|GetNext%20Mode)))

(fn AutoAssignSpawnPoints
  (bind _outactors (Actor|GetAllActorsOfClass "/Game/Tech/Blueprints/BP_PlayerSpawn.BP_PlayerSpawn_C"))
  (bind _output_get (LocalVariables|SetPlayer%20Spawners _outactors))
  (Utilities|Array|Shuffle _output_get)
  (bind (_array_element _array_index) (Utilities|Array|ForEachLoopwithBreak _output_get :!label _label)
    (:LoopBody
      (if (> _array_index 3)
        (goto _label Break)
        (else
          (Variables|/Game/Tech/Blueprints/BP_PlayerSpawn.BP_PlayerSpawn_C|SetPlayer%20ID _array_element _array_index))))))

(fn GetCurrentMode
  (return (Variables|Default|GetCurrent%20Mode)))

(fn GetGameMode
  (return self))

(fn GetScoretoWin
  (return (Variables|/Game/Tech/BPC_Scores.BPC_Scores_C|GetPoints%20To%20Win (Variables|Default|GetBPC_Scores))))

(fn GetSoundtrackManager
  (return (Variables|Default|GetBPC_SoundtrackManager)))

(fn GetWinCondition
  (return (Variables|Default|GetCurrent%20Win%20Condition)))