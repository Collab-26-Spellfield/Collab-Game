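; Soundtrack manager component that switches music between lobby, combat and transition-screen states, with victory currently reusing combat music.
; State events set target strengths, and a self-clearing looping timer ramps current values linearly toward them, feeding float parameters on one audio component.
; Init mutes the soundtrack to avoid a startup blip until LobbyMusic restores volume.
; Init also loads saved settings and applies master, music and SFX sound-mix overrides.
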(event Custom|CombatMusic
  (Variables|Default|SetTargetCombatStrength 1.0)
  (Variables|Default|SetTargetLobbyStrength 0.0)
  (CallFunction|StartTimer))

(event Custom|TransitionScreenMusic
  (Variables|Default|SetTargetCombatStrength 0.0)
  (Variables|Default|SetTargetLobbyStrength 0.0)
  (CallFunction|StartTimer))

(event Custom|LobbyMusic
  (Variables|Default|SetTargetCombatStrength 0.0)
  (Variables|Default|SetTargetLobbyStrength 1.0)
  (CallFunction|StartTimer)
  ;[0.15 0.15 0.15 0.5] Resets to 1 after audio mix set up
  (Audio|Components|Audio|SetVolumeMultiplier (Variables|Default|GetSoundtrack) 1.0 :!class /Script/Engine.AudioComponent))

(event Custom|StartTimer
  (bind _returnvalue (Utilities|Time|SetTimerbyEvent (delegate Custom|Update) 0.001 true true))
  (Variables|Default|SetTimer _returnvalue))

(event Custom|Update
  (Variables|Default|SetCurrentCombatStrength (Math|Float|SelectFloat (Variables|Default|GetTargetCombatStrength) (+ (* (Utilities|Time|GetWorldDeltaSeconds) (Math|Float|Sign(Float) (- (Variables|Default|GetTargetCombatStrength) (Variables|Default|GetCurrentCombatStrength)))) (Variables|Default|GetCurrentCombatStrength)) (!= (Math|Float|Sign(Float) (- (Variables|Default|GetTargetCombatStrength) (+ (* (Utilities|Time|GetWorldDeltaSeconds) (Math|Float|Sign(Float) (- (Variables|Default|GetTargetCombatStrength) (Variables|Default|GetCurrentCombatStrength)))) (Variables|Default|GetCurrentCombatStrength)))) (Math|Float|Sign(Float) (- (Variables|Default|GetTargetCombatStrength) (Variables|Default|GetCurrentCombatStrength))))))
  (Variables|Default|SetCurrentLobbyStrength (Math|Float|SelectFloat (Variables|Default|GetTargetLobbyStrength) (+ (* (Utilities|Time|GetWorldDeltaSeconds) (Math|Float|Sign(Float) (- (Variables|Default|GetTargetLobbyStrength) (Variables|Default|GetCurrentLobbyStrength)))) (Variables|Default|GetCurrentLobbyStrength)) (!= (Math|Float|Sign(Float) (- (Variables|Default|GetTargetLobbyStrength) (+ (* (Utilities|Time|GetWorldDeltaSeconds) (Math|Float|Sign(Float) (- (Variables|Default|GetTargetLobbyStrength) (Variables|Default|GetCurrentLobbyStrength)))) (Variables|Default|GetCurrentLobbyStrength)))) (Math|Float|Sign(Float) (- (Variables|Default|GetTargetLobbyStrength) (Variables|Default|GetCurrentLobbyStrength))))))
  (CallFunction|SetParameters)
  (if (and (== (Variables|Default|GetCurrentCombatStrength) (Variables|Default|GetTargetCombatStrength)) (== (Variables|Default|GetCurrentLobbyStrength) (Variables|Default|GetTargetLobbyStrength)))
    (Utilities|Time|ClearandInvalidateTimerbyHandle (Variables|Default|GetTimer))))

(event Custom|Init
  (params (Soundtrack :type Audio%20Component%20Object%20Reference))
  ;[0.15 0.15 0.15 0.5] Stops Audio Blip
  (Audio|Components|Audio|SetVolumeMultiplier Soundtrack 0.0 :!class /Script/Engine.AudioComponent)
  (CallFunction|LoadAudioSettings)
  (Variables|Default|SetSoundtrack Soundtrack)
  (CallFunction|SetParameters))

(event Custom|SetParameters
  (bind _soundtrack (Variables|Default|GetSoundtrack))
  (Audio|Parameter|SetFloatParameter _soundtrack "CombatMusic" (Variables|Default|GetCurrentCombatStrength) :!class /Script/AudioExtensions.AudioParameterControllerInterface)
  (Audio|Parameter|SetFloatParameter _soundtrack "LobbyMusic" (Variables|Default|GetCurrentLobbyStrength) :!class /Script/AudioExtensions.AudioParameterControllerInterface))

(event Custom|VictoryMusic
  ;[0.15 0.15 0.15 0.5] For now, use combat as victory
  (CallFunction|CombatMusic))

(fn LoadAudioSettings
  (Class|GameplayStatics|ClearSoundMixModifiers)
  (Utilities|IsValid (Variables|Default|GetSaveSettingsObj)
    (:Is%20Valid
      (Audio|SetSoundMixClassOverride "/Game/Audio/GenericSoundClass.GenericSoundClass" "/Game/Audio/MasterSound.MasterSound" 1.0 1.0 0.1 true)
      (Audio|SetSoundMixClassOverride "/Game/Audio/GenericSoundClass.GenericSoundClass" "/Game/Audio/MusicSound.MusicSound" 1.0 1.0 0.1 true)
      (Audio|SetSoundMixClassOverride "/Game/Audio/GenericSoundClass.GenericSoundClass" "/Game/Audio/SFXSound.SFXSound" 1.0 1.0 0.1 true)
      (Audio|PushSoundMixModifier "/Game/Audio/GenericSoundClass.GenericSoundClass")
      (return true (Variables|Default|GetSaveSettingsObj)))
    (:Is%20Not%20Valid
      (bind _returnvalue (SaveGame|CreateSaveGameObject "/Game/UI/PauseMenu/BP_SaveSettingsObject.BP_SaveSettingsObject_C"))
      (bind _returnvalue_2 (SaveGame|LoadGamefromSlot (Variables|/Game/UI/PauseMenu/BP_SaveSettingsObject.BP_SaveSettingsObject_C|GetSlotName _returnvalue) (Variables|/Game/UI/PauseMenu/BP_SaveSettingsObject.BP_SaveSettingsObject_C|GetUserIndex _returnvalue)))
      (bind _asbp_save_settings_object (Utilities|Casting|CastToBP_SaveSettingsObject _returnvalue_2)
        (:then
          (Variables|Default|SetSaveSettingsObj _asbp_save_settings_object))
        (:CastFailed
          (Variables|Default|SetSaveSettingsObj _returnvalue)))
      (Audio|SetSoundMixClassOverride "/Game/Audio/GenericSoundClass.GenericSoundClass" "/Game/Audio/MasterSound.MasterSound" (* (Variables|/Game/UI/PauseMenu/BP_SaveSettingsObject.BP_SaveSettingsObject_C|GetMasterVolumeAmount (Variables|Default|GetSaveSettingsObj)) 0.01) 1.0 0.1 true)
      (Audio|PushSoundMixModifier "/Game/Audio/GenericSoundClass.GenericSoundClass")
      (Audio|SetSoundMixClassOverride "/Game/Audio/GenericSoundClass.GenericSoundClass" "/Game/Audio/MusicSound.MusicSound" (* (Variables|/Game/UI/PauseMenu/BP_SaveSettingsObject.BP_SaveSettingsObject_C|GetMusicVolumeAmount (Variables|Default|GetSaveSettingsObj)) 0.01) 1.0 0.1 true)
      (Audio|PushSoundMixModifier "/Game/Audio/GenericSoundClass.GenericSoundClass")
      (Audio|SetSoundMixClassOverride (LocalVariables|GetIn%20Sound%20Mix%20Modifier) "/Game/Audio/SFXSound.SFXSound" (* (Variables|/Game/UI/PauseMenu/BP_SaveSettingsObject.BP_SaveSettingsObject_C|GetSFXVolumeAmount (Variables|Default|GetSaveSettingsObj)) 0.01) 1.0 0.1 true)
      (Audio|PushSoundMixModifier "/Game/Audio/GenericSoundClass.GenericSoundClass")
      (return false (Variables|Default|GetSaveSettingsObj)))))