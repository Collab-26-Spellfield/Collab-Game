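; BP_Moonlight controls the scene's moonlight, fading it between its regular look and a red blood moon.
; It caches the light's starting colour and intensity, then binds to GM_Main's SetMoon event to choose the target state.
; A looping timer steps a blend value at a state-specific rate without overshooting, lerping colour in HSV and intensity linearly until it reaches the target and clears itself.
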(event Custom|BloodMoon
  (Variables|Default|SetTargetValue 1.0)
  (CallFunction|SetMoonTimer)
  (Variables|Default|SetLerpTime 4.0))

(event Custom|RegularMoon
  (Variables|Default|SetTargetValue 0.0)
  (CallFunction|SetMoonTimer)
  (Variables|Default|SetLerpTime 1.0))

(event Custom|SetMoonTimer
  (bind _returnvalue (Utilities|Time|SetTimerbyEvent (delegate Custom|MoonTick) 0.01 true))
  (Variables|Default|SetMoonTimer _returnvalue))

(event Custom|MoonTick
  (Variables|Default|SetMoonValue (Math|Float|SelectFloat (Variables|Default|GetTargetValue) (+ (* (Utilities|Time|GetWorldDeltaSeconds) (Math|Float|Sign(Float) (- (Variables|Default|GetTargetValue) (Variables|Default|GetMoonValue))) (/ 1.0 (Variables|Default|GetLerpTime))) (Variables|Default|GetMoonValue)) (!= (Math|Float|Sign(Float) (- (Variables|Default|GetTargetValue) (+ (* (Utilities|Time|GetWorldDeltaSeconds) (Math|Float|Sign(Float) (- (Variables|Default|GetTargetValue) (Variables|Default|GetMoonValue))) (/ 1.0 (Variables|Default|GetLerpTime))) (Variables|Default|GetMoonValue)))) (Math|Float|Sign(Float) (- (Variables|Default|GetTargetValue) (Variables|Default|GetMoonValue))))))
  (Rendering|Components|Light|SetLightColor (Variables|Default|GetMoonlight) (Class|KismetMathLibrary|LinearColorLerpUsingHSV (Variables|Default|GetColour%20Base) (Variables|Default|GetColour%20Red) (Variables|Default|GetMoonValue)) true)
  (Rendering|Components|Light|SetIntensity (Variables|Default|GetMoonlight) (Math|Float|Lerp (Variables|Default|GetBaseIntensity) (Variables|Default|GetBloodIntensity) (Variables|Default|GetMoonValue)))
  (if (== (Variables|Default|GetMoonValue) (Variables|Default|GetTargetValue))
    (Utilities|Time|ClearandInvalidateTimerbyHandle (Variables|Default|GetMoonTimer))))

(event Custom|SetMoon
  (params (IsBloodMoon :type Boolean))
  (if IsBloodMoon
    (CallFunction|BloodMoon)
    (else
      (CallFunction|RegularMoon))))

(event EventBeginPlay
  (Variables|Default|SetColour%20Base (Rendering|Components|Light|GetLightColor (Variables|Default|GetMoonlight)))
  (bind _asgm_main (Utilities|Casting|CastToGM_Main (Game|GetGameMode)))
  (EventDispatchers|BindEventtoSetMoon _asgm_main (delegate Custom|SetMoon))
  (Variables|Default|SetBaseIntensity (Variables|/Script/Engine.LightComponentBase|GetIntensity (Variables|Default|GetMoonlight))))

(fn ConstructionScript)